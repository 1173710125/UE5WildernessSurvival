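; Behavior tree task that stops an AI pawn and holds it in an aiming state for a limited time.
; It sets the aiming and upper body interaction states through a pawn interface, clearing the second after the shooting block delay.
; Aiming then continues for a random duration before the task succeeds.
; Aborting the task clears both states.
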(event `self.ReceiveExecuteAI`
  (params (OwnerController :type "AIController Object Reference") (ControlledPawn :type "Pawn Object Reference"))
  ;[1 1 1] Set aiming state for controlled pawn for specific duration.
  (`Controller.StopMovement` OwnerController)
  (message `/Game/EasySurvivalRPG/Blueprints/Interfaces/BPI_Character.SetInteractionState_BPI` ControlledPawn "NewEnumerator9" true)
  (message `/Game/EasySurvivalRPG/Blueprints/Interfaces/BPI_Character.SetInteractionState_BPI` ControlledPawn "NewEnumerator2" true)
  (`KismetSystemLibrary.Delay` (`self.BlockShootingTime`))
  (message `/Game/EasySurvivalRPG/Blueprints/Interfaces/BPI_Character.SetInteractionState_BPI` ControlledPawn "NewEnumerator2" false)
  (`KismetSystemLibrary.Delay` (`KismetMathLibrary.RandomFloatInRange` (`self.MinAimingTime`) (`self.MaxAimingTime`)))
  (message `/Game/EasySurvivalRPG/Blueprints/Interfaces/BPI_Character.SetInteractionState_BPI` ControlledPawn "NewEnumerator9" false)
  (`self.FinishExecute` true))

(event `self.ReceiveAbortAI`
  (params (OwnerController :type "AIController Object Reference") (ControlledPawn :type "Pawn Object Reference"))
  ;[1 1 1] Reset aiming and upper body states on abort.
  (message `/Game/EasySurvivalRPG/Blueprints/Interfaces/BPI_Character.SetInteractionState_BPI` ControlledPawn "NewEnumerator9" false)
  (message `/Game/EasySurvivalRPG/Blueprints/Interfaces/BPI_Character.SetInteractionState_BPI` ControlledPawn "NewEnumerator2" false)
  (`self.FinishAbort`))