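; Behavior tree task that picks a strafe destination around the AI's target actor and writes it to a blackboard vector.
; It rotates the target-to-pawn yaw by a random signed angle and offsets the current distance randomly, with a lower clamp.
; The point is projected onto the navmesh, falling back to the raw point if projection fails.
; The task fails only when the target actor is invalid.
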(event `self.ReceiveExecuteAI`
  (params (OwnerController :type "AIController Object Reference") (ControlledPawn :type "Pawn Object Reference"))
  ;[1 1 1] Move strafe arount target actor.
  (set `self.OwnerController` OwnerController)
  (set `self.ControlledPawn` ControlledPawn)
  (bind (_success _resultlocation) (`self.FindLocationAroundTarget`))
  (if _success
    (`BTFunctionLibrary.SetBlackboardValueAsVector` (`self.UpdateTargetLocation`) _resultlocation)
    (`self.FinishExecute` true)
    (else
      (`self.FinishExecute` false))))

(fn `FindLocationAroundTarget`
  (returns (Success :type Boolean) (ResultLocation :type "Vector Structure"))
  (locals (LocalTargetActor :type "Actor Object Reference") (LocalCenterLocation :type "Vector Structure") (LocalPawnLocation :type "Vector Structure") (LocalLookRotation :type "Rotator Structure") (LocalDistanceToTarget :type "Float (double-precision)") (LocalNewLocation :type "Vector Structure" :default (0.0 0.0 0.0)))
  (bind _localcenterlocation (`local.LocalCenterLocation`))
  (bind _returnvalue (`BTFunctionLibrary.GetBlackboardValueAsActor` (`self.TargetActor`)))
  (bind _returnvalue_2 (+ (`local.LocalDistanceToTarget`) (`KismetMathLibrary.RandomFloatInRange` (`self.MinDistanceOffset`) (`self.MaxDistanceOffset`))))
  (`/Engine/EditorBlueprintResources/StandardMacros.IsValid` _returnvalue
    (:`Is Valid`
      (set `local.LocalTargetActor` _returnvalue)
      (set `local.LocalCenterLocation` (`Actor.K2_GetActorLocation` _returnvalue))
      (bind _output_get (set `local.LocalPawnLocation` (`Actor.K2_GetActorLocation` (`self.ControlledPawn`))))
      (bind _output_get_2 (set `local.LocalLookRotation` (`KismetMathLibrary.FindLookAtRotation` _localcenterlocation _output_get)))
      (set `local.LocalDistanceToTarget` (`KismetMathLibrary.VSize` (- (`local.LocalPawnLocation`) _localcenterlocation)))
      (bind _output_get_3 (set `local.LocalNewLocation` (+ (`local.LocalCenterLocation`) (* (`KismetMathLibrary.GetForwardVector` (`KismetMathLibrary.MakeRotator` 0.0 0.0 (+ (.yaw _output_get_2) (* (`KismetMathLibrary.RandomFloatInRange` (`self.MinAngle`) (`self.MaxAngle`)) (select `bool` (`KismetMathLibrary.RandomBool`) :`false` -1.0 :`true` 1.0 :!type "Float (single-precision)"))))) (`KismetMathLibrary.FClamp` _returnvalue_2 100.0 _returnvalue_2)))))
      (bind (_projectedlocation _returnvalue_3) (`NavigationSystemV1.K2_ProjectPointToNavigation` _output_get_3))
      (if _returnvalue_3
        (return true _projectedlocation)
        (else
          (return true (`local.LocalNewLocation`)))))
    (:`Is Not Valid`
      (return false (0.0 0.0 0.0)))))