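; Behavior tree task that sends a swine to a nearby pig for breeding.
; It restarts the swine's find-pig timer, then uses sphere traces to find an empty pig coop and a pig not already breeding.
; After walking to the pig, it rechecks the coop and activates find-coop behavior on both animals.
; The task fails when either search fails, but reports success even if the move fails.
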(event `self.ReceiveExecuteAI`
  (params (OwnerController :type "AIController Object Reference") (ControlledPawn :type "Pawn Object Reference"))
  ;[1 1 1] Move to available pig for mating.
  (bind _asbp_character_swine (cast `/Game/EasySurvivalRPG/Blueprints/Characters/Base/BP_Character_Swine` ControlledPawn)
    (:`then`
      (`/Game/EasySurvivalRPG/Blueprints/Characters/Base/BP_Character_Swine.StartFindPigTimer` _asbp_character_swine)
      (bind (_found _targetcoop) (`self.TryToFindCoop` _asbp_character_swine))
      (if _found
        (bind (_found_2 _targetpig) (`self.TryToFindPig` _asbp_character_swine))
        (if _found_2
          (`|AIMoveTo` _asbp_character_swine (0.0 0.0 0.0) _targetpig 100.0 true
            (:`OnSuccess`
              (`/Engine/EditorBlueprintResources/StandardMacros.IsValid` _targetcoop
                (:`Is Valid`
                  (`/Engine/EditorBlueprintResources/StandardMacros.IsValid` _targetpig
                    (:`Is Valid`
                      (`self.SetTargetCoopForPigs` _asbp_character_swine _targetpig _targetcoop))
                    (:`Is Not Valid`
                      _)))
                (:`Is Not Valid`
                  _)))
            (:`OnFail`
              _))
          (`self.FinishExecute` true)
          (else
            (`self.FinishExecute` false :!label _label)))
        (else
          (goto _label))))
    (:`CastFailed`
      (goto _label))))

(fn `SetTargetCoopForPigs`
  (params (Swine :type "/Game/EasySurvivalRPG/Blueprints/Characters/Base/BP_Character_Swine Object Reference") (Pig :type "/Game/EasySurvivalRPG/Blueprints/Characters/Base/BP_Character_Pig Object Reference") (TargetCoop :type "/Game/EasySurvivalRPG/Blueprints/InteractionObjects/BuildingObjects/Farming/BP_Building_PigCoop Object Reference"))
  ;[1 1 1] Activate find coop behavior for pigs.
  (if (`/Game/EasySurvivalRPG/Blueprints/InteractionObjects/BuildingObjects/Farming/BP_Building_PigCoop.CoopIsEmpty` TargetCoop)
    (`|ExecutionSequence`
      (:`then_0`
        (`/Engine/EditorBlueprintResources/StandardMacros.IsValid` Swine
          (:`Is Valid`
            (`/Game/EasySurvivalRPG/Blueprints/Characters/Base/BP_Character_Swine.ActivateFindCoopBehavior` Swine TargetCoop)
            (`/Game/EasySurvivalRPG/Blueprints/Characters/Base/BP_Character_Swine.StartFindPigTimer` Swine))))
      (:`then_1`
        (`/Engine/EditorBlueprintResources/StandardMacros.IsValid` Pig
          (:`Is Valid`
            (`/Game/EasySurvivalRPG/Blueprints/Characters/Base/BP_Character_Pig.ActivateFindCoopBehavior` Pig TargetCoop)))))))

(fn `TryToFindCoop`
  (params (ControlledPawn :type "Pawn Object Reference"))
  (returns (Found :type Boolean) (TargetCoop :type "/Game/EasySurvivalRPG/Blueprints/InteractionObjects/BuildingObjects/Farming/BP_Building_PigCoop Object Reference") (TargetLocation :type "Vector Structure"))
  (bind _returnvalue (`Actor.K2_GetActorLocation` ControlledPawn))
  ;[1 1 1] Try to find available coop.
  (bind _outhits (`KismetSystemLibrary.SphereTraceMultiForObjects` _returnvalue _returnvalue 1000.0 (`|MakeArray` "ObjectTypeQuery2" :!type "EObjectTypeQuery Enum")))
  (for _array_element _outhits
    (bind _asbp_building_pig_coop (cast `/Game/EasySurvivalRPG/Blueprints/InteractionObjects/BuildingObjects/Farming/BP_Building_PigCoop` (`.HitActor` (`GameplayStatics.BreakHitResult` _array_element))))
    (if (`/Game/EasySurvivalRPG/Blueprints/InteractionObjects/BuildingObjects/Farming/BP_Building_PigCoop.CoopIsEmpty` _asbp_building_pig_coop)
      (return true _asbp_building_pig_coop (`Actor.K2_GetActorLocation` _asbp_building_pig_coop))))
  (return false null (0.0 0.0 0.0)))

(fn `TryToFindPig`
  (params (ControlledPawn :type "Pawn Object Reference"))
  (returns (Found :type Boolean) (TargetPig :type "/Game/EasySurvivalRPG/Blueprints/Characters/Base/BP_Character_Pig Object Reference"))
  (bind _returnvalue (`Actor.K2_GetActorLocation` ControlledPawn))
  ;[1 1 1] Try to find pig without active breeding timer.
  (bind _outhits (`KismetSystemLibrary.SphereTraceMultiForObjects` _returnvalue _returnvalue 500.0 (`|MakeArray` "ObjectTypeQuery3" :!type "EObjectTypeQuery Enum")))
  (for _array_element _outhits
    (bind _asbp_character_pig (cast `/Game/EasySurvivalRPG/Blueprints/Characters/Base/BP_Character_Pig` (`.HitActor` (`GameplayStatics.BreakHitResult` _array_element))))
    (if (not (`/Game/EasySurvivalRPG/Blueprints/Characters/Base/BP_Character_Pig.BreedingInProcess` _asbp_character_pig))
      (return true _asbp_character_pig)))
  (return false null))