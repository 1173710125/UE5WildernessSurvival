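; Behavior tree task that sends a pig, swine or piglet to a nearby feeder with food to eat.
; It restarts the pawn's find-food timer, then sphere-traces around it for the first pig feeder reporting food and moves there with AI MoveTo.
; On arrival the pawn tries to eat and the feeder consumes food.
; The task fails if no feeder is found, but still succeeds when the move fails.
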(event `self.ReceiveExecuteAI`
  (params (OwnerController :type "AIController Object Reference") (ControlledPawn :type "Pawn Object Reference"))
  ;[1 1 1] Move to available feeder and play eat animation.
  (bind _success (`self.PigStartFindFoodTimer` ControlledPawn))
  (if _success
    (bind (_found _targetactor) (`self.TryToFindFood` ControlledPawn))
    (if _found
      (`|AIMoveTo` ControlledPawn (0.0 0.0 0.0) _targetactor 75.0 true
        (:`OnSuccess`
          (`/Engine/EditorBlueprintResources/StandardMacros.IsValid` _targetactor
            (:`Is Valid`
              (`self.PigTryEat` ControlledPawn _targetactor))
            (:`Is Not Valid`
              _)))
        (:`OnFail`
          _))
      (`self.FinishExecute` true)
      (else
        (`self.FinishExecute` false :!label _label)))
    (else
      (goto _label))))

(fn `PigStartFindFoodTimer`
  (params (ControlledPawn :type "Pawn Object Reference"))
  (returns (Success :type Boolean))
  ;[1 1 1] Start find food timer.
  (bind _asbp_character_pig (cast `/Game/EasySurvivalRPG/Blueprints/Characters/Base/BP_Character_Pig` ControlledPawn)
    (:`then`
      (`/Game/EasySurvivalRPG/Blueprints/Characters/Base/BP_Character_Pig.StartFindFoodTimer` _asbp_character_pig))
    (:`CastFailed`
      (bind _asbp_character_swine (cast `/Game/EasySurvivalRPG/Blueprints/Characters/Base/BP_Character_Swine` ControlledPawn)
        (:`then`
          (`/Game/EasySurvivalRPG/Blueprints/Characters/Base/BP_Character_Swine.StartFindFoodTimer` _asbp_character_swine))
        (:`CastFailed`
          (bind _asbp_character_piglet (cast `/Game/EasySurvivalRPG/Blueprints/Characters/Base/BP_Character_Piglet` ControlledPawn)
            (:`then`
              (`/Game/EasySurvivalRPG/Blueprints/Characters/Base/BP_Character_Piglet.StartFindFoodTimer` _asbp_character_piglet))
            (:`CastFailed`
              (return false)))))))
  (return true))

(fn `PigTryEat`
  (params (ControlledPawn :type "Pawn Object Reference") (TargetActor :type "Actor Object Reference"))
  (returns (Success :type Boolean))
  ;[1 1 1] Try to eat.
  (bind _asbp_character_pig (cast `/Game/EasySurvivalRPG/Blueprints/Characters/Base/BP_Character_Pig` ControlledPawn)
    (:`then`
      (`/Game/EasySurvivalRPG/Blueprints/Characters/Base/BP_Character_Pig.TryEat` _asbp_character_pig)
      (`/Game/EasySurvivalRPG/Blueprints/Characters/Base/BP_Character_Pig.StartFindFoodTimer` _asbp_character_pig)
      (bind _asbp_building_pig_feeder (cast `/Game/EasySurvivalRPG/Blueprints/InteractionObjects/BuildingObjects/Farming/BP_Building_PigFeeder` TargetActor :!label _label)
        (:`then`
          _)
        (:`CastFailed`
          (return false))))
    (:`CastFailed`
      (bind _asbp_character_swine (cast `/Game/EasySurvivalRPG/Blueprints/Characters/Base/BP_Character_Swine` ControlledPawn)
        (:`then`
          (`/Game/EasySurvivalRPG/Blueprints/Characters/Base/BP_Character_Swine.TryEat` _asbp_character_swine)
          (`/Game/EasySurvivalRPG/Blueprints/Characters/Base/BP_Character_Swine.StartFindFoodTimer` _asbp_character_swine)
          (goto _label))
        (:`CastFailed`
          (bind _asbp_character_piglet (cast `/Game/EasySurvivalRPG/Blueprints/Characters/Base/BP_Character_Piglet` ControlledPawn)
            (:`then`
              (`/Game/EasySurvivalRPG/Blueprints/Characters/Base/BP_Character_Piglet.TryEat` _asbp_character_piglet)
              (`/Game/EasySurvivalRPG/Blueprints/Characters/Base/BP_Character_Piglet.StartFindFoodTimer` _asbp_character_piglet)
              (goto _label))
            (:`CastFailed`
              (return false)))))))
  (`/Game/EasySurvivalRPG/Blueprints/InteractionObjects/BuildingObjects/Farming/BP_Building_PigFeeder.ConsumeFood` _asbp_building_pig_feeder)
  (return true))

(fn `TryToFindFood`
  (params (ControlledPawn :type "Pawn Object Reference"))
  (returns (Found :type Boolean) (TargetActor :type "Actor Object Reference") (TargetLocation :type "Vector Structure"))
  (bind _returnvalue (`Actor.K2_GetActorLocation` ControlledPawn))
  ;[1 1 1] Try to find available feeder.
  (bind _outhits (`KismetSystemLibrary.SphereTraceMultiForObjects` _returnvalue _returnvalue 500.0 (`|MakeArray` "ObjectTypeQuery2" :!type "EObjectTypeQuery Enum")))
  (for _array_element _outhits
    (bind _asbp_building_pig_feeder (cast `/Game/EasySurvivalRPG/Blueprints/InteractionObjects/BuildingObjects/Farming/BP_Building_PigFeeder` (`.HitActor` (`GameplayStatics.BreakHitResult` _array_element))))
    (if (`/Game/EasySurvivalRPG/Blueprints/InteractionObjects/BuildingObjects/Farming/BP_Building_PigFeeder.HasFood` _asbp_building_pig_feeder)
      (return true _asbp_building_pig_feeder (`Actor.K2_GetActorLocation` _asbp_building_pig_feeder))))
  (return false null (0.0 0.0 0.0)))