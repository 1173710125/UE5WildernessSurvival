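; Behavior tree decorator that passes when the AI pawn's distance to its target is within an acceptance radius.
; Each check recomputes the radius from a fixed value, a blackboard key, or the sum of both, depending on two flags.
; It then compares that radius against the DistanceToTarget value read from the blackboard rather than measuring the distance itself.
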(fn `PerformConditionCheckAI`
  (params (OwnerController :type "AIController Object Reference") (ControlledPawn :type "Pawn Object Reference"))
  (returns (ReturnValue :type Boolean))
  ;[1 1 1] Return true if distance to target in result acceptance radius.
  (`self.UpdateAcceptanceRadius`)
  (return (<= (`BTFunctionLibrary.GetBlackboardValueAsFloat` (`self.DistanceToTarget`)) (`self.ResultAcceptanceRadius`))))

(fn `UpdateAcceptanceRadius`
  (bind _acceptanceradius (`self.AcceptanceRadius`))
  (bind _returnvalue (`BTFunctionLibrary.GetBlackboardValueAsFloat` (`self.BlackboardRadius`)))
  ;[1 1 1] Update acceptance radius.
  (if (`self.UseBlackboardRadius`)
    (set `self.ResultAcceptanceRadius` (select `bool` (`self.SumRadiusValues`) :`false` _returnvalue :`true` (+ _acceptanceradius _returnvalue)))
    (else
      (set `self.ResultAcceptanceRadius` _acceptanceradius))))