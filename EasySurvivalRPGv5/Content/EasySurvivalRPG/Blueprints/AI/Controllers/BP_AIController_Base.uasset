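; Base AI controller that bridges blackboard, perception and aiming data to its controlled pawn through Blueprint interface messages.
; On BeginPlay, the server sets up the base blackboard, then after a short delay tells the pawn to run its AI.
; Perception updates are forwarded to the pawn.
; Interface getters supply fixed accuracy values and a focus rotation toward the focus actor, falling back to control rotation.
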(event `self.ReceiveBeginPlay`
  ;[1 1 1] Initialize Blackboard and Behavior Tree for AI Controller.
  (`/Engine/EditorBlueprintResources/ActorMacros.Switch Has Authority`
    (:`Authority`
      (`self.UseBlackboard` "/Game/EasySurvivalRPG/Blueprints/AI/Behaviors/Base/BB_Base.BB_Base")
      (`KismetSystemLibrary.Delay` 0.1)
      (message `/Game/EasySurvivalRPG/Blueprints/Interfaces/BPI_Character.RunAI_BPI` (`self.K2_GetPawn`)))))

(event `self.AIPerceptionComponent.OnTargetPerceptionUpdated`
  (params (Actor :type "Actor Object Reference") (Stimulus :type "AIStimulus Structure"))
  ;[1 1 1] Update perception.
  (message `/Game/EasySurvivalRPG/Blueprints/Interfaces/BPI_Character.UpdatePerceptionTarget_BPI` (`self.K2_GetPawn`) Actor Stimulus false))

(fn `GetAccuracyVariables_BPI`
  (returns (Success :type Boolean) (Accuracy :type "Float (double-precision)") (MaxPitch :type "Float (double-precision)") (MaxYaw :type "Float (double-precision)"))
  ;[1 1 1] Returns accuracy variable of the controller.
  (return true 0.5 5.0 5.0))

(fn `GetFocusVariables_BPI`
  (returns (Success :type Boolean) (Location :type "Vector Structure") (Rotation :type "Rotator Structure"))
  (bind _returnvalue (`self.K2_GetActorLocation`))
  (bind _returnvalue_2 (`self.GetFocusActor`))
  ;[1 1 1] Returns focus variables of the controller.
  (`/Engine/EditorBlueprintResources/StandardMacros.IsValid` _returnvalue_2
    (:`Is Valid`
      (return true _returnvalue (`KismetMathLibrary.FindLookAtRotation` _returnvalue (`self.K2_GetActorLocation` _returnvalue_2))))
    (:`Is Not Valid`
      (return true _returnvalue (`self.GetControlRotation`)))))

(fn `UserConstructionScript`)