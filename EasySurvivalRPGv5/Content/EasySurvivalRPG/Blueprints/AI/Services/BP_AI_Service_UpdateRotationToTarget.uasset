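; Behavior tree service that keeps an AI's look-at rotation toward its target updated in the blackboard.
; On each tick it reads the target actor key and checks that the actor is valid and reports alive through a Blueprint interface message.
; It then writes the rotation from the controlled pawn to that actor into the rotation blackboard key, without rotating the pawn itself.
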(event `self.ReceiveTickAI`
  (params (OwnerController :type "AIController Object Reference") (ControlledPawn :type "Pawn Object Reference") (DeltaSeconds :type "Float (single-precision)"))
  ;[1 1 1] Update rotation to target actor on tick.
  (`self.UpdateRotationToTarget` OwnerController ControlledPawn))

(fn `UpdateRotationToTarget`
  (params (OwnerController :type "AIController Object Reference") (ControlledPawn :type "Pawn Object Reference"))
  (returns (Success :type Boolean))
  (locals (LocalOrderTarget :type "Actor Object Reference") (LocalTargetActor :type "Actor Object Reference"))
  ;[1 1 1] Update rotation to target actor blackboard value.
  (bind _output_get (set `local.LocalTargetActor` (`BTFunctionLibrary.GetBlackboardValueAsActor` (`self.TargetActor`))))
  (`/Engine/EditorBlueprintResources/StandardMacros.IsValid` _output_get
    (:`Is Valid`
      (bind _result (message `/Game/EasySurvivalRPG/Blueprints/Interfaces/BPI_Character.IsAlive_BPI` _output_get))
      (if _result
        (`BTFunctionLibrary.SetBlackboardValueAsRotator` (`self.RotationToTarget`) (`KismetMathLibrary.FindLookAtRotation` (`Actor.K2_GetActorLocation` ControlledPawn) (`Actor.K2_GetActorLocation` _output_get)))
        (return true)))))