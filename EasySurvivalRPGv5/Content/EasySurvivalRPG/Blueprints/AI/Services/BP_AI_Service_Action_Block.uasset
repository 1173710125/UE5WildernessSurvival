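; Behavior tree action service that makes an AI pawn block when its target attacks.
; The condition check extends the parent's check by querying the blackboard target actor's interaction state through an interface message.
; The action sends a try-block interface message with a blocking time to the controlled pawn, running the parent action only if that succeeds.
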(fn `CheckConditions`
  (params (ControlledPawn :type "Pawn Object Reference"))
  (returns (Success :type Boolean))
  (bind _returnvalue (`BTFunctionLibrary.GetBlackboardValueAsActor` (`self.TargetActor`)))
  ;[1 1 1] Check that the target attacks.
  (bind _success (`parent.CheckConditions` ControlledPawn))
  (if _success
    (`/Engine/EditorBlueprintResources/StandardMacros.IsValid` _returnvalue
      (:`Is Valid`
        (bind _state (message `/Game/EasySurvivalRPG/Blueprints/Interfaces/BPI_Character.GetInteractionState_BPI` _returnvalue "NewEnumerator0"))
        (return _state))
      (:`Is Not Valid`
        _)))
  (return false))

(fn `DoActions`
  (params (ControlledPawn :type "Pawn Object Reference"))
  (returns (Success :type Boolean))
  ;[1 1 1] Try block.
  (bind _success (message `/Game/EasySurvivalRPG/Blueprints/Interfaces/BPI_Character.TryBlock_BPI` ControlledPawn (`self.BlockingTime`)))
  (if _success
    (bind _success_2 (`parent.DoActions` ControlledPawn))
    (return _success_2)
    (else
      (return false))))