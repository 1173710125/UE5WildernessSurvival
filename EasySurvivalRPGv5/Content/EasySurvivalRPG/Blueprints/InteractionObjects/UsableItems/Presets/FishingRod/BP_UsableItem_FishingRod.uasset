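; Fishing rod usable item that manages a cast floater projectile, its fishing line and catch attempts.
; InitFloater links rod and floater, TryCatchFish delegates to the floater, and the server destroys the floater when it exceeds the maximum line distance.
; FloaterReference's RepNotify attaches and shows the cable on the floater, or resets and hides it when none exists.
; Named start and end fishing animations play through multicast events as dynamic slot montages.
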(event `self.ReceiveTick`
  (params (DeltaSeconds :type "Float (single-precision)"))
  (bind _floaterreference (`self.FloaterReference`))
  ;[1 1 1] Event tick.Check floater distance.
  (`/Engine/EditorBlueprintResources/ActorMacros.Switch Has Authority`
    (:`Authority`
      (`/Engine/EditorBlueprintResources/StandardMacros.IsValid` _floaterreference
        (:`Is Valid`
          (if (> (`KismetMathLibrary.VSize` (- (`self.K2_GetActorLocation` _floaterreference) (`SceneComponent.GetSocketLocation` (`self.StaticMeshComponent`) "Start"))) (`self.FishingLineMaxDistance`))
            (`self.RemoveFloater`)))))))

(event `/Game/EasySurvivalRPG/Blueprints/Interfaces/BPI_UsableItem.PlayAnimationByName_BPI`
  (params (Name :type Name))
  ;[1 1 1] Play start and end fishing animations.
  (switch `name` Name
    (:`StartFishing`
      (`self.PlayStartFishingAnimation (Multicast)`))
    (:`EndFishing`
      (`self.PlayEndFishingAnimation (Multicast)`))))

(event `PlayStartFishingAnimation (Multicast)`
  (bind (_anim _slotname _blendintime _blendouttime _inplayrate _loopcount _blendouttriggertime _intimetostartmontageat) (break `/Game/EasySurvivalRPG/Blueprints/Structures/Misc/STR_AnimationPlayData` (`self.StartFishingAnim`)))
  ;[1 1 1] Play start and end fishing animations.
  (`AnimInstance.PlaySlotAnimationAsDynamicMontage` (`SkeletalMeshComponent.GetAnimInstance` (`self.SkeletalMeshComponent`)) _anim _slotname _blendintime _blendouttime _inplayrate _loopcount _blendouttriggertime _intimetostartmontageat))

(event `PlayEndFishingAnimation (Multicast)`
  (bind (_anim _slotname _blendintime _blendouttime _inplayrate _loopcount _blendouttriggertime _intimetostartmontageat) (break `/Game/EasySurvivalRPG/Blueprints/Structures/Misc/STR_AnimationPlayData` (`self.EndFishingAnim`)))
  ;[1 1 1] Play start and end fishing animations.
  (`AnimInstance.PlaySlotAnimationAsDynamicMontage` (`SkeletalMeshComponent.GetAnimInstance` (`self.SkeletalMeshComponent`)) _anim _slotname _blendintime _blendouttime _inplayrate _loopcount _blendouttriggertime _intimetostartmontageat))

(fn `InitFloater`
  (params (Floater :type "Actor Object Reference"))
  ;[1 1 1] Init floater reference.
  (bind _asbp_projectile_floater (cast `/Game/EasySurvivalRPG/Blueprints/InteractionObjects/Projectiles/Presets/BP_Projectile_Floater` Floater))
  (bind _output_get (set `self.FloaterReference` _asbp_projectile_floater))
  (`/Game/EasySurvivalRPG/Blueprints/InteractionObjects/Projectiles/Presets/BP_Projectile_Floater.SetFishingRod` _output_get self))

(fn `OnRep_FloaterReference`
  (bind _floaterreference (`self.FloaterReference`))
  (bind _fishingline (`self.FishingLine`))
  ;[1 1 1] Attach cable to floater if reference is valid and update cable visibility.
  (`/Engine/EditorBlueprintResources/StandardMacros.IsValid` _floaterreference
    (:`Is Valid`
      (`CableComponent.SetAttachEndTo` _fishingline _floaterreference "FloaterMesh" "FishingLine"))
    (:`Is Not Valid`
      (`CableComponent.SetAttachEndTo` _fishingline self "SkeletalMeshComponent" "Start")))
  (`SceneComponent.SetVisibility` _fishingline (`KismetSystemLibrary.IsValid` _floaterreference) false))

(fn `RemoveFloater`
  (bind _floaterreference (`self.FloaterReference`))
  ;[1 1 1] Destroy floater and clear reference.
  (`/Engine/EditorBlueprintResources/StandardMacros.IsValid` _floaterreference
    (:`Is Valid`
      (`self.K2_DestroyActor` _floaterreference)
      (set `self.FloaterReference` null))))

(fn `TryCatchFish`
  (returns (Success :type Boolean))
  (bind _floaterreference (`self.FloaterReference`))
  ;[1 1 1] Try catch a fish.
  (`/Engine/EditorBlueprintResources/StandardMacros.IsValid` _floaterreference
    (:`Is Valid`
      (bind _success (`/Game/EasySurvivalRPG/Blueprints/InteractionObjects/Projectiles/Presets/BP_Projectile_Floater.TryCatchFish` _floaterreference))
      (return _success))))

(fn `UserConstructionScript`
  (`parent.UserConstructionScript`))