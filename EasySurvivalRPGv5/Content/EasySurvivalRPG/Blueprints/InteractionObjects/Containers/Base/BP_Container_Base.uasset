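; Base interactable loot container for the survival RPG, with configurable mesh, slot count and name.
; Interaction release opens its ContainerComponent through the player controller, and the first open rolls loot from LootHandle into it, passing the actor's location for overflow drops.
; The server initializes the component, and open/close events multicast sounds.
; Save/load persists the one-time loot flag by SaveID and forwards data to components implementing BPI_SaveData.
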(event `self.ReceiveBeginPlay`
  ;[1 1 1] Begin play. Components initialization.
  (`/Engine/EditorBlueprintResources/ActorMacros.Switch Has Authority`
    (:`Authority`
      (`/Game/EasySurvivalRPG/Blueprints/Components/BP_ContainerComponent.InitComponent` (`self.ContainerComponent`)))))

(event `/Game/EasySurvivalRPG/Blueprints/Interfaces/BPI_InteractionObject.TryInteract_BPI`
  (params (Release :type Boolean) (PlayerController :type "PlayerController Object Reference"))
  (bind _returnvalue (not (`self.LootWasAdded`)))
  ;[1 1 1] Interactions.
  (if Release
    (message `/Game/EasySurvivalRPG/Blueprints/Interfaces/BPI_Player.OpenContainer_BPI` PlayerController (`self.ContainerComponent`))
    (if _returnvalue
      (set `self.LootWasAdded` _returnvalue)
      (`/Game/EasySurvivalRPG/Blueprints/Components/BP_ContainerComponent.TryAddItemsOrDropAtLocation` (`self.ContainerComponent`) (`/Game/EasySurvivalRPG/Blueprints/Game/Libraries/BP_ItemsLibrary.MakeLootItems` (`self.LootHandle`)) (`self.K2_GetActorLocation`)))))

(event `self.ContainerComponent.OnOpened`
  ;[1 1 1] Interactions.
  (`self.PlaySound (Multicast)` (`self.OpenContainerSound`)))

(event `self.ContainerComponent.OnClosed`
  ;[1 1 1] Interactions.
  (`self.PlaySound (Multicast)` (`self.CloseContainerSound`)))

(event `PlaySound (Multicast)`
  (params (Sound :type "SoundBase Object Reference"))
  ;[1 1 1] Sound effects.
  (`GameplayStatics.PlaySoundAtLocation` Sound (`self.K2_GetActorLocation`) (struct) 1.0 1.0 0.0 null null null))

(fn `CheckCanInteract_BPI`
  (params (PlayerController :type "PlayerController Object Reference"))
  (returns (CanInteract :type Boolean))
  (return true))

(fn `DoesIgnoreSaveLoad_BPI`
  (returns (Result :type Boolean))
  (return false))

(fn `GetComponentSaveID_BPI`
  (returns (Success :type Boolean) (ComponentSaveID :type Integer))
  (return false 0))

(fn `GetFormattedVariables_BPI`
  (returns (FormattedVariables :type "Array of String"))
  (return (`|MakeArray` (`/Game/EasySurvivalRPG/Blueprints/Game/Libraries/BP_SaveLibrary.FormatBooleanVariableToString` "LootWasAdded" (`self.LootWasAdded`)))))

(fn `GetInteractionObjectName_BPI`
  (returns (Name :type Text))
  (return (`self.ContainerName`)))

(fn `GetInteractionText_BPI`
  (params (PlayerController :type "PlayerController Object Reference"))
  (returns (InteractionText :type Text))
  (return (`|FormatText` "Open {ContainerName}" (`self.ContainerName`))))

(fn `GetSaveID_BPI`
  (returns (Success :type Boolean) (SaveID :type Integer))
  (return true (`self.SaveID`)))

(fn `IsTurnedOn_BPI`
  (returns (IsTurnedOn :type Boolean))
  (return false))

(fn `LoadData_BPI`
  (params (SaveData :type "SaveGame Object Reference"))
  (returns (Success :type Boolean))
  (locals (LocalSaveData :type "SaveGame Object Reference"))
  (bind _output_get (set `local.LocalSaveData` SaveData))
  (for _array_element (`self.K2_GetComponentsByClass` "/Script/Engine.ActorComponent")
    (if (`KismetSystemLibrary.DoesImplementInterface` _array_element "/Game/EasySurvivalRPG/Blueprints/Interfaces/BPI_SaveData.BPI_SaveData_C")
      (message `/Game/EasySurvivalRPG/Blueprints/Interfaces/BPI_SaveData.LoadData_BPI` _array_element (`local.LocalSaveData`))))
  (bind (_success _savedata) (message `/Game/EasySurvivalRPG/Blueprints/Interfaces/BPI_GameSave.GetActorSaveData_BPI` _output_get (`self.SaveID`)))
  (bind (_success_2 _value) (`/Game/EasySurvivalRPG/Blueprints/Game/Libraries/BP_SaveLibrary.GetFormattedVariableBooleanValue` (`.FormattedVariables_38_8140374D4327F2E43E03C3B17B80F74B` (break `/Game/EasySurvivalRPG/Blueprints/Structures/SaveData/STR_SaveData_Actor` _savedata)) "LootWasAdded"))
  (set `self.LootWasAdded` _value)
  (return true))

(fn `SaveData_BPI`
  (params (SaveData :type "SaveGame Object Reference"))
  (returns (Success :type Boolean))
  (locals (LocalSaveData :type "SaveGame Object Reference"))
  (bind _formattedvariables (`/Game/EasySurvivalRPG/Blueprints/Interfaces/BPI_SaveData.GetFormattedVariables_BPI`))
  (bind _output_get (set `local.LocalSaveData` SaveData))
  (message `/Game/EasySurvivalRPG/Blueprints/Interfaces/BPI_GameSave.SetActorSaveData_BPI` _output_get (`self.SaveID`) (make `/Game/EasySurvivalRPG/Blueprints/Structures/SaveData/STR_SaveData_Actor` (`GameplayStatics.GetObjectClass` self) (`self.GetTransform`) _formattedvariables))
  (for _array_element (`self.K2_GetComponentsByClass` "/Script/Engine.ActorComponent")
    (if (`KismetSystemLibrary.DoesImplementInterface` _array_element "/Game/EasySurvivalRPG/Blueprints/Interfaces/BPI_SaveData.BPI_SaveData_C")
      (message `/Game/EasySurvivalRPG/Blueprints/Interfaces/BPI_SaveData.SaveData_BPI` _array_element (`local.LocalSaveData`))))
  (return true))

(fn `SetSaveID_BPI`
  (params (SaveID :type Integer))
  (returns (Success :type Boolean))
  (set `self.SaveID` SaveID)
  (return true))

(fn `UserConstructionScript`
  (set `/Game/EasySurvivalRPG/Blueprints/Components/BP_ContainerComponent.Slots` (`self.ContainerSlots`) (`self.ContainerComponent`))
  (`StaticMeshComponent.SetStaticMesh` (`self.Mesh`) (`self.StaticMesh`)))