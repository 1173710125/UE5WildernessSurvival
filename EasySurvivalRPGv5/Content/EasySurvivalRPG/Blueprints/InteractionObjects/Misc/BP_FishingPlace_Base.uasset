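; BP_FishingPlace_Base is a base fishing spot actor that supplies randomized catch results and timings for fishing.
; It picks a random loot handle from its CatchFishLootHandles array, with a valid-index check.
; Two other helpers roll random catch and fish-off times within configurable min/max ranges.
; It has no event logic of its own, only these query functions.
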(fn `GetRandomCatchFishTime`
  (returns (CatchTime :type "Float (double-precision)"))
  ;[1 1 1] Returns random catch fish time.
  (return (`KismetMathLibrary.RandomFloatInRange` (`self.MinCatchFishTime`) (`self.MaxCatchFishTime`))))

(fn `GetRandomFishLootHandle`
  (returns (FishLootHandle :type "DataTableRowHandle Structure"))
  (locals (LocalIndex :type Integer :default 0))
  (bind _catchfishloothandles (`self.CatchFishLootHandles`))
  ;[1 1 1] Returns random fish loot handle.
  (bind _output_get (set `local.LocalIndex` (`KismetMathLibrary.RandomIntegerInRange` 0 (`KismetArrayLibrary.Array_LastIndex` _catchfishloothandles))))
  (if (`KismetArrayLibrary.Array_IsValidIndex` _catchfishloothandles _output_get)
    (return (`|GetArrayItem` _catchfishloothandles _output_get))))

(fn `GetRandomFishOffTime`
  (returns (CatchTime :type "Float (double-precision)"))
  ;[1 1 1] Returns random fish off time.
  (return (`KismetMathLibrary.RandomFloatInRange` (`self.MinFishOffTime`) (`self.MaxFishOffTime`))))

(fn `UserConstructionScript`)