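; Bomb projectile preset that turns into a physics-simulated body on its first hit instead of continuing its scripted flight and spin.
; Later impacts at sufficient speed play surface-based sounds and particles from the physical material.
; On destroy, the server starts a short timer and multicasts effect shutdown, which freezes physics, hides the mesh, stops audio and deactivates smoke and spark trails.
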(event `self.ReceiveHit`
  (params (MyComp :type "PrimitiveComponent Object Reference") (Other :type "Actor Object Reference") (OtherComp :type "PrimitiveComponent Object Reference") (bSelfMoved :type Boolean) (HitLocation :type "Vector Structure") (HitNormal :type "Vector Structure") (NormalImpulse :type "Vector Structure") (Hit :type "HitResult Structure (by ref)"))
  ;[1 1 1] Hit event of projectile.
  (`/Engine/EditorBlueprintResources/StandardMacros.DoOnce` false
    (:`Completed`
      (`PrimitiveComponent.SetSimulatePhysics` (`self.RootMeshComponent`) true)
      (`ActorComponent.Deactivate` (`self.ProjectileMovement`))
      (`ActorComponent.Deactivate` (`self.RotatingMovement`)))))

(event `self.DestroyProjectile`
  ;[1 1 1] Destroy projectile with delay.
  (`/Engine/EditorBlueprintResources/ActorMacros.Switch Has Authority`
    (:`Authority`
      (`KismetSystemLibrary.K2_SetTimerDelegate` (`|CreateDelegate` :!event `K2_DestroyActor`) 2.0)
      (`self.DisableBombEffects (Multicast)`))))

(event `DisableBombEffects (Multicast)`
  (bind _smoketrailparticle (`self.SmokeTrailParticle`))
  ;[1 1 1] Destroy projectile with delay.
  (`PrimitiveComponent.SetSimulatePhysics` (`self.RootMeshComponent`) false)
  (`SceneComponent.SetVisibility` (`self.ProjectileMesh`) false true)
  (`AudioComponent.Stop` (`self.Audio`))
  (`SceneComponent.SetVisibility` _smoketrailparticle true false)
  (`SceneComponent.SetVisibility` (`self.SparksParticle`) true false)
  (`ActorComponent.Deactivate` _smoketrailparticle)
  (`ActorComponent.Deactivate` (`self.SparksParticle`)))

(event `self.RootMeshComponent.OnComponentHit`
  (params (HitComponent :type "PrimitiveComponent Object Reference") (OtherActor :type "Actor Object Reference") (OtherComp :type "PrimitiveComponent Object Reference") (NormalImpulse :type "Vector Structure") (Hit :type "HitResult Structure (by ref)"))
  ;[1 1 1] Hit event of projectile.
  (if (>= (`KismetMathLibrary.VSize` (`self.GetVelocity`)) 100.0)
    (`self.PlayHitEffects` Hit)))

(fn `PlayHitEffects`
  (params (HitResult :type "HitResult Structure (by ref)"))
  (returns (Success :type Boolean))
  (locals (LocalHit :type "HitResult Structure") (LocalSurface :type "EPhysicalSurface Enum") (LocalLocation :type "Vector Structure") (LocalNormal :type "Vector Structure"))
  (bind (_bblockinghit _binitialoverlap _time _distance _location _impactpoint _normal _impactnormal _physmat) (`GameplayStatics.BreakHitResult` HitResult))
  ;[1 1 1] Play hit effects.
  (set `local.LocalHit` HitResult)
  (`/Engine/EditorBlueprintResources/StandardMacros.IsValid` _physmat
    (:`Is Valid`
      (bind _output_get (set `local.LocalSurface` (`PhysicalMaterial.SurfaceType` _physmat)))
      (bind _output_get_2 (set `local.LocalLocation` _location))
      (bind _output_get_3 (set `local.LocalNormal` _normal))
      (`self.PlayHitSound` _output_get _output_get_2)
      (`self.SpawnHitParticle` _output_get _output_get_2 _output_get_3)
      (return true))
    (:`Is Not Valid`
      (return false))))

(fn `UserConstructionScript`
  (`parent.UserConstructionScript`))