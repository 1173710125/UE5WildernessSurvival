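; BP_Projectile_Meteor is a meteor projectile preset that explodes on hit.
; It overrides events from a parent projectile, triggering the explosion only on the server.
; Destruction sets a short server-side timer to delay removal.
; The multicast explosion-effects event runs the parent effects, then deactivates the trail particle system on impact.
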(event `self.ReceiveHit`
  (params (MyComp :type "PrimitiveComponent Object Reference") (Other :type "Actor Object Reference") (OtherComp :type "PrimitiveComponent Object Reference") (bSelfMoved :type Boolean) (HitLocation :type "Vector Structure") (HitNormal :type "Vector Structure") (NormalImpulse :type "Vector Structure") (Hit :type "HitResult Structure (by ref)"))
  ;[1 1 1] Hit event of projectile.
  (`/Engine/EditorBlueprintResources/ActorMacros.Switch Has Authority`
    (:`Authority`
      (`self.ExplodeProjectile`))))

(event `/Game/EasySurvivalRPG/Blueprints/InteractionObjects/Projectiles/Base/BP_Projectile_Base.DestroyProjectile`
  ;[1 1 1] Destroy projectile delayed.
  (`/Engine/EditorBlueprintResources/ActorMacros.Switch Has Authority`
    (:`Authority`
      (`KismetSystemLibrary.K2_SetTimerDelegate` (`|CreateDelegate` :!event `K2_DestroyActor`) 1.0))))

(event `self.PlayExplosionEffects (Multicast)`
  (params (Location :type "Vector Structure"))
  ;[1 1 1] Deactivate trail particle after hit.
  (`parent.PlayExplosionEffects (Multicast)` Location)
  (`ActorComponent.Deactivate` (`self.ParticleSystem`)))

(fn `UserConstructionScript`
  (`parent.UserConstructionScript`))