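; BP_Building_WaterStorage is a placeable water storage building that players interact with as a crafting place.
; On begin play, if built, the authority initializes its container and feeds it to the crafting component.
; Releasing the interact input opens the crafting interface on both components with manual crafting disabled.
; Interaction is always allowed, name and prompt come from the building settings, and the turned-on state is unused.
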(event `self.ReceiveBeginPlay`
  (bind _containercomponent (`self.ContainerComponent`))
  ;[1 1 1] Begin play. Components initialization.
  (`parent.ReceiveBeginPlay`)
  (if (`self.Built`)
    (`/Engine/EditorBlueprintResources/ActorMacros.Switch Has Authority`
      (:`Authority`
        (`/Game/EasySurvivalRPG/Blueprints/Components/BP_ContainerComponent.InitComponent` _containercomponent)
        (`/Game/EasySurvivalRPG/Blueprints/Components/BP_CraftingComponent.InitComponent` (`self.CraftingComponent`) _containercomponent)))))

(event `/Game/EasySurvivalRPG/Blueprints/Interfaces/BPI_InteractionObject.TryInteract_BPI`
  (params (Release :type Boolean) (PlayerController :type "PlayerController Object Reference"))
  ;[1 1 1] Interactions.
  (if Release
    (message `/Game/EasySurvivalRPG/Blueprints/Interfaces/BPI_Player.OpenCraftingPlace_BPI` PlayerController (`self.CraftingComponent`) (`self.ContainerComponent`) false true)))

(fn `CheckCanInteract_BPI`
  (params (PlayerController :type "PlayerController Object Reference"))
  (returns (CanInteract :type Boolean))
  ;[1 1 1] Always allows interact with object.
  (return true))

(fn `GetInteractionObjectName_BPI`
  (returns (Name :type Text))
  ;[1 1 1] Returns interaction object name.
  (return (`.Name_48_0C2E1CB24B48846B5E49308F12848518` (break `/Game/EasySurvivalRPG/Blueprints/Structures/BuildingSystem/STR_BuildingObjectSettings` (`self.BuildingObjectSettings`)))))

(fn `GetInteractionText_BPI`
  (params (PlayerController :type "PlayerController Object Reference"))
  (returns (InteractionText :type Text))
  ;[1 1 1] Returns interaction text.
  (return (`.Name_48_0C2E1CB24B48846B5E49308F12848518` (break `/Game/EasySurvivalRPG/Blueprints/Structures/BuildingSystem/STR_BuildingObjectSettings` (`self.BuildingObjectSettings`)))))

(fn `IsTurnedOn_BPI`
  (returns (IsTurnedOn :type Boolean))
  ;[1 1 1] Is not used.
  (return false))

(fn `UserConstructionScript`
  (`parent.UserConstructionScript`))