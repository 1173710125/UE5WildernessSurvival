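; Remote-detonated trap building object that activates when a detonate call supplies a matching RemoteKey, recording the instigator.
; The key is set and read through interface functions and saved and restored as a formatted variable alongside parent data.
; When built, it creates item data from its Pickup handle, letting players take it back into inventory.
; It can attach to components, and replication of the attach target makes its mesh ignore Pawn and Camera collision.
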(event `self.ReceiveBeginPlay`
  (bind (_value _returnvalue) (`BlueprintMapLibrary.Map_Find` (`.Handles_72_197844E74CEF81DC828BECA6D464CF92` (break `/Game/EasySurvivalRPG/Blueprints/Structures/BuildingSystem/STR_BuildingObjectSettings` (`self.BuildingObjectSettings`))) "Pickup"))
  ;[1 1 1] Begin play. Init pickup item data.
  (`parent.ReceiveBeginPlay`)
  (if (`self.Built`)
    (if _returnvalue
      (set `self.ItemData` (`/Game/EasySurvivalRPG/Blueprints/Game/Libraries/BP_ItemsLibrary.MakeItemByHandle` _value)))))

(event `/Game/EasySurvivalRPG/Blueprints/Interfaces/BPI_InteractionObject.TryInteract_BPI`
  (params (Release :type Boolean) (PlayerController :type "PlayerController Object Reference"))
  (bind _itemdata (`self.ItemData`))
  ;[1 1 1] Interactions.
  (if Release
    (bind _inventorycontainer (message `/Game/EasySurvivalRPG/Blueprints/Interfaces/BPI_Player.GetInventoryContainer_BPI` PlayerController))
    (bind (_success _remainingitem) (`/Game/EasySurvivalRPG/Blueprints/Components/BP_ContainerComponent.TryAddItem` _inventorycontainer _itemdata))
    (if _success
      (`self.PlaySoundAtLocation (Multicast)` (`/Game/EasySurvivalRPG/Blueprints/Game/Libraries/BP_ItemsLibrary.GetItemSound` _itemdata "Take") (`self.K2_GetActorLocation`))
      (`self.K2_DestroyActor`)
      (else
        (set `self.ItemData` _remainingitem)))))

(fn `CheckAndAttachToComponent`
  (params (Component :type "SceneComponent Object Reference") (SocketName :type Name))
  (returns (Success :type Boolean))
  ;[1 1 1] Try to attach target component.
  (`/Engine/EditorBlueprintResources/StandardMacros.IsValid` Component
    (:`Is Valid`
      (`self.K2_AttachToComponent` Component SocketName "KeepWorld" "KeepWorld" "KeepWorld")
      (set `self.AttachTarget` (`ActorComponent.GetOwner` Component))
      (return true))))

(fn `CheckCanInteract_BPI`
  (params (PlayerController :type "PlayerController Object Reference"))
  (returns (CanInteract :type Boolean))
  ;[1 1 1] Returns true if player can interact with the actor.
  (return true))

(fn `GetFormattedVariables_BPI`
  (returns (FormattedVariables :type "Array of String"))
  ;[1 1 1] Save remote variables.
  (bind _formattedvariables (`parent.GetFormattedVariables_BPI`))
  (`KismetArrayLibrary.Array_Append` _formattedvariables (`|MakeArray` (`/Game/EasySurvivalRPG/Blueprints/Game/Libraries/BP_SaveLibrary.FormatStringVariableToString` "RemoteKey" (`self.RemoteKey`))))
  (return _formattedvariables))

(fn `GetInteractionObjectName_BPI`
  (returns (Name :type Text))
  ;[1 1 1] Returns interaction object name.
  (return (`/Game/EasySurvivalRPG/Blueprints/Game/Libraries/BP_ItemsLibrary.GetItemName` (`self.ItemData`))))

(fn `GetInteractionText_BPI`
  (params (PlayerController :type "PlayerController Object Reference"))
  (returns (InteractionText :type Text))
  ;[1 1 1] Returns interaction text.
  (return (`|FormatText` "Pick Up {ItemName}" (`/Game/EasySurvivalRPG/Blueprints/Game/Libraries/BP_ItemsLibrary.GetItemName` (`self.ItemData`)))))

(fn `GetRemoteKey_BPI`
  (returns (Success :type Boolean) (RemoteKey :type String))
  ;[1 1 1] Returns remote key of the actor.
  (return true (`self.RemoteKey`)))

(fn `LoadData_BPI`
  (params (SaveData :type "SaveGame Object Reference"))
  (returns (Success :type Boolean))
  ;[1 1 1] Load data for the actor.
  (bind _success (`parent.LoadData_BPI` SaveData))
  (if _success
    (bind (_success_2 _savedata) (message `/Game/EasySurvivalRPG/Blueprints/Interfaces/BPI_GameSave.GetActorSaveData_BPI` SaveData (`self.SaveID`)))
    (if _success_2
      (bind (_success_3 _value) (`/Game/EasySurvivalRPG/Blueprints/Game/Libraries/BP_SaveLibrary.GetFormattedVariableStringValue` (`.FormattedVariables_38_8140374D4327F2E43E03C3B17B80F74B` (break `/Game/EasySurvivalRPG/Blueprints/Structures/SaveData/STR_SaveData_Actor` _savedata)) "RemoteKey"))
      (if _success_3
        (set `self.RemoteKey` _value)
        (return true)
        (else
          _))))
  (return false))

(fn `OnRep_AttachTarget`
  (bind _staticmesh (`self.StaticMesh`))
  ;[1 1 1] Update mesh collision.
  (`PrimitiveComponent.SetCollisionResponseToChannel` _staticmesh "ECC_Pawn" "ECR_Ignore")
  (`PrimitiveComponent.SetCollisionResponseToChannel` _staticmesh "ECC_Camera" "ECR_Ignore"))

(fn `SetRemoteKey_BPI`
  (params (RemoteKey :type String))
  (returns (Success :type Boolean))
  ;[1 1 1] Set remote key for the actor.
  (set `self.RemoteKey` RemoteKey)
  (return true))

(fn `TryDetonate_BPI`
  (params (RemoteKey :type String) (Instigator :type "Pawn Object Reference"))
  (returns (Success :type Boolean))
  ;[1 1 1] Check remote key and detonate actor.
  (if (`KismetStringLibrary.EqualEqual_StrStr` RemoteKey (`self.RemoteKey`))
    (set `self.Instigator` Instigator)
    (`self.TryActivateTrap`)
    (return true)
    (else
      (return false))))

(fn `UserConstructionScript`
  (`parent.UserConstructionScript`))