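; Launch ability in EasySurvivalRPG that spawns and casts a fishing floater for the fishing rod item.
; SpawnProjectile extends the parent spawn and hands the new projectile to the instigator's BP_UsableItem_FishingRod through InitFloater, failing if no rod is found.
; LaunchProjectile aims it from its spawn point at a distant point along the controller's focus direction, applying any launch speed override reported by the instigator.
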(fn `LaunchProjectile`
  (returns (Success :type Boolean))
  (locals (LocalStartLocation :type "Vector Structure") (LocalProjectile :type "/Game/EasySurvivalRPG/Blueprints/InteractionObjects/Projectiles/Base/BP_Projectile_Base Object Reference") (LocalTargetRotation :type "Rotator Structure"))
  ;[1 1 1] Spawn and launch floater actor.
  (bind (_success _projectile) (`self.SpawnProjectile`))
  (if _success
    (set `local.LocalProjectile` _projectile)
    (set `local.LocalStartLocation` (`self.K2_GetActorLocation` _projectile))
    (bind (_location _rotation) (`/Game/EasySurvivalRPG/Blueprints/Game/Libraries/BP_GameLibrary.GetFocusVariables` (`self.GetInstigatorController`)))
    (set `local.LocalTargetRotation` (`KismetMathLibrary.FindLookAtRotation` (`local.LocalStartLocation`) (+ _location (* (`KismetMathLibrary.GetForwardVector` _rotation) 10000.0))))
    (bind (_isoverridden _overriddenspeed) (message `/Game/EasySurvivalRPG/Blueprints/Interfaces/BPI_Character.GetLaunchItemSpeed_BPI` (`self.GetInstigator`)))
    (`/Game/EasySurvivalRPG/Blueprints/InteractionObjects/Projectiles/Base/BP_Projectile_Base.LaunchProjectile` (`local.LocalProjectile`) (`KismetMathLibrary.GetForwardVector` (`local.LocalTargetRotation`)) _isoverridden _overriddenspeed)
    (return false)
    (else
      (return false))))

(fn `SpawnProjectile`
  (returns (Success :type Boolean) (Projectile :type "/Game/EasySurvivalRPG/Blueprints/InteractionObjects/Projectiles/Base/BP_Projectile_Base Object Reference"))
  ;[1 1 1] Spawn floated projectile and set references.
  (bind (_success _projectile) (`parent.SpawnProjectile`))
  (if _success
    (bind (_success_2 _usableitem) (message `/Game/EasySurvivalRPG/Blueprints/Interfaces/BPI_Character.GetUsableItem_BPI` (`self.GetInstigator`)))
    (if _success_2
      (bind _asbp_usable_item_fishing_rod (cast `/Game/EasySurvivalRPG/Blueprints/InteractionObjects/UsableItems/Presets/FishingRod/BP_UsableItem_FishingRod` _usableitem)
        (:`then`
          (`/Game/EasySurvivalRPG/Blueprints/InteractionObjects/UsableItems/Presets/FishingRod/BP_UsableItem_FishingRod.InitFloater` _asbp_usable_item_fishing_rod _projectile)
          (return true _projectile))
        (:`CastFailed`
          _))))
  (return false null))

(fn `UserConstructionScript`
  (`parent.UserConstructionScript`))