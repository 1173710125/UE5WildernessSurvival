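; Trace-based teleport ability that moves the instigator character to the traced hit location.
; Activation requires the parent condition checks to pass, then updates the trace variables and runs a trial trace that must register a hit.
; On a blocking hit, CheckHit places the instigator slightly above the impact using an unswept teleport, so obstacles along the way are ignored.
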(fn `CheckAbilityConditions`
  (returns (Success :type Boolean))
  ;[1 1 1] Check ability cost and trace hit.
  (bind _success (`parent.CheckAbilityConditions`))
  (if _success
    (`self.UpdateTraceVariables`)
    (bind (_hitresult _washit) (`self.TryHitTrace`))
    (return _washit)
    (else
      (return _success))))

(fn `CheckHit`
  (params (HitResult :type "HitResult Structure"))
  (returns (Success :type Boolean))
  (bind (_bblockinghit _binitialoverlap _time _distance _location) (`GameplayStatics.BreakHitResult` HitResult))
  ;[1 1 1] Check hit and teleport instigator character to hit location.
  (if _bblockinghit
    (`self.K2_SetActorLocation` (`self.GetInstigator`) (+ _location (0.0 0.0 50.0)) false true)
    (return false)))

(fn `UserConstructionScript`
  (`parent.UserConstructionScript`))