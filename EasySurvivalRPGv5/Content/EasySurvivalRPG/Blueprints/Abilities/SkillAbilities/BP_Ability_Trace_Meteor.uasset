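; Meteor shower skill ability that drops a volley of projectiles from the sky toward a traced hit location.
; A blocking hit sets a randomly offset spawn point high above it, aimed at the impact, and starts a looping timer to stagger launches.
; Each meteor gets its class from a data table row, random angular spread and any instigator speed override.
; The ability actor destroys itself once the count runs out.
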(fn `CheckAbilityConditions`
  (returns (Success :type Boolean))
  ;[1 1 1] Check ability cost and trace hit.
  (bind _success (`parent.CheckAbilityConditions`))
  (if _success
    (`self.UpdateTraceVariables`)
    (bind (_hitresult _washit) (`self.TryHitTrace`))
    (return _washit)
    (else
      (return _success))))

(fn `CheckHit`
  (params (HitResult :type "HitResult Structure"))
  (returns (Success :type Boolean))
  (locals (LocalHitLocation :type "Vector Structure") (LocalSpawnLocation :type "Vector Structure" :default (0.0 0.0 0.0)))
  (bind (_bblockinghit _binitialoverlap _time _distance _location) (`GameplayStatics.BreakHitResult` HitResult))
  (bind _meteorscount (`self.MeteorsCount`))
  ;[1 1 1] Check trace hit result and spawn projectile.
  (if _bblockinghit
    (bind _output_get (set `local.LocalHitLocation` _location))
    (bind _output_get_2 (set `local.LocalSpawnLocation` (+ _output_get (`KismetMathLibrary.MakeVector` (* (`KismetMathLibrary.RandomFloatInRange` 3000.0 5000.0) (`KismetMathLibrary.RandomFloatInRange` -1.0 1.0)) (* (`KismetMathLibrary.RandomFloatInRange` 3000.0 5000.0) (`KismetMathLibrary.RandomFloatInRange` -1.0 1.0)) 10000.0))))
    (set `self.SpawnLocation` _output_get_2)
    (set `self.SpawnRotation` (`KismetMathLibrary.FindLookAtRotation` (`local.LocalSpawnLocation`) _output_get))
    (set `self.CountRemaining` _meteorscount)
    (set `self.MeteorIndex` (/ _meteorscount 2))
    (`KismetSystemLibrary.K2_SetTimerDelegate` (`|CreateDelegate` :!event `LaunchMeteor`) 0.125 true)
    (return true)))

(fn `FindProjectileSettings`
  (returns (ProjectileClass :type "/Game/EasySurvivalRPG/Blueprints/InteractionObjects/Projectiles/Base/BP_Projectile_Base Class Reference") (ProjectileHandle :type "DataTableRowHandle Structure"))
  (bind (_value _returnvalue) (`BlueprintMapLibrary.Map_Find` (`.Handles_63_88DAB6504152B8CF608F39A3D2A5D080` (break `/Game/EasySurvivalRPG/Blueprints/Structures/AbilitySystem/STR_AbilityInstance` (`self.AbilitySettings`))) "Projectile"))
  (bind (_datatable _rowname) (break `DataTableRowHandle` _value))
  ;[1 1 1] Try to find projectile class and handle.
  (if _returnvalue
    (`/Engine/EditorBlueprintResources/StandardMacros.IsValid` _datatable
      (:`Is Valid`
        (bind _returnvalue_2 (`|GetDataTableRow` _datatable _rowname)
          (:`then`
            (bind ((`Handle_2_36E7D8A44585B051C187BEAF03821A24` _handle) (`ProjectileClass_5_6EED3A7E422F7A257075538A38385778` _projectileclass)) (break `/Game/EasySurvivalRPG/Blueprints/Structures/AbilitySystem/STR_ProjectileInstance` _returnvalue_2))
            (bind _output_get (set `self.ProjectileHandle` _handle))
            (bind _output_get_2 (set `self.ProjectileClass` _projectileclass)))
          (:`RowNotFound`
            _)))
      (:`Is Not Valid`
        _)))
  (return _output_get_2 _output_get))

(fn `LaunchMeteor`
  (bind _countremaining (`self.CountRemaining`))
  ;[1 1 1] Spawn meteor and launch it from the sky.
  (if (> _countremaining 0)
    (set `self.CountRemaining` (- _countremaining 1))
    (bind (_success _projectile) (`self.SpawnProjectile`))
    (if _success
      (bind (_isoverridden _overriddenspeed) (message `/Game/EasySurvivalRPG/Blueprints/Interfaces/BPI_Character.GetLaunchItemSpeed_BPI` (`self.GetInstigator`)))
      (`/Game/EasySurvivalRPG/Blueprints/InteractionObjects/Projectiles/Base/BP_Projectile_Base.LaunchProjectileForward` _projectile _isoverridden _overriddenspeed))
    (else
      (`self.K2_DestroyActor`))))

(fn `SpawnProjectile`
  (returns (Success :type Boolean) (Projectile :type "/Game/EasySurvivalRPG/Blueprints/InteractionObjects/Projectiles/Base/BP_Projectile_Base Object Reference"))
  ;[1 1 1] Spawn and launch projectile by specific class with target direction.
  (bind (_projectileclass _projectilehandle) (`self.FindProjectileSettings`))
  (bind _returnvalue (`|SpawnActorFromClass` _projectileclass (`KismetMathLibrary.MakeTransform` (`self.SpawnLocation`) (`KismetMathLibrary.ComposeRotators` (`self.SpawnRotation`) (`KismetMathLibrary.MakeRotator` 0.0 (`KismetMathLibrary.RandomFloatInRange` -5.0 5.0) (`KismetMathLibrary.RandomFloatInRange` -5.0 5.0))) (`self.ProjectileScale`)) "AlwaysSpawn" "OverrideRootScale" null _projectilehandle (`self.GetInstigator`)))
  (return true _returnvalue))

(fn `UserConstructionScript`
  (`parent.UserConstructionScript`))