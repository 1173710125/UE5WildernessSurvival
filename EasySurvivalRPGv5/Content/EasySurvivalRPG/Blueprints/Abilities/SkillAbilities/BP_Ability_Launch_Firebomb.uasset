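; Firebomb launch skill ability that throws one or more projectiles from the instigator toward where its controller is aiming.
; It starts at the weapon socket, or above the actor if that returns zero, and targets a long focus trace's hit or end point.
; The first projectile flies straight at the target and extras get random pitch and yaw spread.
; The instigator can override launch speed through interface messages.
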(fn `LaunchProjectile`
  (returns (Success :type Boolean))
  (locals (LocalStartLocation :type "Vector Structure") (LocalTraceHitLocation :type "Vector Structure") (LocalTargetRotation :type "Rotator Structure") (LocalOverrideSpeed :type Boolean :default false) (LocalOverriddenSpeed :type "Float (double-precision)" :default 0.0))
  (bind _returnvalue (`self.GetInstigator`))
  (bind _localstartlocation (`local.LocalStartLocation`))
  (bind _localtargetrotation (`local.LocalTargetRotation`))
  ;[1 1 1] Try to launch a few projectiles.
  (`/Engine/EditorBlueprintResources/StandardMacros.IsValid` _returnvalue
    (:`Is Valid`
      (bind _sockettransform (message `/Game/EasySurvivalRPG/Blueprints/Interfaces/BPI_Character.GetWeaponSocketTransform_BPI` _returnvalue (`self.WeaponStartSocketName`)))
      (bind _location (.location _sockettransform))
      (set `local.LocalStartLocation` (select `bool` (== _location (0.0 0.0 0.0)) :`false` _location :`true` (+ (`self.K2_GetActorLocation` _returnvalue) (0.0 0.0 100.0))))
      (bind (_location_2 _rotation) (`/Game/EasySurvivalRPG/Blueprints/Game/Libraries/BP_GameLibrary.GetFocusVariables` (`self.GetInstigatorController`)))
      (bind (_washit _hitlocation) (`self.GetTraceHitLocation` _location_2 _rotation 10000.0))
      (if _washit
        (bind _output_get (set `local.LocalTraceHitLocation` _hitlocation))
        (set `local.LocalTargetRotation` (`KismetMathLibrary.FindLookAtRotation` _localstartlocation _output_get))
        (else
          (set `local.LocalTargetRotation` (`KismetMathLibrary.FindLookAtRotation` _localstartlocation (+ _location_2 (* (`KismetMathLibrary.GetForwardVector` _rotation) 10000.0))))))
      (bind (_isoverridden _overriddenspeed) (message `/Game/EasySurvivalRPG/Blueprints/Interfaces/BPI_Character.GetLaunchItemSpeed_BPI` (`self.GetInstigator`)))
      (set `local.LocalOverrideSpeed` _isoverridden)
      (set `local.LocalOverriddenSpeed` _overriddenspeed)
      (for _index (range (`self.ProjectilesCount`))
        (bind (_success _projectile) (`self.SpawnProjectile`))
        (if _success
          (`/Game/EasySurvivalRPG/Blueprints/InteractionObjects/Projectiles/Base/BP_Projectile_Base.LaunchProjectile` _projectile (`KismetMathLibrary.GetForwardVector` (select `bool` (> _index 0) :`false` _localtargetrotation :`true` (`KismetMathLibrary.ComposeRotators` _localtargetrotation (`KismetMathLibrary.MakeRotator` 0.0 (`KismetMathLibrary.RandomFloatInRange` -5.0 5.0) (`KismetMathLibrary.RandomFloatInRange` -5.0 5.0))))) (`local.LocalOverrideSpeed`) (`local.LocalOverriddenSpeed`))))
      (return true))
    (:`Is Not Valid`
      (return false))))

(fn `UserConstructionScript`
  (`parent.UserConstructionScript`))