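; BP_Ability_AddBlueprint is an ability actor that adds a blueprint to a crafting list on the player's controller when used.
; On Use, it checks for a valid instigator and sends an AddBlueprintToList interface message to that instigator's controller.
; The list and blueprint come from the AbilitySettings handle map, falling back to TargetBlueprintList and TargetBlueprint when absent.
; The actor then destroys itself, even without a valid instigator.
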(event `self.Use`
  (bind _returnvalue (`self.GetInstigator`))
  (bind ((`AbilityClass_85_CD109F3E44C8D93EE112DFA782147A8A` _abilityclass) (`Handles_63_88DAB6504152B8CF608F39A3D2A5D080` _handles)) (break `/Game/EasySurvivalRPG/Blueprints/Structures/AbilitySystem/STR_AbilityInstance` (`self.AbilitySettings`)))
  (bind (_value _returnvalue_2) (`BlueprintMapLibrary.Map_Find` _handles "CraftingList"))
  (bind (_value_2 _returnvalue_3) (`BlueprintMapLibrary.Map_Find` _handles "Blueprint"))
  ;[1 1 1] Execute for use ability. Adds blueprint to the crafting list for player controller.
  (`/Engine/EditorBlueprintResources/StandardMacros.IsValid` _returnvalue
    (:`Is Valid`
      (message `/Game/EasySurvivalRPG/Blueprints/Interfaces/BPI_Player.AddBlueprintToList_BPI` (`Pawn.GetController` _returnvalue) (select `bool` _returnvalue_2 :`false` (`self.TargetBlueprintList`) :`true` _value) (select `bool` _returnvalue_3 :`false` (`self.TargetBlueprint`) :`true` _value_2)))
    (:`Is Not Valid`
      _))
  (`self.K2_DestroyActor`))

(fn `UserConstructionScript`
  (`parent.UserConstructionScript`))