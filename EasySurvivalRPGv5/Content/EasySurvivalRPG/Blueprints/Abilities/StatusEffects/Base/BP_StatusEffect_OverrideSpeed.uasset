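; Base status effect actor in EasySurvivalRPG that overrides its owner's walk speed for as long as it exists.
; On BeginPlay it sends an OverrideWalkSpeed interface message to the owner with the configured speed and interpolation speed.
; On Destroyed it sends the same message with the override disabled, resetting the owner's walk speed.
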(event `self.ReceiveBeginPlay`
  ;[1 1 1] Begin play. Override walk speed on begin play.
  (`parent.ReceiveBeginPlay`)
  (message `/Game/EasySurvivalRPG/Blueprints/Interfaces/BPI_Character.OverrideWalkSpeed_BPI` (`self.GetOwner`) true (`self.OverridedWalkSpeed`) (`self.OverriddedWalkInterpSpeed`)))

(event `self.ReceiveDestroyed`
  ;[1 1 1] Reset walk speed.
  (`parent.ReceiveDestroyed`)
  (message `/Game/EasySurvivalRPG/Blueprints/Interfaces/BPI_Character.OverrideWalkSpeed_BPI` (`self.GetOwner`) false 0.0 0.0))

(fn `UserConstructionScript`
  (`parent.UserConstructionScript`))