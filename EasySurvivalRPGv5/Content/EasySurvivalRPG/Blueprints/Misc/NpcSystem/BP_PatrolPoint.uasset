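; BP_PatrolPoint is an NPC system patrol point actor whose graphs contain only save/load plumbing, with no patrol logic.
; It saves its class, transform and formatted variables (none filled in here) under a settable Save ID through save-data interface calls.
; Loading only forwards the save data to components implementing BPI_SaveData, without applying actor state itself.
; It opts into save/load and exposes no component save ID.
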(fn `DoesIgnoreSaveLoad_BPI`
  (returns (Result :type Boolean))
  (return false))

(fn `GetComponentSaveID_BPI`
  (returns (Success :type Boolean) (ComponentSaveID :type Integer))
  (return false 0))

(fn `GetFormattedVariables_BPI`
  (returns (FormattedVariables :type "Array of String"))
  (return))

(fn `GetSaveID_BPI`
  (returns (Success :type Boolean) (SaveID :type Integer))
  ;[1 1 1] Returns the Save ID variable value.
  (return true (`self.SaveID`)))

(fn `LoadData_BPI`
  (params (SaveData :type "SaveGame Object Reference"))
  (returns (Success :type Boolean))
  (locals (LocalSaveData :type "SaveGame Object Reference"))
  ;[1 1 1] Load common actor data.
  (set `local.LocalSaveData` SaveData)
  (for _array_element (`self.K2_GetComponentsByClass` "/Script/Engine.ActorComponent")
    (if (`KismetSystemLibrary.DoesImplementInterface` _array_element "/Game/EasySurvivalRPG/Blueprints/Interfaces/BPI_SaveData.BPI_SaveData_C")
      (message `/Game/EasySurvivalRPG/Blueprints/Interfaces/BPI_SaveData.LoadData_BPI` _array_element (`local.LocalSaveData`))))
  (return true))

(fn `SaveData_BPI`
  (params (SaveData :type "SaveGame Object Reference"))
  (returns (Success :type Boolean))
  (locals (LocalSaveData :type "SaveGame Object Reference"))
  ;[1 1 1] Save common actor data.
  (bind _formattedvariables (`/Game/EasySurvivalRPG/Blueprints/Interfaces/BPI_SaveData.GetFormattedVariables_BPI`))
  (bind _output_get (set `local.LocalSaveData` SaveData))
  (bind _success (message `/Game/EasySurvivalRPG/Blueprints/Interfaces/BPI_GameSave.SetActorSaveData_BPI` _output_get (`self.SaveID`) (make `/Game/EasySurvivalRPG/Blueprints/Structures/SaveData/STR_SaveData_Actor` (`GameplayStatics.GetObjectClass` self) (`self.GetTransform`) _formattedvariables)))
  (return _success))

(fn `SetSaveID_BPI`
  (params (SaveID :type Integer))
  (returns (Success :type Boolean))
  ;[1 1 1] Sets the Save ID variable value.
  (set `self.SaveID` SaveID)
  (return true))

(fn `UserConstructionScript`)