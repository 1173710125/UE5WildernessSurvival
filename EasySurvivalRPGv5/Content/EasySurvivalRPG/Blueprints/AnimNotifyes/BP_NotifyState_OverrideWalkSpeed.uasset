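; Anim notify state that temporarily overrides the walk speed of the animated mesh's owner during a montage or animation window.
; On begin it sends a Blueprint interface message to the owner with the configured target speed and interpolation speed.
; On end it sends the same message to clear the override.
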(fn `GetNotifyName`
  (returns (ReturnValue :type String))
  (return "Override Walk Speed"))

(fn `Received_NotifyBegin`
  (params (MeshComp :type "SkeletalMeshComponent Object Reference") (Animation :type "AnimSequenceBase Object Reference") (TotalDuration :type "Float (double-precision)"))
  (returns (ReturnValue :type Boolean))
  ;[1 1 1] Begin override walking speed.
  (message `/Game/EasySurvivalRPG/Blueprints/Interfaces/BPI_Character.OverrideWalkSpeed_BPI` (`ActorComponent.GetOwner` MeshComp) true (`self.OverridedWalkSpeed`) (`self.OverridedInterpWalkSpeed`))
  (return false))

(fn `Received_NotifyEnd`
  (params (MeshComp :type "SkeletalMeshComponent Object Reference") (Animation :type "AnimSequenceBase Object Reference"))
  (returns (ReturnValue :type Boolean))
  ;[1 1 1] Clear overrided walking speed.
  (message `/Game/EasySurvivalRPG/Blueprints/Interfaces/BPI_Character.OverrideWalkSpeed_BPI` (`ActorComponent.GetOwner` MeshComp) false 0.0 0.0)
  (return false))