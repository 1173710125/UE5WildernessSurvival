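; Indoor bed interactable that plays a sleep sequence when the player interacts while the direction check passes and no sequence is running.
; It locks movement and input, shows a sleepy line in the character dialogue widget, and fades the camera dark by lerping a post-process color vector on a timeline.
; After a delay, a reversed timeline restores the view as movement, Animation Blueprint mode and input return, with a brief refreshed message.
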(event `/Game/my_game/Blueprints/jiekou/交互临时.物件交互`
  (bind _as_my_character (`self.As My Character`))
  (bind _camera (`/Game/my_game/Blueprints/My_Character_shengchun.Camera` _as_my_character))
  (if (`self.是否同向`)
    (if (not (`self.是否正在做`))
      (`CharacterMovementComponent.DisableMovement` (`Character.CharacterMovement` (`GameplayStatics.GetPlayerCharacter` 0)))
      (`self.DisableInput` _as_my_character (`GameplayStatics.GetPlayerController` 0))
      (bind _asjuese_yuyan (cast `/Game/my_game/UI/角色_speak/juese_yuyan` (`WidgetComponent.GetWidget` (`/Game/my_game/Blueprints/My_Character_shengchun.my_Widget` _as_my_character))))
      (set `/Game/my_game/UI/角色_speak/juese_yuyan.角色文字` "太困了，我需要睡眠" _asjuese_yuyan)
      (`|ExecutionSequence`
        (:`then_0`
          (set `self.是否正在做` true)
          (`KismetSystemLibrary.Delay` 3.0)
          (`|ExecutionSequence`
            (:`then_0`
              (bind (_direction `_新建轨道_0`) (`Timeline|时间轴_0` :!via `ReverseFromEnd`)
                (:`Update`
                  (bind _returnvalue (`KismetMathLibrary.Lerp` 1.0 0.0 `_新建轨道_0`))
                  (set `CameraComponent.PostProcessSettings` (make `PostProcessSettings` :`ColorGamma` (`KismetMathLibrary.MakeVector4` _returnvalue _returnvalue _returnvalue 1.0)) _camera))))
            (:`then_1`
              (`CharacterMovementComponent.SetMovementMode` (`Character.CharacterMovement` (`GameplayStatics.GetPlayerCharacter` 0)) "MOVE_Walking" 0)
              (`SkeletalMeshComponent.SetAnimationMode` (`Character.Mesh` _as_my_character) "AnimationBlueprint" true)
              (`self.EnableInput` (`self.As My Character`) (`GameplayStatics.GetPlayerController` 0))
              (set `/Game/my_game/UI/角色_speak/juese_yuyan.角色文字` "又是精神充足的一天" _asjuese_yuyan)
              (`KismetSystemLibrary.Delay` 2.0)
              (set `/Game/my_game/UI/角色_speak/juese_yuyan.角色文字` "" _asjuese_yuyan)
              (set `self.是否正在做` false))))
        (:`then_1`
          (bind (_direction_2 `_新建轨道_0_2`) (`Timeline|时间轴` :!via `PlayFromStart`)
            (:`Update`
              (bind _returnvalue_2 (`KismetMathLibrary.Lerp` 1.0 0.0 `_新建轨道_0_2`))
              (set `CameraComponent.PostProcessSettings` (make `PostProcessSettings` :`ColorGamma` (`KismetMathLibrary.MakeVector4` _returnvalue_2 _returnvalue_2 _returnvalue_2 1.0)) _camera))))))))

(fn `UserConstructionScript`
  (`parent.UserConstructionScript`))