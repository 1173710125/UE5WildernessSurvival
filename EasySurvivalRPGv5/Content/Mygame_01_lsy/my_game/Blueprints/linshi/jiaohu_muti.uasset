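; Base interactable Blueprint (jiaohu_muti) that tracks whether the shengchun player character is in range and correctly facing the object.
; Box overlap events toggle the in-range flag, and while it is set, Tick runs a facing check between the Box and the cached character to update the same-direction flag.
; A separate interaction animation event briefly raises the interaction flag on the character's AnimBP, clearing it after a short delay.
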(event `CustomEvent`)

(event `self.ReceiveBeginPlay`
  (bind _asmy_character (cast `/Game/my_game/Blueprints/My_Character_shengchun` (`GameplayStatics.GetPlayerCharacter` 0)))
  (set `self.As My Character` _asmy_character))

(event `self.ReceiveTick`
  (params (DeltaSeconds :type "Float (single-precision)"))
  ;[1 1 1] 交互事件
  (if (`self.是否在交互范围`)
    (bind `_是否同向` (`/Game/my_game/Blueprints/hanshuku/my_hanshuku.角色与物体朝向交互判断` (`self.Box`) (`self.As My Character`)))
    (set `self.是否同向` `_是否同向`)))

(event `self.Box.OnComponentBeginOverlap`
  (params (OverlappedComponent :type "PrimitiveComponent Object Reference") (OtherActor :type "Actor Object Reference") (OtherComp :type "PrimitiveComponent Object Reference") (OtherBodyIndex :type Integer) (bFromSweep :type Boolean) (SweepResult :type "HitResult Structure (by ref)"))
  ;[1 1 1] 交互事件
  (cast `/Game/my_game/Blueprints/My_Character_shengchun` OtherActor)
  (set `self.是否在交互范围` true))

(event `self.Box.OnComponentEndOverlap`
  (params (OverlappedComponent :type "PrimitiveComponent Object Reference") (OtherActor :type "Actor Object Reference") (OtherComp :type "PrimitiveComponent Object Reference") (OtherBodyIndex :type Integer))
  ;[1 1 1] 交互事件
  (cast `/Game/my_game/Blueprints/My_Character_shengchun` OtherActor)
  (set `self.是否在交互范围` false))

(event `交互动画`
  (bind _as_my_ani_02 (`/Game/my_game/Blueprints/My_Character_shengchun.As My Ani 02` (`self.As My Character`)))
  (set `/Game/my_game/ani/100501_unit_Skeleton_AnimBlueprint.是否播放交互动画` true _as_my_ani_02)
  (`KismetSystemLibrary.Delay` 0.6)
  (set `/Game/my_game/ani/100501_unit_Skeleton_AnimBlueprint.是否播放交互动画` false _as_my_ani_02))

(fn `UserConstructionScript`)