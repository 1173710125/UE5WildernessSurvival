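; Interactable book actor that runs a timed interaction when its 物件交互 (object interaction) event fires and the 是否同向 (same direction) flag is true.
; It calls 交互动画 (interaction animation), then, unless one is already in progress, shows a Chushi widget and disables player movement.
; After a short delay it collapses the widget, restores walking, returns the character mesh to Animation Blueprint mode and clears the busy flag.
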(event `/Game/my_game/Blueprints/jiekou/交互临时.物件交互`
  (if (`self.是否同向`)
    (`self.交互动画`)
    (if (not (`self.是否正在做`))
      (bind _returnvalue (`|CreateWidget` "/Game/my_game/UI/chushi.chushi_C"))
      (`UserWidget.AddToViewport` _returnvalue 0)
      (`Widget.SetVisibility` _returnvalue "Visible")
      (`CharacterMovementComponent.DisableMovement` (`Character.CharacterMovement` (`GameplayStatics.GetPlayerCharacter` 0)))
      (set `self.是否正在做` true)
      (`KismetSystemLibrary.Delay` 2.0)
      (`Widget.SetVisibility` _returnvalue "Collapsed")
      (`CharacterMovementComponent.SetMovementMode` (`Character.CharacterMovement` (`GameplayStatics.GetPlayerCharacter` 0)) "MOVE_Walking" 0)
      (`SkeletalMeshComponent.SetAnimationMode` (`Character.Mesh` (`self.As My Character`)) "AnimationBlueprint" true)
      (set `self.是否正在做` false))))

(fn `UserConstructionScript`
  (`parent.UserConstructionScript`))