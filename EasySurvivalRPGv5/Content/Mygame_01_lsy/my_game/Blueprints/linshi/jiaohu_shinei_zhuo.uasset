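; Indoor table interactable that lets the player character eat when its interaction event fires and the same-direction check (是否同向) passes.
; It calls 交互动画, then, unless already busy, disables movement and plays a one-shot eat animation on the character mesh.
; After timed delays it restores walking and the Animation Blueprint, briefly shows an "I'm full" line in the character's juese_yuyan widget, then clears the busy flag.
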(event `/Game/my_game/Blueprints/jiekou/交互临时.物件交互`
  (bind _as_my_character (`self.As My Character`))
  (bind _mesh (`Character.Mesh` _as_my_character))
  (if (`self.是否同向`)
    (`self.交互动画`)
    (if (not (`self.是否正在做`))
      (`CharacterMovementComponent.DisableMovement` (`Character.CharacterMovement` (`GameplayStatics.GetPlayerCharacter` 0)))
      (`SkeletalMeshComponent.PlayAnimation` _mesh "/Game/my_game/ani/1001/my_01_A_Jess_Eat.my_01_A_Jess_Eat" false)
      (set `self.是否正在做` true)
      (`KismetSystemLibrary.Delay` 2.5)
      (`CharacterMovementComponent.SetMovementMode` (`Character.CharacterMovement` (`GameplayStatics.GetPlayerCharacter` 0)) "MOVE_Walking" 0)
      (`SkeletalMeshComponent.SetAnimationMode` _mesh "AnimationBlueprint" true)
      (bind _asjuese_yuyan (cast `/Game/my_game/UI/角色_speak/juese_yuyan` (`WidgetComponent.GetWidget` (`/Game/my_game/Blueprints/My_Character_shengchun.my_Widget` _as_my_character))))
      (set `/Game/my_game/UI/角色_speak/juese_yuyan.角色文字` "吃饱了啦" _asjuese_yuyan)
      (`KismetSystemLibrary.Delay` 1.5)
      (set `/Game/my_game/UI/角色_speak/juese_yuyan.角色文字` "" _asjuese_yuyan)
      (set `self.是否正在做` false))))

(fn `UserConstructionScript`
  (`parent.UserConstructionScript`))