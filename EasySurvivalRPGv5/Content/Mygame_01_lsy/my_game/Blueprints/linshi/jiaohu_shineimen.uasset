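; Interactable door that swings open and loads the "jiayuan_inside" level.
; The interaction event (物件交互) checks a same-direction flag, plays the interaction animation, then flip-flops a timeline forward or in reverse.
; Each timeline update rotates the mesh's yaw up to 90 degrees and feeds a short delay before the level load, so closing also reaches that load.
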(event `/Game/my_game/Blueprints/jiekou/交互临时.物件交互`
  (if (`self.是否同向`)
    (`self.交互动画`)
    (`/Engine/EditorBlueprintResources/StandardMacros.FlipFlop`
      (:`A`
        (bind (_direction `_门动画插值`) (`Timeline|时间轴` :!label _label)
          (:`Update`
            (`SceneComponent.K2_SetRelativeTransform` (`self.StaticMesh`) (`KismetMathLibrary.MakeTransform` (0.0 0.0 0.0) (`KismetMathLibrary.MakeRotator` 0.0 0.0 (`KismetMathLibrary.Lerp` 0.0 90.0 `_门动画插值`))) false false)
            (`KismetSystemLibrary.Delay` 0.8)
            (`GameplayStatics.OpenLevel` "jiayuan_inside"))))
      (:`B`
        (goto _label :!via `Reverse`)))))

(fn `UserConstructionScript`
  (`parent.UserConstructionScript`))