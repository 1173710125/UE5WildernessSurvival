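; Indoor warehouse interactable that opens a storage box UI (Xiangzi01) for the player.
; Interaction passes a same-direction check, plays an animation, then enters a FlipFlop that the widget's close button also triggers through a custom event.
; Opening creates a fresh widget, shows the cursor and locks movement and look.
; Closing collapses it and restores game-only input, walking and look.
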(event `自定义事件`
  (bind _returnvalue (`GameplayStatics.GetPlayerController` 0))
  (bind _returnvalue_2 (`GameplayStatics.GetPlayerController` 0))
  (bind `_箱子ui` (`self.箱子UI`))
  (`/Engine/EditorBlueprintResources/StandardMacros.FlipFlop` :!label _label
    (:`A`
      (`|ExecutionSequence`
        (:`then_0`
          (bind _returnvalue_3 (`|CreateWidget` "/Game/my_game/UI/jiayuan_nei/xiangzi01.xiangzi01_C" (`GameplayStatics.GetPlayerController` 0)))
          (bind _output_get (set `self.箱子UI` _returnvalue_3))
          (`UserWidget.AddToViewport` _output_get 0)
          (add `Button.OnClicked` (`/Game/my_game/UI/jiayuan_nei/xiangzi01.关闭按钮` (`self.箱子UI`)) (delegate `自定义事件`)))
        (:`then_1`
          (`WidgetBlueprintLibrary.SetInputMode_GameAndUIEx` (`GameplayStatics.GetPlayerController` 0) `_箱子ui`)
          (set `PlayerController.bShowMouseCursor` true _returnvalue_2)
          (`CharacterMovementComponent.DisableMovement` (`Character.CharacterMovement` (`GameplayStatics.GetPlayerCharacter` 0)))
          (`Controller.SetIgnoreLookInput` _returnvalue_2 true)
          (`Widget.SetVisibility` `_箱子ui` "Visible"))))
    (:`B`
      (`WidgetBlueprintLibrary.SetInputMode_GameOnly` _returnvalue)
      (set `PlayerController.bShowMouseCursor` false _returnvalue)
      (`CharacterMovementComponent.SetMovementMode` (`Character.CharacterMovement` (`GameplayStatics.GetPlayerCharacter` 0)) "MOVE_Walking" 0)
      (`Controller.ResetIgnoreLookInput` _returnvalue)
      (`Widget.SetVisibility` (`self.箱子UI`) "Collapsed"))))

(event `/Game/my_game/Blueprints/jiekou/交互临时.物件交互`
  (if (`self.是否同向`)
    (`self.交互动画`)
    (goto _label)))

(fn `UserConstructionScript`
  (`parent.UserConstructionScript`))