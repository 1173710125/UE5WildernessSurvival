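; Blueprint Interface for the in-game HUD of a survival/RPG-style game, declaring calls that drive the UI without exposing its implementation.
; It covers opening and closing screens such as inventory, crafting, trade, building, map, journal, dialogue, chat and pause, plus boolean open-state queries.
; Update calls push container, hotbar, quest, skill, status effect and character data, alongside combat reaction triggers.
; All functions are signatures only, including a parameterless my_jiaohu hook.
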(fn `AddChatMessage_BPI`
  (params (Message :type "/Game/EasySurvivalRPG/Blueprints/Structures/Misc/STR_ChatMessage Structure")))

(fn `AddEventMessage_BPI`
  (params (Text :type "Object Object Reference" :default "NSLOCTEXT(\"[323AA8D24E913BA0A3527B9E3E6839D7]\", \"B92B65164E2E6D26ED0F38846562AF5A\", \"Message\")") (TextColor :type "LinearColor Structure" :default (struct :`R` 1.0 :`G` 1.0 :`B` 1.0 :`A` 1.0))))

(fn `AddStatusEffect_BPI`
  (params (StatusEffectData :type "/Game/EasySurvivalRPG/Blueprints/Structures/AbilitySystem/STR_StatusEffectData Structure")))

(fn `BlockHotbarSlot_BPI`
  (params (Block :type Boolean) (HotbarSlot :type Integer)))

(fn `CloseBuildingMenu_BPI`)

(fn `CloseChat_BPI`)

(fn `CloseDialogue_BPI`)

(fn `CloseHUD_BPI`)

(fn `CloseMalletMenu_BPI`)

(fn `ClosePauseMenu_BPI`)

(fn `CloseSubMenu_BPI`)

(fn `CreateDeathMenu_BPI`)

(fn `CreateHUD_BPI2`)

(fn `DialogueIsOpen_BPI`
  (returns (IsOpen :type Boolean))
  (return false))

(fn `HUDIsOpen_BPI`
  (returns (IsOpen :type Boolean))
  (return false))

(fn `InitPlayerContainers_BPI`
  (params (InventoryContainer :type "/Game/EasySurvivalRPG/Blueprints/Components/BP_ContainerComponent Object Reference") (HotbarContainer :type "/Game/EasySurvivalRPG/Blueprints/Components/BP_HotbarComponent Object Reference") (EquipmentContainer :type "/Game/EasySurvivalRPG/Blueprints/Components/BP_EquipmentComponent Object Reference")))

(fn `InventoryIsOpen_BPI`
  (returns (IsOpen :type Boolean))
  (return false))

(fn `JournalIsOpen_BPI`
  (returns (IsOpen :type Boolean))
  (return false))

(fn `MapIsOpen_BPI`
  (returns (IsOpen :type Boolean))
  (return false))

(fn `my_jiaohu`)

(fn `OnItemPicked_BPI`
  (params (Item :type "/Game/EasySurvivalRPG/Blueprints/Structures/Items/STR_Item Structure")))

(fn `OpenBuildingMenu_BPI`
  (params (BuildingObject :type "/Game/EasySurvivalRPG/Blueprints/InteractionObjects/BuildingObjects/Base/BP_Building_BaseObject Object Reference")))

(fn `OpenChat_BPI`)

(fn `OpenCodelock_BPI`
  (params (IsLocked :type Boolean) (IsAuthorized :type Boolean) (Password :type String)))

(fn `OpenContainer_BPI`
  (params (ContainerComponent :type "/Game/EasySurvivalRPG/Blueprints/Components/BP_ContainerComponent Object Reference")))

(fn `OpenCrafting_BPI`
  (params (OnlyCraftingQueue :type Boolean) (DisableManualCrafting :type Boolean)))

(fn `OpenDialogue_BPI`)

(fn `OpenHUD_BPI`)

(fn `OpenInteractionSwitcher_BPI`
  (params (InteractionObject :type "Actor Object Reference")))

(fn `OpenInventory_BPI`)

(fn `OpenJournal_BPI`)

(fn `OpenMalletMenu_BPI`
  (params (BuildingObject :type "/Game/EasySurvivalRPG/Blueprints/InteractionObjects/BuildingObjects/Base/BP_Building_BaseObject Object Reference")))

(fn `OpenMap_BPI`)

(fn `OpenPauseMenu_BPI`)

(fn `OpenSubMenu_BPI`)

(fn `OpenTrade_BPI`)

(fn `PlayBlockReaction_BPI`)

(fn `PlayDamageReaction_BPI`)

(fn `PlayHitReaction_BPI`)

(fn `QuickSelectDialogueReply_BPI`
  (params (ReplyIndex :type Integer)))

(fn `RemoveHUD_BPI`)

(fn `RemoveStatusEffect_BPI`
  (params (StatusEffectHandle :type "DataTableRowHandle Structure")))

(fn `ResizeContainer_BPI`
  (params (Container :type "/Game/EasySurvivalRPG/Blueprints/Components/BP_ContainerComponent Object Reference") (NewSlots :type Integer)))

(fn `SetMapEnabled_BPI`
  (params (MapEnabled :type Boolean)))

(fn `SetMinimapEnabled_BPI`
  (params (MinimapEnabled :type Boolean)))

(fn `SetShowBuildingDurability_BPI`
  (params (ShowBuildingDurability :type Boolean)))

(fn `SetShowCharacterState_BPI`
  (params (ShowCharacterState :type Boolean)))

(fn `SetShowMinimap_BPI`
  (params (ShowMinimap :type Boolean)))

(fn `SubMenuIsOpen_BPI`
  (returns (IsOpen :type Boolean))
  (return false))

(fn `UpdateActiveQuestNote_BPI`
  (params (QuestNote :type "/Game/EasySurvivalRPG/Blueprints/Structures/DialogueSystem/STR_JournalNote Structure")))

(fn `UpdateBlueprintList_BPI`
  (params (Blueprints :type "Array of DataTableRowHandle Structure")))

(fn `UpdateCharacterInfo_BPI`
  (params (CharacterInfo :type "/Game/EasySurvivalRPG/Blueprints/Structures/Misc/STR_CharacterInfo Structure")))

(fn `UpdateCharacterSkill_BPI`
  (params (Skill :type "/Game/EasySurvivalRPG/Blueprints/Structures/AbilitySystem/STR_Skill Structure")))

(fn `UpdateCharacterSkills_BPI`
  (params (Skills :type "Array of /Game/EasySurvivalRPG/Blueprints/Structures/AbilitySystem/STR_Skill Structure")))

(fn `UpdateChatMessages_BPI`
  (params (ChatMessages :type "Array of /Game/EasySurvivalRPG/Blueprints/Structures/Misc/STR_ChatMessage Structure")))

(fn `UpdateContainerResource_BPI`
  (params (Container :type "/Game/EasySurvivalRPG/Blueprints/Components/BP_ContainerComponent Object Reference") (Resource :type "/Game/EasySurvivalRPG/Blueprints/Structures/Items/STR_ResourceValue Structure")))

(fn `UpdateContainerSlot_BPI`
  (params (Container :type "/Game/EasySurvivalRPG/Blueprints/Components/BP_ContainerComponent Object Reference") (Slot :type Integer) (ItemTransfer :type "/Game/EasySurvivalRPG/Blueprints/Structures/Items/STR_ItemTransferData Structure")))

(fn `UpdateCraftingQueue_BPI`
  (params (QueueBlueprints :type "Array of /Game/EasySurvivalRPG/Blueprints/Structures/Items/STR_QueueBlueprint Structure")))

(fn `UpdateCraftingQueueBlueprint_BPI`
  (params (Index :type Integer) (QueueBlueprint :type "/Game/EasySurvivalRPG/Blueprints/Structures/Items/STR_QueueBlueprint Structure")))

(fn `UpdateDialogue_BPI`
  (params (SpeakerName :type Text) (SpeakerText :type Text) (SpeakerIcon :type "Texture2D Object Reference") (PlayerReplies :type "Array of /Game/EasySurvivalRPG/Blueprints/Structures/DialogueSystem/STR_DialogueReply Structure")))

(fn `UpdateJournalNotes_BPI`
  (params (JournalNotes :type "Array of /Game/EasySurvivalRPG/Blueprints/Structures/DialogueSystem/STR_JournalNote Structure")))

(fn `UpdateSelectedHotbarSlot_BPI`
  (params (HotbarSlot :type Integer)))

(fn `UpdateSelectedItem_BPI`
  (params (ItemTransfer :type "/Game/EasySurvivalRPG/Blueprints/Structures/Items/STR_ItemTransferData Structure")))

(fn `UpdateSelectedTradingItem_BPI`
  (params (ItemHandle :type "DataTableRowHandle Structure")))

(fn `UpdateStatusEffect_BPI`
  (params (StatusEffectData :type "/Game/EasySurvivalRPG/Blueprints/Structures/AbilitySystem/STR_StatusEffectData Structure")))

(fn `UpdateTargetActor_BPI`
  (params (TargetActor :type "Actor Object Reference")))

(fn `UpdateTradeList_BPI`
  (params (TradeItems :type "Array of /Game/EasySurvivalRPG/Blueprints/Structures/Items/STR_Item Structure") (TradeList :type "/Game/EasySurvivalRPG/Blueprints/Structures/Items/STR_TradeList Structure")))

(fn `UpdateWeight_BPI`
  (params (Weight :type "Float (double-precision)") (MaxWeight :type "Float (double-precision)") (OverloadFactor :type "Float (double-precision)")))