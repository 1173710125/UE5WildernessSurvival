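; Base harvestable tree actor that stands in for a foliage instance, removing it on BeginPlay via the foliage manager.
; Damage lowers durability, spawning hit effects and loot, then switches to a cut mesh with wood and apple drops before full destruction by damage or digging.
; Timers handle respawn and server-side return of instance-spawned trees to foliage, with a sphere trace for nearby buildings.
; Save interface functions persist durability, destruction state and respawn time.
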(event `self.ReceiveAnyDamage`
  (params (Damage :type "Float (single-precision)") (DamageType :type "DamageType Object Reference") (InstigatedBy :type "Controller Object Reference") (DamageCauser :type "Actor Object Reference"))
  ;[1 1 1] 互动。当树木受损时。
  (bind _damagedata (`/Game/EasySurvivalRPG/Blueprints/Game/Libraries/BP_DamageSystemLibrary.MakeObjectDamageData` Damage DamageType))
  (`self.建筑物受损时的行动` _damagedata InstigatedBy DamageCauser))

(event `self.ReceivePointDamage`
  (params (Damage :type "Float (single-precision)") (DamageType :type "DamageType Object Reference") (HitLocation :type "Vector Structure") (HitNormal :type "Vector Structure") (HitComponent :type "PrimitiveComponent Object Reference") (BoneName :type Name) (ShotFromDirection :type "Vector Structure") (InstigatedBy :type "Controller Object Reference") (DamageCauser :type "Actor Object Reference") (HitInfo :type "HitResult Structure (by ref)"))
  ;[1 1 1] 互动。当树木受损时。
  (bind _damagedata (`/Game/EasySurvivalRPG/Blueprints/Game/Libraries/BP_DamageSystemLibrary.MakeObjectDamageData` Damage DamageType))
  (`self.建筑物受损时的行动` _damagedata InstigatedBy DamageCauser HitInfo))

(event `self.ReceiveBeginPlay`
  ;[1 1 1] 开始游戏。尝试删除树实例。
  (`parent.ReceiveBeginPlay`)
  (`self.从适当的实例化组件中删除树实例`)
  (`self.启动返回树定时器`))

(event `/Game/EasySurvivalRPG/Blueprints/Interfaces/BPI_DamageSystemActor.ApplyPointDamage_BPI`
  (params (DamageData :type "/Game/EasySurvivalRPG/Blueprints/Structures/DamageSystem/STR_DamageData Structure") (HitFromDirection :type "Vector Structure") (HitInfo :type "HitResult Structure") (EventInstigator :type "Controller Object Reference") (DamageCauser :type "Actor Object Reference"))
  ;[1 1 1] 互动。当树木受损时。
  (`self.建筑物受损时的行动` DamageData EventInstigator DamageCauser HitInfo))

(event `/Game/EasySurvivalRPG/Blueprints/Interfaces/BPI_DiggingActor.TryToDig_BPI`
  (params (Instigator :type "Controller Object Reference") (Value :type "Float (double-precision)"))
  ;[1 1 1] 互动。当树木受损时。
  (if (`self.是否正在破环`)
    (`self.完全摧毁树并将演员从游戏中删除` Instigator)))

(event `启动返回树定时器`
  ;[1 1 1] 将树返回到实例。
  (`/Engine/EditorBlueprintResources/ActorMacros.Switch Has Authority`
    (:`Authority`
      (`KismetSystemLibrary.K2_SetTimerDelegate` (`|CreateDelegate` :!event `返回树到实例`) 60.0))))

(event `返回树到实例`
  ;[1 1 1] 将树返回到实例。
  (`/Engine/EditorBlueprintResources/ActorMacros.Switch Has Authority`
    (:`Authority`
      (if (and (`self.从实例中生成`) (not (`self.是否正在破环`)))
        (`self.将树实例添加到适当的实例化组件中`)
        (`self.K2_DestroyActor`)))))

(event `HitEffects (Multicast)打击效果（多播）`
  (params (HitLocation :type "Vector Structure") (Rotation :type "Rotator Structure"))
  ;[1 1 1] Effects.
  (`GameplayStatics.SpawnEmitterAtLocation` "/Game/EasySurvivalRPG/Effects/PS_CuttingTree.PS_CuttingTree" HitLocation (`KismetMathLibrary.MakeRotator` 90.0 0.0 (.yaw Rotation)))
  (bind _returnvalue (`GameplayStatics.SpawnDecalAtLocation` "/Game/EasySurvivalRPG/Materials/Instances/MI_Decal_002.MI_Decal_002" (25.0 25.0 10.0) HitLocation (struct) 60.0))
  (`KismetArrayLibrary.Array_Add` (`self.Decals`) _returnvalue))

(event `DestructEffects (Multicast)破坏效果（多播）`
  (bind _decals (`self.Decals`))
  ;[1 1 1] Effects.
  (`GameplayStatics.PlaySoundAtLocation` (`self.CutDownSound`) (`self.K2_GetActorLocation`) (struct) 1.0 1.0 0.0 null null null null)
  (for _array_element _decals
    (`/Engine/EditorBlueprintResources/StandardMacros.IsValid` _array_element
      (:`Is Valid`
        (`ActorComponent.K2_DestroyComponent` _array_element))))
  (`KismetArrayLibrary.Array_Clear` _decals))

(fn `DoesIgnoreSaveLoad_BPI`
  (returns (Result :type Boolean))
  (return false))

(fn `GetComponentSaveID_BPI`
  (returns (Success :type Boolean) (ComponentSaveID :type Integer))
  (return false 0))

(fn `GetFormattedVariables_BPI`
  (returns (FormattedVariables :type "Array of String"))
  ;[1 1 1] Format simple variables.
  (return (`|MakeArray` (`/Game/EasySurvivalRPG/Blueprints/Game/Libraries/BP_SaveLibrary.FormatBooleanVariableToString` "FullyDestructed" (`self.是否完全毁坏`)) (`/Game/EasySurvivalRPG/Blueprints/Game/Libraries/BP_SaveLibrary.FormatBooleanVariableToString` "SpawnedFromInstance" (`self.从实例中生成`)))))

(fn `GetSaveID_BPI`
  (returns (Success :type Boolean) (SaveID :type Integer))
  (return true (`self.SaveID`)))

(fn `LoadData_BPI`
  (params (SaveData :type "SaveGame Object Reference"))
  (returns (Success :type Boolean))
  ;[1 1 1] Load tree data.
  (`|ExecutionSequence`
    (:`then_0`
      (bind (_success _savedata) (message `/Game/EasySurvivalRPG/Blueprints/Interfaces/BPI_GameSave.GetTreeSaveData_BPI` SaveData (`self.SaveID`)))
      (if _success
        (bind (_durability _destructed _respawntimeremaining) (break `/Game/EasySurvivalRPG/Blueprints/Structures/SaveData/STR_SaveData_Tree` _savedata))
        (set `self.耐久性` _durability)
        (bind _output_get (set `self.是否正在破环` _destructed))
        (if _output_get
          (`self.检查并重新生成树` _respawntimeremaining))
        (else
          (return false))))
    (:`then_1`
      (`|ExecutionSequence`
        (:`then_0`
          (bind (_success_2 _savedata_2) (message `/Game/EasySurvivalRPG/Blueprints/Interfaces/BPI_GameSave.GetActorSaveData_BPI` SaveData (`self.SaveID`)))
          (if _success_2
            (bind ((`FormattedVariables_38_8140374D4327F2E43E03C3B17B80F74B` _formattedvariables)) (break `/Game/EasySurvivalRPG/Blueprints/Structures/SaveData/STR_SaveData_Actor` _savedata_2))
            (bind (_success_3 _value) (`/Game/EasySurvivalRPG/Blueprints/Game/Libraries/BP_SaveLibrary.GetFormattedVariableBooleanValue` _formattedvariables "FullyDestructed"))
            (bind (_success_4 _value_2) (`/Game/EasySurvivalRPG/Blueprints/Game/Libraries/BP_SaveLibrary.GetFormattedVariableBooleanValue` _formattedvariables "SpawnedFromInstance"))
            (if (and _success_3 _success_4)
              (set `self.是否完全毁坏` _value)
              (set `self.从实例中生成` _value_2))
            (else
              (return false))))
        (:`then_1`
          (return true))))))

(fn `SaveData_BPI`
  (params (SaveData :type "SaveGame Object Reference"))
  (returns (Success :type Boolean))
  (locals (LocalSaveData :type "SaveGame Object Reference"))
  (bind _saveid (`self.SaveID`))
  ;[1 1 1] Save tree data.
  (bind _formattedvariables (`/Game/EasySurvivalRPG/Blueprints/Interfaces/BPI_SaveData.GetFormattedVariables_BPI`))
  (bind _output_get (set `local.LocalSaveData` SaveData))
  (message `/Game/EasySurvivalRPG/Blueprints/Interfaces/BPI_GameSave.SetActorSaveData_BPI` _output_get _saveid (make `/Game/EasySurvivalRPG/Blueprints/Structures/SaveData/STR_SaveData_Actor` (`GameplayStatics.GetObjectClass` self) (`self.GetTransform`) _formattedvariables))
  (message `/Game/EasySurvivalRPG/Blueprints/Interfaces/BPI_GameSave.SetTreeSaveData_BPI` _output_get _saveid (make `/Game/EasySurvivalRPG/Blueprints/Structures/SaveData/STR_SaveData_Tree` (`self.耐久性`) (`self.是否正在破环`) (`KismetSystemLibrary.K2_GetTimerRemainingTimeHandle` (`self.RespawnTimerHandle`))))
  (return true))

(fn `SetSaveID_BPI`
  (params (SaveID :type Integer))
  (returns (Success :type Boolean))
  ;[1 1 1] Set save ID.
  (set `self.SaveID` SaveID)
  (return true))

(fn `UserConstructionScript`
  ;[1 1 1] 在结构上更新耐用性和树网。
  (set `self.耐久性` (`self.最大耐用性`))
  (`self.根据已破坏的变量更新树网格`))

(fn `产卵会破坏战利品并激活破坏效果`
  (params (Instigator :type "Controller Object Reference"))
  (bind _returnvalue_location (`KismetMathLibrary.BreakTransform` (`SceneComponent.K2_GetComponentToWorld` (`self.StaticMesh`))))
  (bind _returnvalue (`KismetMathLibrary.MakeTransform` (+ _returnvalue_location (2.0 2.0 2.0))))
  ;[1 1 1] 产卵会破坏战利品并激活破坏效果。
  (set `self.是否正在破环` true)
  (`self.根据已破坏的变量更新树网格`)
  (`|SpawnActorFromClass` "/Game/Survival_Inventory/Blueprints/Items/All_Items/wood01.wood01_C" _returnvalue "Undefined" "MultiplyWithRoot" null (struct) null)
  (`|SpawnActorFromClass` "/Game/Survival_Inventory/Blueprints/Items/All_Items/Apple.Apple_C" _returnvalue "Undefined" "MultiplyWithRoot" null (struct) null)
  (`self.检查并重新生成树` (`self.重生时间`))
  (`self.DestructEffects (Multicast)破坏效果（多播）`))

(fn `从适当的实例化组件中删除树实例`
  (locals (LocalComponents :type "Array of /Game/EasySurvivalRPG/Blueprints/Components/InstancedComponents/BP_InstancedComponent_Tree_Base Object Reference"))
  (bind _returnvalue (`self.GetComponentByClass` (`GameplayStatics.GetGameState`) "/Game/EasySurvivalRPG/Blueprints/Components/BP_FoliageManagerComponent.BP_FoliageManagerComponent_C"))
  ;[1 1 1] 从适当的实例化组件中删除树实例。
  (`/Engine/EditorBlueprintResources/StandardMacros.IsValid` _returnvalue
    (:`Is Valid`
      (`/Game/EasySurvivalRPG/Blueprints/Components/BP_FoliageManagerComponent.RemoveInstanceInTransform` _returnvalue (`self.InstancedComponentClass`) (`self.GetTransform`)))))

(fn `完全摧毁树并将演员从游戏中删除`
  (params (Instigator :type "Controller Object Reference"))
  ;[1 1 1] 完全摧毁树并将演员从游戏中删除。
  (set `self.是否完全毁坏` true)
  (`self.OnTreeFullyDestructed` self Instigator)
  (message `/Game/EasySurvivalRPG/Blueprints/Interfaces/BPI_Player.PlayerFullyDestructTree_BPI` Instigator self)
  (message `/Game/EasySurvivalRPG/Blueprints/Interfaces/BPI_GameInstance.SpawnLootItems_BPI` (`GameplayStatics.GetGameInstance`) (`self.FullDestructLootHandle`) (`self.K2_GetActorLocation`) 0.0 0.0 50.0 100.0)
  (if (`self.从实例中生成`)
    (`self.检查并重新生成树` (`self.重生时间`))
    (else
      (`self.K2_DestroyActor`))))

(fn `将从实例生成它将在重生后返回树实例`
  ;[1 1 1] 将“从实例生成”变量设置为true。
  ; 它将在重生后返回树实例。
  (set `self.从实例中生成` true))

(fn `将树实例添加到适当的实例化组件中`
  (locals (LocalComponents :type "Array of /Game/EasySurvivalRPG/Blueprints/Components/InstancedComponents/BP_InstancedComponent_Tree_Base Object Reference"))
  (bind _returnvalue (`self.GetComponentByClass` (`GameplayStatics.GetGameState`) "/Game/EasySurvivalRPG/Blueprints/Components/BP_FoliageManagerComponent.BP_FoliageManagerComponent_C"))
  ;[1 1 1] 将树实例添加到适当的实例化组件中
  (`/Engine/EditorBlueprintResources/StandardMacros.IsValid` _returnvalue
    (:`Is Valid`
      (`/Game/EasySurvivalRPG/Blueprints/Components/BP_FoliageManagerComponent.TryAddInstanceInTransform` _returnvalue (`self.InstancedComponentClass`) (`self.GetTransform`)))))

(fn `建筑物受损时的行动`
  (params (DamageData :type "/Game/EasySurvivalRPG/Blueprints/Structures/DamageSystem/STR_DamageData Structure (by ref)") (InstigatedBy :type "Controller Object Reference") (DamageCauser :type "Actor Object Reference") (HitInfo :type "HitResult Structure"))
  (bind _damage (`/Game/EasySurvivalRPG/Blueprints/Game/Libraries/BP_DamageSystemLibrary.GetDamageValue` DamageData))
  (bind (_bblockinghit _binitialoverlap _time _distance _location) (`GameplayStatics.BreakHitResult` HitInfo))
  ;[1 1 1] 建筑物受损时的行动。
  (if (`self.bCanBeDamaged`)
    (if (>= _damage 0.0)
      (`self.启动返回树定时器`)
      (`|ExecutionSequence`
        (:`then_0`
          (`self.计算树的耐久性并激活命中效果` _location _damage InstigatedBy)
          (`self.HitEffects (Multicast)打击效果（多播）` _location (`self.K2_GetActorRotation` DamageCauser)))
        (:`then_1`
          (if (`/Game/EasySurvivalRPG/Blueprints/Game/Libraries/BP_DamageSystemLibrary.DoesDamageShowDamageText` DamageData)
            (message `/Game/EasySurvivalRPG/Blueprints/Interfaces/BPI_Player.CreateFloatingTextAtLocation_BPI` InstigatedBy _location (`KismetTextLibrary.Conv_DoubleToText` _damage "HalfToEven" false true 1 324 0 0) (struct :`R` 1.0 :`A` 1.0) "NewEnumerator0")))))))

(fn `当完全破坏变量发生变化时更新树网格`
  ;[1 1 1] 当“完全破坏”变量发生变化时，更新树网格。
  (`self.根据已破坏的变量更新树网格`))

(fn `当解构变量发生变化时更新树网格`
  ;[1 1 1] 当“解构”变量发生变化时，更新树网格。
  (`self.根据已破坏的变量更新树网格`))

(fn `恢复树木`
  (bind _returnvalue (`self.K2_GetActorLocation`))
  ;[1 1 1] 恢复树木。
  (bind _outhits (`KismetSystemLibrary.SphereTraceMultiForObjects` _returnvalue _returnvalue 500.0 (`|MakeArray` "ObjectTypeQuery2" :!type "EObjectTypeQuery Enum")))
  (for _array_element _outhits
    (bind (_bblockinghit _binitialoverlap _time _distance _location _impactpoint _normal _impactnormal _physmat _hitactor _hitcomponent) (`GameplayStatics.BreakHitResult` _array_element))
    (if (`PrimitiveComponent.K2_IsPhysicsCollisionEnabled` _hitcomponent)
      (cast `/Game/EasySurvivalRPG/Blueprints/InteractionObjects/BuildingObjects/Base/BP_Building_BaseObject` _hitactor)
      (bind _returnvalue_2 (`KismetSystemLibrary.K2_SetTimerDelegate` (`|CreateDelegate` :!event `恢复树木`) (`self.重生时间`)))
      (set `self.RespawnTimerHandle` _returnvalue_2)
      (return)))
  (set `self.是否正在破环` false)
  (set `self.是否完全毁坏` false)
  (set `self.耐久性` (`self.最大耐用性`))
  (if (`self.从实例中生成`)
    (`self.返回树到实例`)
    (`self.K2_DestroyActor`)))

(fn `根据已破坏的变量更新树网格`
  (bind _staticmesh (`self.StaticMesh`))
  ;[1 1 1] 根据已破坏的变量更新树网格。
  (if (`self.是否完全毁坏`)
    (`StaticMeshComponent.SetStaticMesh` _staticmesh null)
    (else
      (`StaticMeshComponent.SetStaticMesh` _staticmesh (select `bool` (`self.是否正在破环`) :`false` (`self.DefaultMesh`) :`true` (`self.CuttedMesh`))))))

(fn `检查并重新生成树`
  (params (RespawnTime :type "Float (double-precision)"))
  ;[1 1 1] Check and respawn tree.
  (if (`self.可以重生`)
    (if (> RespawnTime 0.0)
      (bind _returnvalue (`KismetSystemLibrary.K2_SetTimerDelegate` (`|CreateDelegate` :!event `恢复树木`) RespawnTime))
      (set `self.RespawnTimerHandle` _returnvalue))))

(fn `计算树的耐久性并激活命中效果`
  (params (HitLocation :type "Vector Structure") (Damage :type "Float (double-precision)") (Instigator :type "Controller Object Reference"))
  (locals (LocalDamage :type "Float (double-precision)") (LocalLocation :type "Vector Structure") (LocalInstigator :type "Controller Object Reference"))
  ;[1 1 1] 计算树的耐久性并激活命中效果
  (set `local.LocalLocation` HitLocation)
  (set `local.LocalDamage` Damage)
  (set `local.LocalInstigator` Instigator)
  (bind _output_get (set `self.耐久性` (- (`self.耐久性`) Damage)))
  (if (not (`self.是否正在破环`))
    (`KismetSystemLibrary.PrintString` (`KismetStringLibrary.Conv_DoubleToString` _output_get))
    (`|ExecutionSequence`
      (:`then_0`
        (if (>= (`local.LocalDamage`) 10.0)
          (message `/Game/EasySurvivalRPG/Blueprints/Interfaces/BPI_GameInstance.SpawnLootItems_BPI` (`GameplayStatics.GetGameInstance`) (`self.HitLootHandle`) (`SceneComponent.GetSocketLocation` (`self.StaticMesh`) (`self.HitLootSocketName`)) 50.0 150.0 -25.0 25.0)))
      (:`then_1`
        (if (<= (`self.耐久性`) 20.0)
          (`self.产卵会破坏战利品并激活破坏效果` (`local.LocalInstigator`))))
      (:`then_2`
        (if (<= (`self.耐久性`) 0.0)
          (set `self.是否完全毁坏` false)
          (`self.完全摧毁树并将演员从游戏中删除` (`local.LocalInstigator`)))))))