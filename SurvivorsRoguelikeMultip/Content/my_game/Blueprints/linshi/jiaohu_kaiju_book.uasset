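; Interactable book actor, apparently for the game's opening, that toggles the Chushi UI widget on screen.
; Its object interaction event (物件交互) proceeds only when the same-direction flag (是否同向) is true.
; A FlipFlop alternates between creating and showing a new widget and collapsing it; collapsed widgets are never removed from the viewport.
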(event `/Game/my_game/Blueprints/jiekou/交互临时.物件交互`
  (if (`self.是否同向`)
    (`/Engine/EditorBlueprintResources/StandardMacros.FlipFlop`
      (:`A`
        (bind _returnvalue (`|CreateWidget` "/Game/my_game/UI/chushi.chushi_C"))
        (`UserWidget.AddToViewport` _returnvalue 0)
        (`Widget.SetVisibility` _returnvalue "Visible"))
      (:`B`
        (`Widget.SetVisibility` _returnvalue "Collapsed")))))

(fn `UserConstructionScript`
  (`parent.UserConstructionScript`))