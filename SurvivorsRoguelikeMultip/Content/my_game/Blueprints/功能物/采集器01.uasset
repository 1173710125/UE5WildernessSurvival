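; Gathering tool (采集器01) that serves as the player's main weapon, damaging trees, mine nodes and ani_lu_01 actors it hits.
; Box overlaps count only while the character's animation state matches a specific value, with a cast per target type setting damage.
; Each hit drains durability, initialized to maximum on BeginPlay.
; At zero durability it destroys itself and resets the character's animation, main-weapon flag and state.
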(event `self.ReceiveBeginPlay`
  (bind _asmy_character_shengchun (cast `/Game/my_game/Blueprints/My_Character_shengchun` (`GameplayStatics.GetPlayerCharacter` 0)))
  (set `self.As My Character` _asmy_character_shengchun)
  (set `self.耐久度` (`self.最大耐久`)))

(event `self.Box.OnComponentBeginOverlap`
  (params (OverlappedComponent :type "PrimitiveComponent Object Reference") (OtherActor :type "Actor Object Reference") (OtherComp :type "PrimitiveComponent Object Reference") (OtherBodyIndex :type Integer) (bFromSweep :type Boolean) (SweepResult :type "HitResult Structure (by ref)"))
  (if (`|EnumEquality` (`/Game/my_game/ani/100501_unit_Skeleton_AnimBlueprint.my_zhuangtai` (`/Game/my_game/Blueprints/My_Character_shengchun.As My Ani 02` (`self.As My Character`))) "NewEnumerator4")
    (`|ExecutionSequence`
      (:`then_0`
        ;[1 1 1] 对树造成伤害
        (bind _asbp_tree_base (cast `/Game/my_game/Blueprints/jiaohu_caiji/Trees/BP_Tree_Base` OtherActor))
        (bind _output_get (set `self.As BP Tree Base` _asbp_tree_base))
        (`GameplayStatics.ApplyDamage` _output_get 8.0)
        ;[1 1 1] 销毁后回到初始状态
        (`self.武器损害后回归角色正常状态` 25.0))
      (:`then_1`
        ;[1 1 1] 对sitou造成伤害
        (bind _asbp_mine_base (cast `/Game/my_game/Blueprints/jiaohu_caiji/Mine/BP_Mine_Base` OtherActor))
        (bind _output_get_2 (set `self.As BP Mine Base` _asbp_mine_base))
        (`GameplayStatics.ApplyDamage` _output_get_2 10.0)
        (`self.武器损害后回归角色正常状态` 5.0))
      (:`then_2`
        (bind _asani_lu_01 (cast `/Game/my_game/Blueprints/monster/非猛兽/鹿01/ani_lu_01` OtherActor))
        (`GameplayStatics.ApplyDamage` _asani_lu_01 50.0)
        (`self.武器损害后回归角色正常状态` 5.0)))))

(fn `UserConstructionScript`)

(fn `武器损害后回归角色正常状态`
  (params (`伤害值` :type "Float (double-precision)"))
  (bind _as_my_character (`self.As My Character`))
  (bind _output_get (set `self.耐久度` (- (`self.耐久度`) `伤害值`)))
  (if (<= _output_get 0.0)
    (`self.K2_DestroyActor`)
    (set `/Game/my_game/ani/100501_unit_Skeleton_AnimBlueprint.my_zhuangtai` "NewEnumerator0" (`/Game/my_game/Blueprints/My_Character_shengchun.As My Ani 02` _as_my_character))
    (set `/Game/my_game/Blueprints/My_Character_shengchun.是否生成主武器` false _as_my_character)
    (set `/Game/my_game/Blueprints/My_Character_shengchun.角色状态` "NewEnumerator0" _as_my_character)))