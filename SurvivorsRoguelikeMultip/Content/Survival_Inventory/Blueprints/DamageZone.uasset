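; DamageZone is a zone actor in the survival inventory project, apparently meant to damage players inside it.
; Its DamageZone component's begin and end overlap events add and remove actors in an Actors array, on authority only.
; The damage side is inactive: BeginPlay, Damage and DamageTaken are empty, and the looping timer, array loop, cast and validity check are disconnected, so no damage is applied.
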(event `self.ReceiveBeginPlay`
  ;[1 1 1] Apply damage to players
)

(event `Damage`
  ;[1 1 1] Apply damage to players
)

(event `self.DamageZone.OnComponentBeginOverlap`
  (params (OverlappedComponent :type "PrimitiveComponent Object Reference") (OtherActor :type "Actor Object Reference") (OtherComp :type "PrimitiveComponent Object Reference") (OtherBodyIndex :type Integer) (bFromSweep :type Boolean) (SweepResult :type "HitResult Structure (by ref)"))
  ;[1 1 1] Add and remove actors to array
  (`/Engine/EditorBlueprintResources/ActorMacros.Switch Has Authority`
    (:`Authority`
      (`KismetArrayLibrary.Array_Add` (`self.Actors`) OtherActor))))

(event `self.DamageZone.OnComponentEndOverlap`
  (params (OverlappedComponent :type "PrimitiveComponent Object Reference") (OtherActor :type "Actor Object Reference") (OtherComp :type "PrimitiveComponent Object Reference") (OtherBodyIndex :type Integer))
  ;[1 1 1] Add and remove actors to array
  (`/Engine/EditorBlueprintResources/ActorMacros.Switch Has Authority`
    (:`Authority`
      (`KismetArrayLibrary.Array_RemoveItem` (`self.Actors`) OtherActor))))

(fn `UserConstructionScript`)