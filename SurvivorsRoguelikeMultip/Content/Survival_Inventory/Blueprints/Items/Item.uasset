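; World pickup actor for the survival inventory, taking its static mesh from item struct data at construction and on spawn.
; Interaction passes the item to the player component's server pickup call, and DestroyItem hides and destroys it for all clients, guarded by a destroyed flag.
; Box overlaps flag when a player character is in range, and Tick then stores whether the locally cached player character (index 0) faces the item.
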(event `On Spawned`
  ;[1 1 1] 派生集静态网格上的所有客户端
  (`StaticMeshComponent.SetStaticMesh` (`self.Item World Mesh`) (`.moxing_109_7444C39B45931133AB5875A654072A5A` (break `/Game/Survival_Inventory/Blueprints/Other/my_beibao_wupinshuxing` (`.Item Details Out` (`/Game/Survival_Inventory/Blueprints/Other/InventoryFunctions.总结构体` (`self.Item`)))))))

(event `Destroy Item`
  ;[1 1 1] All clients destroy item
  (if (not (`self.当前拾取已销毁`))
    (`SceneComponent.SetVisibility` (`self.Item World Mesh`) false false)
    (set `self.当前拾取已销毁` true)
    (`self.K2_DestroyActor`)))

(event `self.ReceiveBeginPlay`
  (`|ExecutionSequence`
    (:`then_0`
      (bind _asmy_yewai_01_kongzhiqi (cast `/Game/my_game/my_yewai01_kongzhiqi` (`GameplayStatics.GetPlayerController` 0)))
      (set `self.As My Yewai 01 Kongzhiqi` _asmy_yewai_01_kongzhiqi))
    (:`then_1`
      (bind _asmy_character (cast `/Game/my_game/Blueprints/My_Character` (`GameplayStatics.GetPlayerCharacter` 0)))
      (set `self.As My Character` _asmy_character))))

(event `my_Interact`
  (params (`Player Component` :type "/Game/Survival_Inventory/Blueprints/Components/PlayerInventoryComponent Object Reference"))
  ;[1 1 1] 交互后进入背包
  (if (not (`self.当前拾取已销毁`))
    (`/Game/Survival_Inventory/Blueprints/Components/PlayerInventoryComponent.服务器取货项目` `Player Component` self)
    (set `self.Player Component` `Player Component`)))

(event `self.Box.OnComponentBeginOverlap`
  (params (OverlappedComponent :type "PrimitiveComponent Object Reference") (OtherActor :type "Actor Object Reference") (OtherComp :type "PrimitiveComponent Object Reference") (OtherBodyIndex :type Integer) (bFromSweep :type Boolean) (SweepResult :type "HitResult Structure (by ref)"))
  ;[1 1 1] 交互判断事件
  (cast `/Game/my_game/Blueprints/My_Character` OtherActor)
  (set `self.是否在交互范围` true))

(event `self.ReceiveTick`
  (params (DeltaSeconds :type "Float (single-precision)"))
  ;[1 1 1] 交互判断事件
  (if (`KismetSystemLibrary.IsValid` self)
    (`|ExecutionSequence`
      (:`then_0`
        (if (`self.是否在交互范围`)
          (bind `_是否同向` (`/Game/my_game/Blueprints/hanshuku/my_hanshuku.角色与物体朝向交互判断` (`self.Box`) (`self.As My Character`)))
          (set `self.是否同向` `_是否同向`))))))

(event `self.Box.OnComponentEndOverlap`
  (params (OverlappedComponent :type "PrimitiveComponent Object Reference") (OtherActor :type "Actor Object Reference") (OtherComp :type "PrimitiveComponent Object Reference") (OtherBodyIndex :type Integer))
  ;[1 1 1] 交互判断事件
  (cast `/Game/my_game/Blueprints/My_Character` OtherActor)
  (set `self.是否在交互范围` false))

(fn `UserConstructionScript`
  (bind (_return_value _item_details_out) (`/Game/Survival_Inventory/Blueprints/Other/InventoryFunctions.总结构体` (`self.Item`)))
  (if _return_value
    (`StaticMeshComponent.SetStaticMesh` (`self.Item World Mesh`) (`.moxing_109_7444C39B45931133AB5875A654072A5A` (break `/Game/Survival_Inventory/Blueprints/Other/my_beibao_wupinshuxing` _item_details_out)))))