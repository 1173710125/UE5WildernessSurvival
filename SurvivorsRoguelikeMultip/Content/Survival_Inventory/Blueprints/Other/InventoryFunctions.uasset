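; Inventory function library for item detail lookups and for tracking activated actors by name.
; Item details come from the My_zhenpin data table, keyed by item ID.
; Two checks test names against separate save objects, MyGame and MyGame2, on my_gameinstance.
; Adding a name writes uniquely to the game instance's ActorNamejihuo array rather than those saves; its save-loading branch is unconnected.
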(fn `判断actor是否激活`
  (params (`名字` :type String))
  (returns (ReturnValue :type Boolean))
  (bind _asmy_gameinstance (cast `/Game/MY/存档/my_gameinstance` (`GameplayStatics.GetGameInstance` null)))
  (return (`KismetArrayLibrary.Array_Contains` (`/Game/MY/存档/my_savegame.actor激活名字` (`/Game/MY/存档/my_gameinstance.my_game` _asmy_gameinstance)) `名字`)))

(fn `判断actor是否激活2`
  (params (`名字2` :type String))
  (returns (`返回` :type Boolean))
  (bind _asmy_gameinstance (cast `/Game/MY/存档/my_gameinstance` (`GameplayStatics.GetGameInstance` null)))
  (return (`KismetArrayLibrary.Array_Contains` (`/Game/MY/存档/my_savegame02.actor激活名字2` (`/Game/MY/存档/my_gameinstance.my_game2` _asmy_gameinstance)) `名字2`)))

(fn `总结构体`
  (params (`Item In` :type "/Game/Survival_Inventory/Blueprints/Other/my_beibao_jiegouti Structure"))
  (returns (`Return Value` :type Boolean) (`Item Details Out` :type "/Game/Survival_Inventory/Blueprints/Other/my_beibao_wupinshuxing Structure"))
  ;[1 1 1] Get the items details
  (bind _returnvalue (`|GetDataTableRow` "/Game/Survival_Inventory/Blueprints/Items/my_zhenpin.my_zhenpin" (`KismetStringLibrary.Conv_StringToName` (`.ID_24_9DF34B624AB0F3F6510E998638C6FAE4` (break `/Game/Survival_Inventory/Blueprints/Other/my_beibao_jiegouti` `Item In`))))
    (:`then`
      (return true _returnvalue))
    (:`RowNotFound`
      (return false))))

(fn `添加激活的actor`
  (params (`名字` :type String))
  (bind _asmy_gameinstance (cast `/Game/MY/存档/my_gameinstance` (`GameplayStatics.GetGameInstance` null)))
  (`KismetArrayLibrary.Array_AddUnique` (`/Game/MY/存档/my_gameinstance.actor_namejihuo` _asmy_gameinstance) `名字`))