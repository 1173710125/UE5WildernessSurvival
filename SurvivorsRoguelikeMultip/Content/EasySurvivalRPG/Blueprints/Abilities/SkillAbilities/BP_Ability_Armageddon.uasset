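; Armageddon skill ability that darkens the level and rains a barrage of meteor projectiles around the instigator.
; On use, a timeline lerps the last-found directional light's intensity and color and sky light's intensity toward target values.
; A looping timer paces meteor launches from high above, with randomized position, angle and scale.
; Projectile class comes from a data table handle; the ability destroys itself when the count runs out.
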(event `self.Use`
  ;[1 1 1] Start armageddon on use.
  (`self.StartArmageddon`))

(event `ToDarkness`
  (bind _skylightcomponent (`self.SkyLightComponent`))
  (bind _sunlightcomponent (`self.SunLightComponent`))
  ;[1 1 1] Update intensity of light components.
  (bind (_direction _alpha) (`Timeline|DarknessTimeline`)
    (:`Update`
      (`|ExecutionSequence`
        (:`then_0`
          (`/Engine/EditorBlueprintResources/StandardMacros.IsValid` _sunlightcomponent
            (:`Is Valid`
              (`LightComponent.SetIntensity` _sunlightcomponent (`KismetMathLibrary.Lerp` (`self.InitialSunLightIntensity`) (`self.TargetSunLightIntensity`) _alpha))
              (`LightComponent.SetLightColor` _sunlightcomponent (`KismetMathLibrary.LinearColorLerp` (`self.InitialSunLightColor`) (`self.TargetSunLightColor`) _alpha) true))))
        (:`then_1`
          (`/Engine/EditorBlueprintResources/StandardMacros.IsValid` _skylightcomponent
            (:`Is Valid`
              (`SkyLightComponent.SetIntensity` _skylightcomponent (`KismetMathLibrary.Lerp` (`self.InitialSkyLightIntensity`) (`self.TargetSkyLightIntensity`) _alpha)))))))))

(fn `FindProjectileSettings`
  (returns (ProjectileClass :type "/Game/EasySurvivalRPG/Blueprints/InteractionObjects/Projectiles/Base/BP_Projectile_Base Class Reference") (ProjectileHandle :type "DataTableRowHandle Structure"))
  (bind (_value _returnvalue) (`BlueprintMapLibrary.Map_Find` (`.Handles_63_88DAB6504152B8CF608F39A3D2A5D080` (break `/Game/EasySurvivalRPG/Blueprints/Structures/AbilitySystem/STR_AbilityInstance` (`self.AbilitySettings`))) "Projectile"))
  (bind (_datatable _rowname) (break `DataTableRowHandle` _value))
  ;[1 1 1] Try to find projectile class and handle.
  (if _returnvalue
    (`/Engine/EditorBlueprintResources/StandardMacros.IsValid` _datatable
      (:`Is Valid`
        (bind _returnvalue_2 (`|GetDataTableRow` _datatable _rowname)
          (:`then`
            (bind ((`Handle_2_36E7D8A44585B051C187BEAF03821A24` _handle) (`ProjectileClass_5_6EED3A7E422F7A257075538A38385778` _projectileclass)) (break `/Game/EasySurvivalRPG/Blueprints/Structures/AbilitySystem/STR_ProjectileInstance` _returnvalue_2))
            (bind _output_get (set `self.ProjectileHandle` _handle))
            (bind _output_get_2 (set `self.ProjectileClass` _projectileclass)))
          (:`RowNotFound`
            _)))
      (:`Is Not Valid`
        _)))
  (return _output_get_2 _output_get))

(fn `LaunchMeteor`
  (locals (LocalRandomScale :type "Float (double-precision)" :default 0.0))
  (bind _countremaining (`self.CountRemaining`))
  ;[1 1 1] Spawn meteor and launch it from the sky.
  (if (> _countremaining 0)
    (set `self.CountRemaining` (- _countremaining 1))
    (bind (_success _projectile) (`self.SpawnProjectile`))
    (if _success
      (bind (_isoverridden _overriddenspeed) (message `/Game/EasySurvivalRPG/Blueprints/Interfaces/BPI_Character.GetLaunchItemSpeed_BPI` (`self.GetInstigator`)))
      (`/Game/EasySurvivalRPG/Blueprints/InteractionObjects/Projectiles/Base/BP_Projectile_Base.LaunchProjectileForward` _projectile _isoverridden _overriddenspeed))
    (else
      (`self.K2_DestroyActor`))))

(fn `SpawnProjectile`
  (returns (Success :type Boolean) (Projectile :type "/Game/EasySurvivalRPG/Blueprints/InteractionObjects/Projectiles/Base/BP_Projectile_Base Object Reference"))
  (locals (LocalRandomScale :type "Float (double-precision)") (LocalSpawnTransform :type "Transform Structure"))
  (bind _localrandomscale (`local.LocalRandomScale`))
  ;[1 1 1] Spawn projectile with specific attributes.
  (set `local.LocalRandomScale` (`KismetMathLibrary.RandomFloatInRange` 1.0 2.0))
  (set `local.LocalSpawnTransform` (`KismetMathLibrary.MakeTransform` (+ (`self.SpawnLocation`) (`KismetMathLibrary.MakeVector` (`KismetMathLibrary.RandomFloatInRange` -10000.0 10000.0) (`KismetMathLibrary.RandomFloatInRange` -10000.0 10000.0))) (`KismetMathLibrary.ComposeRotators` (`self.SpawnRotation`) (`KismetMathLibrary.MakeRotator` 0.0 (`KismetMathLibrary.RandomFloatInRange` -15.0 15.0) (`KismetMathLibrary.RandomFloatInRange` -15.0 15.0))) (`KismetMathLibrary.MakeVector` _localrandomscale _localrandomscale _localrandomscale)))
  (bind (_projectileclass _projectilehandle) (`self.FindProjectileSettings`))
  (bind _returnvalue (`|SpawnActorFromClass` _projectileclass (`local.LocalSpawnTransform`) "AlwaysSpawn" "OverrideRootScale" null _projectilehandle (`self.GetInstigator`)))
  (return true _returnvalue))

(fn `StartArmageddon`
  (returns (Success :type Boolean))
  (locals (LocalSpawnLocation :type "Vector Structure"))
  (bind _returnvalue (`self.K2_GetActorLocation` (`self.GetInstigator`)))
  ;[1 1 1] Start darkness timeline and start spawn timer for meteors spawning.
  (`self.StartDarkness`)
  (bind _output_get (set `local.LocalSpawnLocation` (+ _returnvalue (0.0 0.0 10000.0))))
  (set `self.SpawnLocation` _output_get)
  (set `self.SpawnRotation` (`KismetMathLibrary.FindLookAtRotation` (`local.LocalSpawnLocation`) _returnvalue))
  (set `self.CountRemaining` (`self.MeteorsCount`))
  (`KismetSystemLibrary.K2_SetTimerDelegate` (`|CreateDelegate` :!event `LaunchMeteor`) 0.075 true)
  (return true))

(fn `StartDarkness`
  ;[1 1 1] Set sun light and sky light components and start darkness timeline.
  (`|ExecutionSequence`
    (:`then_0`
      (bind _outactors (`GameplayStatics.GetAllActorsOfClass` "/Script/Engine.DirectionalLight"))
      (for _array_element _outactors
        (bind _output_get (set `self.SunLightComponent` (`Light.LightComponent` _array_element)))
        (set `self.InitialSunLightIntensity` (`LightComponentBase.Intensity` _output_get))
        (set `self.InitialSunLightColor` (`LightComponentBase.GetLightColor` _output_get))))
    (:`then_1`
      (bind _outactors_2 (`GameplayStatics.GetAllActorsOfClass` "/Script/Engine.SkyLight"))
      (for _array_element_2 _outactors_2
        (bind _lightcomponent (`SkyLight.LightComponent` _array_element_2))
        (set `self.SkyLightComponent` _lightcomponent)
        (set `self.InitialSkyLightIntensity` (`LightComponentBase.Intensity` _lightcomponent)))
      (`self.ToDarkness`))))

(fn `UserConstructionScript`
  (`parent.UserConstructionScript`))