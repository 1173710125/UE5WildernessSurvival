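; Item ability actor that remotely detonates nearby devices when used, then destroys itself whether or not anything was triggered.
; It fetches a remote key from the instigator's controller, then runs a stationary sphere trace for WorldDynamic objects around its own location.
; Each hit actor implementing BPI_Remote receives a detonate message with that key and the instigator, leaving the response to that actor.
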(event `self.Use`
  ;[1 1 1] Use event.
  (`|ExecutionSequence`
    (:`then_0`
      (`self.TryDetonate`))
    (:`then_1`
      (`self.K2_DestroyActor`))))

(fn `TryDetonate`
  (returns (Success :type Boolean))
  (locals (LocalRemoteKey :type String))
  (bind _returnvalue (`self.K2_GetActorLocation`))
  ;[1 1 1] Try to detonate remote actors.
  (bind (_success _remotekey) (message `/Game/EasySurvivalRPG/Blueprints/Interfaces/BPI_Remote.GetRemoteKey_BPI` (`self.GetInstigatorController`)))
  (if _success
    (set `local.LocalRemoteKey` _remotekey)
    (bind _outhits (`KismetSystemLibrary.SphereTraceMultiForObjects` _returnvalue _returnvalue 3000.0 (`|MakeArray` "ObjectTypeQuery2" :!type "EObjectTypeQuery Enum")))
    (for _array_element _outhits
      (bind (_bblockinghit _binitialoverlap _time _distance _location _impactpoint _normal _impactnormal _physmat _hitactor) (`GameplayStatics.BreakHitResult` _array_element))
      (if (`KismetSystemLibrary.DoesImplementInterface` _hitactor "/Game/EasySurvivalRPG/Blueprints/Interfaces/BPI_Remote.BPI_Remote_C")
        (message `/Game/EasySurvivalRPG/Blueprints/Interfaces/BPI_Remote.TryDetonate_BPI` _hitactor (`local.LocalRemoteKey`) (`self.GetInstigator`))))
    (return true)
    (else
      (return false))))

(fn `UserConstructionScript`
  (`parent.UserConstructionScript`))