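; Instanced foliage component for ferns that spawns a fern actor at a given instance transform.
; Spawn passes itself to the actor as its owning component and always spawns regardless of collision.
; For locations in HiddenLocations, it multiplies the scale by 100 and calls TryHideFoliage on the new actor with HideLevel.
; Saving clears the added and removed transform lists before calling the parent, so those changes are not saved.
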(fn `SaveData_BPI`
  (params (SaveData :type "SaveGame Object Reference"))
  (returns (Success :type Boolean))
  ;[1 1 1] Clear transform variables before saving.
  (`KismetArrayLibrary.Array_Clear` (`self.AddedTransforms`))
  (`KismetArrayLibrary.Array_Clear` (`self.RemovedTransforms`))
  (bind _success (`parent.SaveData_BPI` SaveData))
  (return _success))

(fn `Spawn`
  (params (Transform :type "Transform Structure"))
  (returns (Success :type Boolean))
  (bind _location (.location Transform))
  (bind _scale (.scale Transform))
  (bind _returnvalue (`KismetArrayLibrary.Array_Contains` (`self.HiddenLocations`) _location))
  ;[1 1 1] Spawn the fern actor.
  (bind _returnvalue_2 (`|SpawnActorFromClass` (`self.FernActorClass`) (`KismetMathLibrary.MakeTransform` _location (.rotation Transform) (select `bool` _returnvalue :`false` _scale :`true` (* _scale 100.0))) "AlwaysSpawn" "OverrideRootScale" null self null))
  (if _returnvalue
    (`/Game/EasySurvivalRPG/Blueprints/InteractionObjects/Misc/BP_InteractionFoliage_Base.TryHideFoliage` _returnvalue_2 (`self.HideLevel`)))
  (return true))