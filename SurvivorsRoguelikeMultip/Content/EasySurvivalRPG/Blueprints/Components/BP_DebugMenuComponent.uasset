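; Debug menu component on a player controller that opens a cheat UI for characters, attributes, items, containers, spawning, teleports and level transit.
; It lazily creates the local UI_DebugMenu widget and switches cursor and input mode when toggled.
; Menu events forward to Server RPCs that act on the controlled pawn, mostly through interface messages.
; Spawning uses camera traces or pawn location, and tracks spawned characters, companions and placed spawn points for later clearing.
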(event `self.ReceiveBeginPlay`
  ;[1 1 1] Begin play. Init component.
  (`self.InitComponent`))

(event `SetCharacterCanBeDamaged`
  (params (CanBeDamaged :type Boolean))
  ;[1 1 1] Character page debug events.
  (`self.SetCharacterCanBeDamaged (Server)` CanBeDamaged))

(event `TryChangeAttributeValue`
  (params (AttributeTag :type "GameplayTag Structure") (Value :type "Float (double-precision)") (Operation :type "/Game/EasySurvivalRPG/Blueprints/Enumerations/E_ChangeVariableOperation Enum" :default "NewEnumerator4"))
  ;[1 1 1] Attributes page debug events.
  (`self.TryChangeAttributeValue (Server)` AttributeTag Value Operation))

(event `TryAddItemToContainer`
  (params (ItemData :type "/Game/EasySurvivalRPG/Blueprints/Structures/Items/STR_ItemData Structure") (ContainerName :type Name))
  ;[1 1 1] Items page debug events.
  (`self.TryAddItemToContainer (Server)` (`/Game/EasySurvivalRPG/Blueprints/Game/Libraries/BP_ItemsLibrary.ItemDataToTransfer` ItemData) ContainerName))

(event `TryAddLootToContainer`
  (params (LootListHandle :type "DataTableRowHandle Structure") (ContainerName :type Name))
  ;[1 1 1] Containers page debug events.
  (`self.TryAddLootToContainer (Server)` LootListHandle ContainerName))

(event `TrySpawnCharacters`
  (params (SpawnSettings :type "/Game/EasySurvivalRPG/Blueprints/Structures/Misc/STR_SpawnSettings Structure") (PlaceSpawnPoint :type Boolean))
  ;[1 1 1] Spawn page debug events.
  (`self.TrySpawnCharacters (Server)` SpawnSettings PlaceSpawnPoint))

(event `TryTransitToLevel`
  (params (LevelName :type Name) (PointName :type Name) (SaveName :type Name))
  ;[1 1 1] Levels page debug events.
  (`self.TryTransitToLevel (Server)` LevelName PointName SaveName))

(event `SetCharacterCanBeDamaged (Server)`
  (params (CanBeDamaged :type Boolean))
  (bind _returnvalue (`Controller.K2_GetPawn` (`self.PlayerController`)))
  ;[1 1 1] Character page debug events.
  (`/Engine/EditorBlueprintResources/StandardMacros.IsValid` _returnvalue
    (:`Is Valid`
      (set `Actor.bCanBeDamaged` CanBeDamaged _returnvalue))))

(event `TryAddItemToContainer (Server)`
  (params (ItemTransferData :type "/Game/EasySurvivalRPG/Blueprints/Structures/Items/STR_ItemTransferData Structure") (ContainerName :type Name))
  (bind _itemdata (`/Game/EasySurvivalRPG/Blueprints/Game/Libraries/BP_ItemsLibrary.ItemTransferToData` ItemTransferData))
  (bind _returnvalue (`Controller.K2_GetPawn` (`self.PlayerController`)))
  ;[1 1 1] Items page debug events.
  (`/Engine/EditorBlueprintResources/StandardMacros.IsValid` _returnvalue
    (:`Is Valid`
      (bind (_inventory _equipment _hotbar) (message `/Game/EasySurvivalRPG/Blueprints/Interfaces/BPI_PlayerCharacter.GetPlayerContainers_BPI` _returnvalue))
      (switch `name` ContainerName
        (:`Inventory`
          (`/Game/EasySurvivalRPG/Blueprints/Components/BP_ContainerComponent.TryAddItem` _inventory _itemdata))
        (:`Equipment`
          (`/Game/EasySurvivalRPG/Blueprints/Components/BP_ContainerComponent.TryAddItem` _equipment _itemdata))
        (:`Hotbar`
          (`/Game/EasySurvivalRPG/Blueprints/Components/BP_ContainerComponent.TryAddItem` _hotbar _itemdata))))))

(event `TryAddLootToContainer (Server)`
  (params (LootListHandle :type "DataTableRowHandle Structure") (ContainerName :type Name))
  (bind _lootitems (`/Game/EasySurvivalRPG/Blueprints/Game/Libraries/BP_ItemsLibrary.MakeLootItems` LootListHandle))
  (bind _returnvalue (`Controller.K2_GetPawn` (`self.PlayerController`)))
  ;[1 1 1] Containers page debug events.
  (`/Engine/EditorBlueprintResources/StandardMacros.IsValid` _returnvalue
    (:`Is Valid`
      (bind (_inventory _equipment _hotbar) (message `/Game/EasySurvivalRPG/Blueprints/Interfaces/BPI_PlayerCharacter.GetPlayerContainers_BPI` _returnvalue))
      (switch `name` ContainerName
        (:`Inventory`
          (`/Game/EasySurvivalRPG/Blueprints/Components/BP_ContainerComponent.TryAddItems` _inventory _lootitems))
        (:`Equipment`
          (`/Game/EasySurvivalRPG/Blueprints/Components/BP_ContainerComponent.TryAddItems` _equipment _lootitems))
        (:`Hotbar`
          (`/Game/EasySurvivalRPG/Blueprints/Components/BP_ContainerComponent.TryAddItems` _hotbar _lootitems))))))

(event `TrySpawnCharacters (Server)`
  (params (SpawnSettings :type "/Game/EasySurvivalRPG/Blueprints/Structures/Misc/STR_SpawnSettings Structure") (PlaceSpawnPoint :type Boolean))
  ;[1 1 1] Spawn page debug events.
  (bind (_found _hitresult _hitlocation) (`self.TryFindTraceHit`))
  (if _found
    (`self.PlaceSpawnPoint` _hitlocation SpawnSettings (not PlaceSpawnPoint))))

(event `TryTransitToLevel (Server)`
  (params (LevelName :type Name) (PointName :type Name) (SaveName :type Name))
  ;[1 1 1] Levels page debug events.
  (`self.TransitToLevel` LevelName PointName SaveName))

(event `TryChangeAttributeValue (Server)`
  (params (AttributeTag :type "GameplayTag Structure") (Value :type "Float (double-precision)") (Operation :type "/Game/EasySurvivalRPG/Blueprints/Enumerations/E_ChangeVariableOperation Enum" :default "NewEnumerator4"))
  ;[1 1 1] Attributes page debug events.
  (message `/Game/EasySurvivalRPG/Blueprints/Interfaces/BPI_Player.ChangePlayerAttribute_BPI` (`self.PlayerController`) AttributeTag Value Operation))

(event `ToggleCharacterCanBeDamaged`
  ;[1 1 1] Character page debug events.
  (`self.ToggleCharacterCanBeDamaged (Server)`))

(event `TrySpawnCompanions`
  (params (SpawnSettings :type "/Game/EasySurvivalRPG/Blueprints/Structures/Misc/STR_SpawnSettings Structure"))
  ;[1 1 1] Spawn page debug events.
  (`self.TrySpawnCompanions (Server)` SpawnSettings))

(event `TryTeleportToNextPlayerStart`
  ;[1 1 1] Levels page debug events.
  (`self.TryTeleportToNextPlayerStart (Server)`))

(event `TrySpawnItem`
  (params (ItemData :type "/Game/EasySurvivalRPG/Blueprints/Structures/Items/STR_ItemData Structure"))
  ;[1 1 1] Items page debug events.
  (`self.TrySpawnItem (Server)` (`/Game/EasySurvivalRPG/Blueprints/Game/Libraries/BP_ItemsLibrary.ItemDataToTransfer` ItemData)))

(event `TrySpawnLoot`
  (params (LootListHandle :type "DataTableRowHandle Structure"))
  ;[1 1 1] Containers page debug events.
  (`self.TrySpawnLoot (Server)` LootListHandle))

(event `ToggleCharacterCanBeDamaged (Server)`
  (bind _returnvalue (`Controller.K2_GetPawn` (`self.PlayerController`)))
  ;[1 1 1] Character page debug events.
  (`/Engine/EditorBlueprintResources/StandardMacros.IsValid` _returnvalue
    (:`Is Valid`
      (set `Actor.bCanBeDamaged` (not (`Actor.bCanBeDamaged` _returnvalue)) _returnvalue))))

(event `TrySpawnCompanions (Server)`
  (params (SpawnSettings :type "/Game/EasySurvivalRPG/Blueprints/Structures/Misc/STR_SpawnSettings Structure"))
  (bind _returnvalue (`Controller.K2_GetPawn` (`self.PlayerController`)))
  ;[1 1 1] Spawn page debug events.
  (`/Engine/EditorBlueprintResources/StandardMacros.IsValid` _returnvalue
    (:`Is Valid`
      (bind _spawnedcharacters (`self.PlaceSpawnPoint` (`Actor.K2_GetActorLocation` _returnvalue) SpawnSettings true))
      (for _array_element _spawnedcharacters
        (`self.AddCompanion` _array_element)))))

(event `TryTeleportToNextPlayerStart (Server)`
  ;[1 1 1] Levels page debug events.
  (`self.TeleportToNextPlayerStart`))

(event `TrySpawnItem (Server)`
  (params (ItemTransferData :type "/Game/EasySurvivalRPG/Blueprints/Structures/Items/STR_ItemTransferData Structure"))
  (bind (_itemhandle _amount _charges _durability _decay _name _description _icon _itemclass) (break `/Game/EasySurvivalRPG/Blueprints/Structures/Items/STR_ItemData` (`/Game/EasySurvivalRPG/Blueprints/Game/Libraries/BP_ItemsLibrary.ItemTransferToData` ItemTransferData)))
  ;[1 1 1] Items page debug events.
  (bind (_found _hitresult _hitlocation) (`self.TryFindTraceHit`))
  (if _found
    (`|SpawnActorFromClass` _itemclass (`KismetMathLibrary.MakeTransform` _hitlocation) "AlwaysSpawn" "SelectDefaultAtRuntime" null _itemhandle _amount _charges _durability _decay true true false null)))

(event `TrySpawnLoot (Server)`
  (params (LootListHandle :type "DataTableRowHandle Structure"))
  ;[1 1 1] Containers page debug events.
  (bind (_found _hitresult _hitlocation) (`self.TryFindTraceHit`))
  (if _found
    (`self.SpawnItems` (`/Game/EasySurvivalRPG/Blueprints/Game/Libraries/BP_ItemsLibrary.MakeLootItems` LootListHandle) _hitlocation)))

(event `OverrideMovementSpeed`
  (params (OverrideSpeed :type Boolean) (TargetSpeed :type "Float (double-precision)"))
  ;[1 1 1] Character page debug events.
  (`self.OverrideMovementSpeed (Server)` OverrideSpeed TargetSpeed))

(event `TryClearSpawnPoints`
  (params (ClearPlacedOnly :type Boolean))
  ;[1 1 1] Spawn page debug events.
  (`self.TryClearSpawnPoints (Server)` ClearPlacedOnly))

(event `ClearContainer`
  (params (ContainerName :type Name))
  ;[1 1 1] Containers page debug events.
  (`self.ClearContainer (Server)` ContainerName))

(event `OverrideMovementSpeed (Server)`
  (params (OverrideSpeed :type Boolean) (TargetSpeed :type "Float (double-precision)"))
  (bind _returnvalue (`Controller.K2_GetPawn` (`self.PlayerController`)))
  ;[1 1 1] Character page debug events.
  (`/Engine/EditorBlueprintResources/StandardMacros.IsValid` _returnvalue
    (:`Is Valid`
      (message `/Game/EasySurvivalRPG/Blueprints/Interfaces/BPI_Character.OverrideWalkSpeed_BPI` _returnvalue OverrideSpeed TargetSpeed 0.0))))

(event `TryClearSpawnPoints (Server)`
  (params (ClearPlacedOnly :type Boolean))
  ;[1 1 1] Spawn page debug events.
  (`self.ClearSpawnPoints` ClearPlacedOnly))

(event `TrySpawnRandomItem`
  ;[1 1 1] Items page debug events.
  (`self.TrySpawnRandomItem (Server)`))

(event `ClearContainer (Server)`
  (params (ContainerName :type Name))
  (bind _returnvalue (`Controller.K2_GetPawn` (`self.PlayerController`)))
  ;[1 1 1] Containers page debug events.
  (`/Engine/EditorBlueprintResources/StandardMacros.IsValid` _returnvalue
    (:`Is Valid`
      (bind (_inventory _equipment _hotbar) (message `/Game/EasySurvivalRPG/Blueprints/Interfaces/BPI_PlayerCharacter.GetPlayerContainers_BPI` _returnvalue))
      (switch `name` ContainerName
        (:`Inventory`
          (`/Game/EasySurvivalRPG/Blueprints/Components/BP_ContainerComponent.ClearItems` _inventory))
        (:`Equipment`
          (`/Game/EasySurvivalRPG/Blueprints/Components/BP_ContainerComponent.ClearItems` _equipment))
        (:`Hotbar`
          (`/Game/EasySurvivalRPG/Blueprints/Components/BP_ContainerComponent.ClearItems` _hotbar))))))

(event `TryClearCharacters`
  (params (GroupName :type Name))
  ;[1 1 1] Spawn page debug events.
  (`self.TryClearCharacters (Server)` GroupName))

(event `UpdateCharacterCustomization`
  (params (HairTypeIndex :type Integer) (HairColorIndex :type Integer) (PantsColorIndex :type Integer) (SkinColorIndex :type Integer))
  ;[1 1 1] Character page debug events.
  (`self.UpdateCharacterCustomization (Server)` HairTypeIndex HairColorIndex PantsColorIndex SkinColorIndex))

(event `TrySpawnRandomItem (Server)`
  ;[1 1 1] Items page debug events.
  (`self.SpawnRandomItem`))

(event `ClearContainers`
  ;[1 1 1] Containers page debug events.
  (`self.ClearContainers (Server)`))

(event `TryClearCharacters (Server)`
  (params (GroupName :type Name))
  ;[1 1 1] Spawn page debug events.
  (`self.ClearCharacters` GroupName))

(event `UpdateCharacterCustomization (Server)`
  (params (HairTypeIndex :type Integer) (HairColorIndex :type Integer) (PantsColorIndex :type Integer) (SkinColorIndex :type Integer))
  (bind _returnvalue (`Controller.K2_GetPawn` (`self.PlayerController`)))
  ;[1 1 1] Character page debug events.
  (`/Engine/EditorBlueprintResources/StandardMacros.IsValid` _returnvalue
    (:`Is Valid`
      (message `/Game/EasySurvivalRPG/Blueprints/Interfaces/BPI_PlayerCharacter.CustomizeCharacter_BPI` _returnvalue HairTypeIndex HairColorIndex PantsColorIndex SkinColorIndex))))

(event `ClearContainers (Server)`
  (bind _returnvalue (`Controller.K2_GetPawn` (`self.PlayerController`)))
  ;[1 1 1] Containers page debug events.
  (`/Engine/EditorBlueprintResources/StandardMacros.IsValid` _returnvalue
    (:`Is Valid`
      (bind (_inventory _equipment _hotbar) (message `/Game/EasySurvivalRPG/Blueprints/Interfaces/BPI_PlayerCharacter.GetPlayerContainers_BPI` _returnvalue))
      (`/Game/EasySurvivalRPG/Blueprints/Components/BP_ContainerComponent.ClearItems` _hotbar)
      (`/Game/EasySurvivalRPG/Blueprints/Components/BP_ContainerComponent.ClearItems` _equipment)
      (`/Game/EasySurvivalRPG/Blueprints/Components/BP_ContainerComponent.ClearItems` _inventory))))

(fn `AddCompanion`
  (params (Character :type "Character Object Reference"))
  (bind _returnvalue (`Controller.K2_GetPawn` (`self.PlayerController`)))
  ;[1 1 1] Add companion to player group.
  (`/Engine/EditorBlueprintResources/StandardMacros.IsValid` _returnvalue
    (:`Is Valid`
      (message `/Game/EasySurvivalRPG/Blueprints/Interfaces/BPI_Character.AddCompanionToGroup_BPI` _returnvalue Character)
      (message `/Game/EasySurvivalRPG/Blueprints/Interfaces/BPI_Character.SetOrderGuardTarget_BPI` Character _returnvalue)
      (`KismetArrayLibrary.Array_Add` (`self.SpawnedCompanions`) Character))))

(fn `ClearCharacters`
  (params (GroupName :type Name))
  (locals (LocalCharacters :type "Array of Character Object Reference"))
  ;[1 1 1] Clear characters in specific group.
  (switch `name` GroupName
    (:`All`
      (bind _outactors (`GameplayStatics.GetAllActorsOfClass` "/Script/Engine.Character"))
      (bind _output_get (set `local.LocalCharacters` _outactors)))
    (:`Spawned`
      (set `local.LocalCharacters` (`self.SpawnedCharacters`)))
    (:`Companions`
      (set `local.LocalCharacters` (`self.SpawnedCompanions`))))
  (for _array_element _output_get
    (if (not (`Pawn.IsPlayerControlled` _array_element))
      (`Actor.K2_DestroyActor` _array_element)))
  (`KismetArrayLibrary.Array_Clear` (`self.SpawnedCharacters`)))

(fn `ClearSpawnPoints`
  (params (ClearPlacedOnly :type Boolean))
  (locals (LocalSpawnPoints :type "Array of /Game/EasySurvivalRPG/Blueprints/Misc/NpcSystem/BP_SpawnPoint Object Reference"))
  ;[1 1 1] Clear spawn points on the level.
  (if (not ClearPlacedOnly)
    (bind _outactors (`GameplayStatics.GetAllActorsOfClass` "/Game/EasySurvivalRPG/Blueprints/Misc/NpcSystem/BP_SpawnPoint.BP_SpawnPoint_C"))
    (set `local.LocalSpawnPoints` _outactors)
    (else
      (bind _output_get (set `local.LocalSpawnPoints` (`self.PlacedSpawnPoints`)))))
  (for _array_element _output_get
    (`/Game/EasySurvivalRPG/Blueprints/Misc/NpcSystem/BP_SpawnPoint.DeactivateSpawnPoint` _array_element)
    (`Actor.K2_DestroyActor` _array_element))
  (`KismetArrayLibrary.Array_Clear` (`self.PlacedSpawnPoints`)))

(fn `CloseDebugMenu`
  (bind _debugmenuwidget (`self.DebugMenuWidget`))
  (bind _playercontroller (`self.PlayerController`))
  (bind _returnvalue (`Controller.K2_GetPawn` _playercontroller))
  ;[1 1 1] Try to close debug menu widget and update player input mode.
  (`/Engine/EditorBlueprintResources/StandardMacros.IsValid` _debugmenuwidget
    (:`Is Valid`
      (`/Game/EasySurvivalRPG/Blueprints/UserInterface/Debug/UI_DebugMenu.CloseDebugMenu` _debugmenuwidget)
      (set `self.MenuIsOpen` false)
      (set `PlayerController.bShowMouseCursor` false _playercontroller)
      (`WidgetBlueprintLibrary.SetInputMode_GameOnly` _playercontroller)
      (`/Engine/EditorBlueprintResources/StandardMacros.IsValid` _returnvalue
        (:`Is Valid`
          (`Actor.EnableInput` _returnvalue _playercontroller))))))

(fn `DebugMenuIsOpen`
  (returns (IsOpen :type Boolean))
  ;[1 1 1] Returns true if debug menu is open.
  (return (`self.MenuIsOpen`)))

(fn `InitComponent`
  (returns (Success :type Boolean))
  ;[1 1 1] Init debug menu component and set player controller reference.
  (bind `_as玩家控制器` (cast `PlayerController` (`self.GetOwner`))
    (:`then`
      (set `self.PlayerController` `_as玩家控制器`)
      (return true))
    (:`CastFailed`
      (`KismetSystemLibrary.PrintString` (`self.InitErrorMessage`) true true (struct :`R` 1.0 :`A` 1.0) 5.0)
      (return false))))

(fn `InitDebugMenuWidget`
  (returns (Success :type Boolean))
  (bind _playercontroller (`self.PlayerController`))
  ;[1 1 1] Create debug menu widget and add it to the viewport.
  (`/Engine/EditorBlueprintResources/StandardMacros.IsValid` _playercontroller
    (:`Is Valid`
      (if (`Controller.IsLocalPlayerController` _playercontroller)
        (`/Engine/EditorBlueprintResources/StandardMacros.IsValid` (`self.DebugMenuWidget`)
          (:`Is Valid`
            (return true))
          (:`Is Not Valid`
            (bind _returnvalue (`|CreateWidget` "/Game/EasySurvivalRPG/Blueprints/UserInterface/Debug/UI_DebugMenu.UI_DebugMenu_C" null self))
            (bind _output_get (set `self.DebugMenuWidget` _returnvalue))
            (`UserWidget.AddToViewport` _output_get 1)
            (`Widget.SetVisibility` _output_get "Hidden")
            (return true)))
        (else
          _)))
    (:`Is Not Valid`
      _))
  (return false))

(fn `OpenDebugMenu`
  (bind _debugmenuwidget (`self.DebugMenuWidget`))
  (bind _playercontroller (`self.PlayerController`))
  (bind _returnvalue (`Controller.K2_GetPawn` _playercontroller))
  ;[1 1 1] Try to open debug menu widget and update player input mode.
  (`/Engine/EditorBlueprintResources/StandardMacros.IsValid` _debugmenuwidget
    (:`Is Valid`
      (`/Game/EasySurvivalRPG/Blueprints/UserInterface/Debug/UI_DebugMenu.OpenDebugMenu` _debugmenuwidget :!label _label)
      (set `self.MenuIsOpen` true)
      (set `PlayerController.bShowMouseCursor` true _playercontroller)
      (`WidgetBlueprintLibrary.SetInputMode_GameAndUIEx` _playercontroller null)
      (`/Engine/EditorBlueprintResources/StandardMacros.IsValid` _returnvalue
        (:`Is Valid`
          (`Actor.DisableInput` _returnvalue _playercontroller)
          (message `/Game/EasySurvivalRPG/Blueprints/Interfaces/BPI_PlayerCharacter.Disable Inputs BPI` _returnvalue))))
    (:`Is Not Valid`
      (bind _success (`self.InitDebugMenuWidget`))
      (if _success
        (goto _label)))))

(fn `PlaceSpawnPoint`
  (params (SpawnLocation :type "Vector Structure") (SpawnSettings :type "/Game/EasySurvivalRPG/Blueprints/Structures/Misc/STR_SpawnSettings Structure") (DestroyAfterSpawn :type Boolean))
  (returns (SpawnedCharacters :type "Array of Character Object Reference"))
  (locals (LocalSpawnLocation :type "Vector Structure") (LocalSpawnSettings :type "/Game/EasySurvivalRPG/Blueprints/Structures/Misc/STR_SpawnSettings Structure" :default (struct :`SettingsHandle` (struct) :`SpawnRadius` 300.0 :`MaxSpawnCount` 1 :`InitialSpawnCount` 1 :`InitialSpawnMax` true :`RespawnTime` 5.0 :`RespawnCount` 1 :`MinCharacterLevel` 1 :`MaxCharacterLevel` 1 :`OverriddenLootList` (struct) :`SpawnFaction` "NewEnumerator0" :`SpawnRelationships` (struct) :`RelationshipsHandle` (struct))) (LocalDestroyAfterSpawn :type Boolean) (LocalSpawnPoint :type "/Game/EasySurvivalRPG/Blueprints/Misc/NpcSystem/BP_SpawnPoint Object Reference") (LocalSpawnedCharacters :type "Array of Character Object Reference"))
  (bind _localspawnpoint (`local.LocalSpawnPoint`))
  ;[1 1 1] Place spawn point and spawn characters.
  (bind _output_get (set `local.LocalSpawnLocation` SpawnLocation))
  (set `local.LocalSpawnSettings` SpawnSettings)
  (set `local.LocalDestroyAfterSpawn` DestroyAfterSpawn)
  (bind _returnvalue (`|SpawnActorFromClass` "/Game/EasySurvivalRPG/Blueprints/Misc/NpcSystem/BP_SpawnPoint.BP_SpawnPoint_C" (`KismetMathLibrary.MakeTransform` _output_get) "Undefined" "OverrideRootScale" null false null))
  (bind _output_get_2 (set `local.LocalSpawnPoint` _returnvalue))
  (`/Game/EasySurvivalRPG/Blueprints/Misc/NpcSystem/BP_SpawnPoint.SetSpawnSettings` _output_get_2 (`local.LocalSpawnSettings`))
  (`/Game/EasySurvivalRPG/Blueprints/Misc/NpcSystem/BP_SpawnPoint.InitSpawnPoint` _output_get_2)
  (`/Game/EasySurvivalRPG/Blueprints/Misc/NpcSystem/BP_SpawnPoint.ActivateSpawnPoint` _output_get_2)
  (set `local.LocalSpawnedCharacters` (`/Game/EasySurvivalRPG/Blueprints/Misc/NpcSystem/BP_SpawnPoint.SpawnedCharacters` _output_get_2))
  (if (`local.LocalDestroyAfterSpawn`)
    (`KismetArrayLibrary.Array_Append` (`self.SpawnedCharacters`) (`local.LocalSpawnedCharacters`))
    (`Actor.K2_DestroyActor` _localspawnpoint)
    (else
      (`KismetArrayLibrary.Array_Add` (`self.PlacedSpawnPoints`) _localspawnpoint)))
  (return (`local.LocalSpawnedCharacters`)))

(fn `SpawnItems`
  (params (Items :type "Array of /Game/EasySurvivalRPG/Blueprints/Structures/Items/STR_Item Structure") (Location :type "Vector Structure") (MinRange :type "Float (double-precision)") (MaxRange :type "Float (double-precision)") (MinHeight :type "Float (double-precision)") (MaxHeight :type "Float (double-precision)"))
  (bind _returnvalue (`KismetMathLibrary.RandomFloatInRange` MinRange MaxRange))
  (bind _returnvalue_2 (`KismetMathLibrary.RandomFloatInRange` MinRange MaxRange))
  ;[1 1 1] Spawn items at location with random offset.
  (for _array_element Items
    (for _array_element_2 (`/Game/EasySurvivalRPG/Blueprints/Game/Libraries/BP_ItemsLibrary.MakeItemsDataFromItem` _array_element)
      (if (`/Game/EasySurvivalRPG/Blueprints/Game/Libraries/BP_ItemsLibrary.ItemIsReal` _array_element_2)
        (`|SpawnActorFromClass` (`/Game/EasySurvivalRPG/Blueprints/Game/Libraries/BP_ItemsLibrary.GetItemClass` _array_element_2) (`KismetMathLibrary.MakeTransform` (+ Location (`KismetMathLibrary.MakeVector` (select `bool` (`KismetMathLibrary.RandomBool`) :`false` _returnvalue :`true` (* _returnvalue -1.0)) (select `bool` (`KismetMathLibrary.RandomBool`) :`false` _returnvalue_2 :`true` (* _returnvalue_2 -1.0)) (`KismetMathLibrary.RandomFloatInRange` MinHeight MaxHeight))) (`KismetMathLibrary.RandomRotator` false)) "AdjustIfPossibleButAlwaysSpawn" "SelectDefaultAtRuntime" null (`/Game/EasySurvivalRPG/Blueprints/Game/Libraries/BP_ItemsLibrary.GetItemHandle` _array_element_2) (`/Game/EasySurvivalRPG/Blueprints/Game/Libraries/BP_ItemsLibrary.GetItemAmount` _array_element_2) (`/Game/EasySurvivalRPG/Blueprints/Game/Libraries/BP_ItemsLibrary.GetItemCharges` _array_element_2) (`/Game/EasySurvivalRPG/Blueprints/Game/Libraries/BP_ItemsLibrary.GetItemDurability` _array_element_2) (`/Game/EasySurvivalRPG/Blueprints/Game/Libraries/BP_ItemsLibrary.GetItemDecay` _array_element_2) true true false null)))))

(fn `SpawnRandomItem`
  (locals (LocalItemID :type Name))
  (bind _returnvalue (`KismetMathLibrary.RandomFloatInRange` -150.0 150.0))
  (bind _returnvalue_2 (`Controller.K2_GetPawn` (`self.PlayerController`)))
  ;[1 1 1] Try to spawn random item from items data table.
  (`/Engine/EditorBlueprintResources/StandardMacros.IsValid` _returnvalue_2
    (:`Is Valid`
      (bind _outrownames (`DataTableFunctionLibrary.GetDataTableRowNames` "/Game/EasySurvivalRPG/Blueprints/DataTables/DT_Items.DT_Items"))
      (bind _output_get (set `local.LocalItemID` (`|GetArrayItem` _outrownames (`KismetMathLibrary.RandomIntegerInRange` 0 (- (`KismetArrayLibrary.Array_Length` _outrownames) 1)))))
      (bind _item (`/Game/EasySurvivalRPG/Blueprints/Game/Libraries/BP_ItemsLibrary.MakeItemByID` _output_get))
      (`|SpawnActorFromClass` "/Game/EasySurvivalRPG/Blueprints/InteractionObjects/Items/BP_Item.BP_Item_C" (`KismetMathLibrary.MakeTransform` (+ (`Actor.K2_GetActorLocation` _returnvalue_2) (`KismetMathLibrary.MakeVector` _returnvalue _returnvalue))) "Undefined" "OverrideRootScale" null (`/Game/EasySurvivalRPG/Blueprints/Game/Libraries/BP_ItemsLibrary.GetItemHandle` _item) (`/Game/EasySurvivalRPG/Blueprints/Game/Libraries/BP_ItemsLibrary.GetItemAmount` _item) -1 -1.0 -1.0 true true false null))))

(fn `TeleportToNextPlayerStart`
  (bind _playerstartindex (`self.PlayerStartIndex`))
  (bind _playerstartpoints (`self.PlayerStartPoints`))
  (bind _returnvalue (`Controller.K2_GetPawn` (`self.PlayerController`)))
  (bind _returnvalue_2 (+ (`self.PlayerStartIndex`) 1))
  ;[1 1 1] Teleport to location of next player start on the level.
  (if (`KismetArrayLibrary.Array_IsValidIndex` (`self.PlayerStartPoints`))
    (if (`KismetArrayLibrary.Array_IsValidIndex` (`self.PlayerStartPoints`) _returnvalue_2)
      (set `self.PlayerStartIndex` _returnvalue_2)
      (else
        (set `self.PlayerStartIndex` 0 :!label _label)))
    (else
      (bind _outactors (`GameplayStatics.GetAllActorsOfClass` "/Script/Engine.PlayerStart"))
      (set `self.PlayerStartPoints` _outactors)
      (goto _label)))
  (if (`KismetArrayLibrary.Array_IsValidIndex` _playerstartpoints _playerstartindex)
    (`/Engine/EditorBlueprintResources/StandardMacros.IsValid` _returnvalue
      (:`Is Valid`
        (`Actor.K2_SetActorLocation` _returnvalue (`Actor.K2_GetActorLocation` (`|GetArrayItem` _playerstartpoints _playerstartindex)) false true)))))

(fn `ToggleDebugMenu`
  ;[1 1 1] Open or close debug menu widget.
  (if (`self.MenuIsOpen`)
    (`self.CloseDebugMenu`)
    (else
      (`self.OpenDebugMenu`))))

(fn `TransitToLevel`
  (params (LevelName :type Name) (PointName :type Name) (SaveName :type Name))
  (locals (LocalLevelName :type Name) (LocalPointName :type Name) (LocalSaveName :type Name) (LocalPlayerManagerComponent :type "/Game/EasySurvivalRPG/Blueprints/Components/BP_PlayerManagerComponent Object Reference"))
  ;[1 1 1] Transit to specific level and save game to debug save slot.
  (set `local.LocalLevelName` LevelName)
  (set `local.LocalPointName` PointName)
  (set `local.LocalSaveName` SaveName)
  (bind _result (message `/Game/EasySurvivalRPG/Blueprints/Interfaces/BPI_GameInstance.IsSingleplayer_BPI` (`GameplayStatics.GetGameInstance`)))
  (if _result
    (bind _output_get (set `local.LocalPlayerManagerComponent` (`Actor.GetComponentByClass` (`self.GetOwner`) "/Game/EasySurvivalRPG/Blueprints/Components/BP_PlayerManagerComponent.BP_PlayerManagerComponent_C")))
    (`/Engine/EditorBlueprintResources/StandardMacros.IsValid` _output_get
      (:`Is Valid`
        (message `/Game/EasySurvivalRPG/Blueprints/Interfaces/BPI_GameInstance.SaveSingleplayerGame_BPI` (`GameplayStatics.GetGameInstance`) (`KismetStringLibrary.Conv_NameToString` (`local.LocalSaveName`)) (`/Game/EasySurvivalRPG/Blueprints/Components/BP_PlayerManagerComponent.GetPlayerSaveData` _output_get) (`|MakeArray`))
        (message `/Game/EasySurvivalRPG/Blueprints/Interfaces/BPI_GameInstance.TransitToLevel_BPI` (`GameplayStatics.GetGameInstance`) (`local.LocalLevelName`) (`local.LocalPointName`))))))

(fn `TryFindTraceHit`
  (returns (Found :type Boolean) (HitResult :type "HitResult Structure") (HitLocation :type "Vector Structure"))
  (bind _playercameramanager (`PlayerController.PlayerCameraManager` (`self.PlayerController`)))
  (bind _returnvalue (`PlayerCameraManager.GetCameraLocation` _playercameramanager))
  ;[1 1 1] Try find trace hit result by visibility channel.
  (bind (_outhit _returnvalue_2) (`KismetSystemLibrary.LineTraceSingle` _returnvalue (+ _returnvalue (* (`KismetMathLibrary.GetForwardVector` (`PlayerCameraManager.GetCameraRotation` _playercameramanager)) 3000.0)) "TraceTypeQuery1"))
  (if _returnvalue_2
    (return true _outhit (`.Location` (`GameplayStatics.BreakHitResult` _outhit)))
    (else
      (return false (struct) (0.0 0.0 0.0)))))