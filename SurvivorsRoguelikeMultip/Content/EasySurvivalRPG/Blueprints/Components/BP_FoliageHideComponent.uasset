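; Scene component that hides foliage around its owner, optionally hiding on BeginPlay and restoring on EndPlay.
; Bounds of tagged owner components, or its own location if none, define spheres scaled by per-HideLevel radius multipliers.
; It hides or shows instances in the foliage manager's instanced components.
; A sphere trace at the largest multiplier finds interaction foliage actors, then filters them by each level's radius.
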(event `self.ReceiveBeginPlay`
  ;[1 1 1] Begin play. Try to hide instances on begin play.
  (`self.InitComponent`)
  (if (`self.HideOnBeginPlay`)
    (`self.TryHideFoliage`)))

(event `self.ReceiveEndPlay`
  (params (EndPlayReason :type "EEndPlayReason Enum" :default "Destroyed"))
  ;[1 1 1] End play. Try to show hidden instances on end play.
  (if (`self.ShowOnEndPlay`)
    (`self.TryShowFoliage`)))

(fn `InitComponent`
  (returns (Success :type Boolean))
  (bind _collisioncomponenttag (`self.CollisionComponentTag`))
  ;[1 1 1] Init collision components.
  (if (!= _collisioncomponenttag "None")
    (set `self.CollisionComponents` (`Actor.GetComponentsByTag` (`self.GetOwner`) "/Script/Engine.SceneComponent" _collisioncomponenttag)))
  (return true))

(fn `TryHideDynamicFoliage`
  (returns (Success :type Boolean))
  (locals (LocalRadiusMultiplier :type "Float (double-precision)" :default 0.0) (LocalRadius :type "Float (double-precision)" :default 0.0) (LocalCenter :type "Vector Structure" :default (0.0 0.0 0.0)))
  (bind _collisioncomponents (`self.CollisionComponents`))
  ;[1 1 1] Try to hide dynamic foliage overlapped by bounds of collision components.
  (if (not (`self.FoliageAreHidden`))
    (bind _values (`BlueprintMapLibrary.Map_Values` (`self.HideLevelRadiuses`)))
    (set `local.LocalRadiusMultiplier` (`.MaxValue` (`KismetMathLibrary.MaxOfFloatArray` _values)))
    (if (`KismetArrayLibrary.Array_IsValidIndex` _collisioncomponents)
      (for _array_element _collisioncomponents
        (bind (_origin _boxextent _sphereradius) (`KismetSystemLibrary.GetComponentBounds` _array_element))
        (bind _output_get (set `local.LocalCenter` _origin))
        (set `local.LocalRadius` _sphereradius)
        (bind _outhits (`KismetSystemLibrary.SphereTraceMultiForObjects` _output_get _output_get (* (`local.LocalRadius`) (`local.LocalRadiusMultiplier`)) (`self.DynamicFoliageObjectTypes`) :!label _label))
        (for _array_element_2 _outhits
          (bind _asbp_interaction_foliage_base (cast `/Game/EasySurvivalRPG/Blueprints/InteractionObjects/Misc/BP_InteractionFoliage_Base` (`.HitActor` (`GameplayStatics.BreakHitResult` _array_element_2))))
          (bind _hidelevel (`/Game/EasySurvivalRPG/Blueprints/InteractionObjects/Misc/BP_InteractionFoliage_Base.HideLevel` _asbp_interaction_foliage_base))
          (bind (_value _returnvalue) (`BlueprintMapLibrary.Map_Find` (`self.HideLevelRadiuses`) _hidelevel))
          (if _returnvalue
            (if (<= (`KismetMathLibrary.VSize` (- (`local.LocalCenter`) (`Actor.K2_GetActorLocation` _asbp_interaction_foliage_base))) (* _value (`local.LocalRadius`)))
              (`/Game/EasySurvivalRPG/Blueprints/InteractionObjects/Misc/BP_InteractionFoliage_Base.TryHideFoliage` _asbp_interaction_foliage_base _hidelevel)))))
      (return true)
      (else
        (set `local.LocalCenter` (`self.K2_GetComponentLocation`))
        (`|ExecutionSequence`
          (:`then_0`
            (set `local.LocalRadius` 1.0)
            (goto _label))
          (:`then_1`
            (return true)))))
    (else
      (return false))))

(fn `TryHideFoliage`
  (returns (Success :type Boolean))
  (locals (LocalInstancedComponent :type "/Game/EasySurvivalRPG/Blueprints/Components/InstancedComponents/BP_InstancedComponent_Base Object Reference") (LocalHideLevel :type Integer) (LocalRadiusMultiplier :type "Float (double-precision)") (LocalCenter :type "Vector Structure" :default (0.0 0.0 0.0)) (LocalRadius :type "Float (double-precision)" :default 0.0))
  (bind _collisioncomponents (`self.CollisionComponents`))
  (bind _returnvalue (`Actor.GetComponentByClass` (`GameplayStatics.GetGameState`) "/Game/EasySurvivalRPG/Blueprints/Components/BP_FoliageManagerComponent.BP_FoliageManagerComponent_C"))
  (bind _foliageactor (`/Game/EasySurvivalRPG/Blueprints/Components/BP_FoliageManagerComponent.GetInstancedFoliageActor` _returnvalue))
  ;[1 1 1] Try to hide instances overlapped by bounds of collision components.
  (if (not (`self.FoliageAreHidden`))
    (`/Engine/EditorBlueprintResources/StandardMacros.IsValid` _returnvalue
      (:`Is Valid`
        (`/Engine/EditorBlueprintResources/StandardMacros.IsValid` _foliageactor
          (:`Is Valid`
            (for _array_element (`Actor.K2_GetComponentsByClass` _foliageactor "/Game/EasySurvivalRPG/Blueprints/Components/InstancedComponents/BP_InstancedComponent_Base.BP_InstancedComponent_Base_C")
              (bind _output_get (set `local.LocalInstancedComponent` _array_element))
              (bind _output_get_2 (set `local.LocalHideLevel` (`/Game/EasySurvivalRPG/Blueprints/Components/InstancedComponents/BP_InstancedComponent_Base.HideLevel` _output_get)))
              (bind (_value _returnvalue_2) (`BlueprintMapLibrary.Map_Find` (`self.HideLevelRadiuses`) _output_get_2))
              (if _returnvalue_2
                (set `local.LocalRadiusMultiplier` _value)
                (if (`KismetArrayLibrary.Array_IsValidIndex` _collisioncomponents)
                  (for _array_element_2 _collisioncomponents
                    (bind (_origin _boxextent _sphereradius) (`KismetSystemLibrary.GetComponentBounds` _array_element_2))
                    (set `local.LocalCenter` _origin)
                    (set `local.LocalRadius` _sphereradius)
                    (`/Game/EasySurvivalRPG/Blueprints/Components/InstancedComponents/BP_InstancedComponent_Base.HideInstancesInRadius` (`local.LocalInstancedComponent`) (`local.LocalCenter`) (* (`local.LocalRadius`) (`local.LocalRadiusMultiplier`)) (`local.LocalHideLevel`) :!label _label))
                  (else
                    (set `local.LocalCenter` (`self.K2_GetComponentLocation`))
                    (set `local.LocalRadius` 1.0)
                    (goto _label)))))
            (`self.TryHideDynamicFoliage`)
            (set `self.FoliageAreHidden` true)
            (return true))
          (:`Is Not Valid`
            _)))
      (:`Is Not Valid`
        _)))
  (return false))

(fn `TryShowDynamicFoliage`
  (returns (Success :type Boolean))
  (locals (LocalRadiusMultiplier :type "Float (double-precision)") (LocalCenter :type "Vector Structure") (LocalRadius :type "Float (double-precision)"))
  (bind _collisioncomponents (`self.CollisionComponents`))
  ;[1 1 1] Try to show dynamic foliage overlapped by bounds of collision components.
  (if (`self.FoliageAreHidden`)
    (bind _values (`BlueprintMapLibrary.Map_Values` (`self.HideLevelRadiuses`)))
    (set `local.LocalRadiusMultiplier` (`.MaxValue` (`KismetMathLibrary.MaxOfFloatArray` _values)))
    (if (`KismetArrayLibrary.Array_IsValidIndex` _collisioncomponents)
      (for _array_element _collisioncomponents
        (bind (_origin _boxextent _sphereradius) (`KismetSystemLibrary.GetComponentBounds` _array_element))
        (bind _output_get (set `local.LocalCenter` _origin))
        (set `local.LocalRadius` _sphereradius)
        (bind _outhits (`KismetSystemLibrary.SphereTraceMultiForObjects` _output_get _output_get (* (`local.LocalRadius`) (`local.LocalRadiusMultiplier`)) (`self.DynamicFoliageObjectTypes`) :!label _label))
        (for _array_element_2 _outhits
          (bind _asbp_interaction_foliage_base (cast `/Game/EasySurvivalRPG/Blueprints/InteractionObjects/Misc/BP_InteractionFoliage_Base` (`.HitActor` (`GameplayStatics.BreakHitResult` _array_element_2))))
          (bind _hidelevel (`/Game/EasySurvivalRPG/Blueprints/InteractionObjects/Misc/BP_InteractionFoliage_Base.HideLevel` _asbp_interaction_foliage_base))
          (bind (_value _returnvalue) (`BlueprintMapLibrary.Map_Find` (`self.HideLevelRadiuses`) _hidelevel))
          (if _returnvalue
            (if (<= (`KismetMathLibrary.VSize` (- (`local.LocalCenter`) (`Actor.K2_GetActorLocation` _asbp_interaction_foliage_base))) (* _value (`local.LocalRadius`)))
              (`/Game/EasySurvivalRPG/Blueprints/InteractionObjects/Misc/BP_InteractionFoliage_Base.TryShowFoliage` _asbp_interaction_foliage_base _hidelevel)))))
      (return true)
      (else
        (set `local.LocalCenter` (`self.K2_GetComponentLocation`))
        (`|ExecutionSequence`
          (:`then_0`
            (set `local.LocalRadius` 1.0)
            (goto _label))
          (:`then_1`
            (return true)))))
    (else
      (return false))))

(fn `TryShowFoliage`
  (returns (Success :type Boolean))
  (locals (LocalInstancedComponent :type "/Game/EasySurvivalRPG/Blueprints/Components/InstancedComponents/BP_InstancedComponent_Base Object Reference") (LocalHideLevel :type Integer :default 0) (LocalRadius :type "Float (double-precision)") (LocalRadiusMultiplier :type "Float (double-precision)") (LocalCenter :type "Vector Structure"))
  (bind _collisioncomponents (`self.CollisionComponents`))
  (bind _returnvalue (`Actor.GetComponentByClass` (`GameplayStatics.GetGameState`) "/Game/EasySurvivalRPG/Blueprints/Components/BP_FoliageManagerComponent.BP_FoliageManagerComponent_C"))
  (bind _foliageactor (`/Game/EasySurvivalRPG/Blueprints/Components/BP_FoliageManagerComponent.GetInstancedFoliageActor` _returnvalue))
  ;[1 1 1] Try to show instances overlapped by bounds of collision components.
  (if (`self.FoliageAreHidden`)
    (`/Engine/EditorBlueprintResources/StandardMacros.IsValid` _returnvalue
      (:`Is Valid`
        (`/Engine/EditorBlueprintResources/StandardMacros.IsValid` _foliageactor
          (:`Is Valid`
            (for _array_element (`Actor.K2_GetComponentsByClass` _foliageactor "/Game/EasySurvivalRPG/Blueprints/Components/InstancedComponents/BP_InstancedComponent_Base.BP_InstancedComponent_Base_C")
              (bind _output_get (set `local.LocalInstancedComponent` _array_element))
              (bind _output_get_2 (set `local.LocalHideLevel` (`/Game/EasySurvivalRPG/Blueprints/Components/InstancedComponents/BP_InstancedComponent_Base.HideLevel` _output_get)))
              (bind (_value _returnvalue_2) (`BlueprintMapLibrary.Map_Find` (`self.HideLevelRadiuses`) _output_get_2))
              (if _returnvalue_2
                (set `local.LocalRadiusMultiplier` _value)
                (if (`KismetArrayLibrary.Array_IsValidIndex` _collisioncomponents)
                  (for _array_element_2 _collisioncomponents
                    (bind (_origin _boxextent _sphereradius) (`KismetSystemLibrary.GetComponentBounds` _array_element_2))
                    (set `local.LocalCenter` _origin)
                    (set `local.LocalRadius` _sphereradius)
                    (`/Game/EasySurvivalRPG/Blueprints/Components/InstancedComponents/BP_InstancedComponent_Base.ShowInstancesInRadius` (`local.LocalInstancedComponent`) (`local.LocalCenter`) (* (`local.LocalRadius`) (`local.LocalRadiusMultiplier`)) (`local.LocalHideLevel`) :!label _label))
                  (else
                    (set `local.LocalCenter` (`self.K2_GetComponentLocation`))
                    (set `local.LocalRadius` 1.0)
                    (goto _label)))))
            (`self.TryShowDynamicFoliage`)
            (set `self.FoliageAreHidden` false)
            (return true))
          (:`Is Not Valid`
            _)))
      (:`Is Not Valid`
        _)))
  (return false))