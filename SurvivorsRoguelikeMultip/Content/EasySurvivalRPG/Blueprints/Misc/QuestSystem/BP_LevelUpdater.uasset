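; Level actor that manages save IDs for placed BPI_SaveData actors and keeps destroyed ones gone across save/load.
; Editor tools assign descending negative IDs, validate them, and reset or reassign them behind a confirmation flag.
; At BeginPlay it binds to those actors' OnDestroyed, saves the destroyed IDs, and destroys the matching actors on load.
; It also relays player level events and game tag updates through dispatchers; UpdatePlayerTags is an empty stub.
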(event `self.ReceiveBeginPlay`
  ;[1 1 1] Begin play. Bind OnDestroyed event for save actors.
  (if (< (`self.SaveID`) 0)
    (for _array_element (`self.UniqueSaveActors`)
      (`/Engine/EditorBlueprintResources/StandardMacros.IsValid` _array_element
        (:`Is Valid`
          (add `self.OnDestroyed` _array_element (`|CreateDelegate` :!event `OnSaveActorDestroyed`)))))
    (else
      (`KismetSystemLibrary.PrintText` (`|FormatText` "Unique save ID is not set! \nSelect the Level Updater actor and click the init button.") true true (struct :`R` 1.0 :`A` 1.0) 10.0))))

(event `OnSaveActorDestroyed` :!signature `self.OnDestroyed`
  (params (Actor :type "Actor Object Reference"))
  ;[1 1 1] Begin play. Bind OnDestroyed event for save actors.
  (bind (_success _saveid) (`/Game/EasySurvivalRPG/Blueprints/Game/Libraries/BP_SaveLibrary.TryToGetSaveID` Actor))
  (if _success
    (`KismetArrayLibrary.Array_Add` (`self.DestroyedSaveIDs`) _saveid)))

(event `ExecutePlayerLevelEvent`
  (params (PlayerController :type "PlayerController Object Reference") (EventName :type Name))
  ;[1 1 1] Execute player level event.
  (`self.OnPlayerEvent` PlayerController EventName))

(event `UpdateGameTags`
  (params (GameTags :type "GameplayTagContainer Structure"))
  ;[1 1 1] Update game tags event.
  (`self.OnUpdateGameTags` GameTags))

(event `UpdatePlayerTags`
  (params (PlayerController :type "PlayerController Object Reference") (PlayerTags :type "GameplayTagContainer Structure"))
  ;[1 1 1] 跟新标签事件
)

(fn `CheckUniqueSaveID`
  (params (Actor :type "Actor Object Reference"))
  (returns (Success :type Boolean))
  (locals (LocalActor :type "Actor Object Reference") (LocalIndex :type Integer) (LocalSaveID :type Integer))
  (bind _uniquesaveids (`self.UniqueSaveIDs`))
  (bind _returnvalue (`KismetArrayLibrary.Array_Find` (`self.UniqueSaveActors`) (`local.LocalActor`)))
  ;[1 1 1] Check that actor is correctly initialized with unique save id.
  (bind _output_get (set `local.LocalActor` Actor))
  (bind (_success _saveid) (`/Game/EasySurvivalRPG/Blueprints/Game/Libraries/BP_SaveLibrary.TryToGetSaveID` _output_get))
  (if _success
    (bind _output_get_2 (set `local.LocalIndex` _returnvalue))
    (if (`KismetArrayLibrary.Array_IsValidIndex` _uniquesaveids _returnvalue)
      (bind _output_get_3 (set `local.LocalSaveID` _saveid))
      (return (== _output_get_3 (`|GetArrayItem` _uniquesaveids _output_get_2)))
      (else
        _)))
  (return false))

(fn `CheckUniqueSaveIDs`
  (locals (LocalActor :type "Actor Object Reference"))
  ;[1 1 1] Check that all save actors have correct unique save IDs.
  (bind _outactors (`GameplayStatics.GetAllActorsWithInterface` "/Game/EasySurvivalRPG/Blueprints/Interfaces/BPI_SaveData.BPI_SaveData_C"))
  (for _array_element _outactors
    (bind _output_get (set `local.LocalActor` _array_element))
    (bind _success (`self.CheckUniqueSaveID` _output_get))
    (if (not _success)
      (set `self.TargetActor` (`local.LocalActor`))
      (`KismetSystemLibrary.PrintText` (`|FormatText` "Actor {ActorName} has wrong SaveID." (`KismetTextLibrary.Conv_StringToText` (`KismetSystemLibrary.GetDisplayName` _output_get))) true true (struct :`R` 1.0 :`A` 1.0) 10.0)
      (return)))
  (`KismetSystemLibrary.PrintText` (`|FormatText` "All save actors are initialized correctly!") true true (struct :`G` 1.0 :`A` 1.0) 10.0))

(fn `DoesIgnoreSaveLoad_BPI`
  (returns (Result :type Boolean))
  (return false))

(fn `GetComponentSaveID_BPI`
  (returns (Success :type Boolean) (ComponentSaveID :type Integer))
  (return false 0))

(fn `GetFormattedVariables_BPI`
  (returns (FormattedVariables :type "Array of String"))
  ;[1 1 1] Save destroyed save IDs.
  (return (`|MakeArray` (`/Game/EasySurvivalRPG/Blueprints/Game/Libraries/BP_SaveLibrary.FormatIntegerArrayToString` "DestroyedSaveIDs" (`self.DestroyedSaveIDs`)))))

(fn `GetSaveID_BPI`
  (returns (Success :type Boolean) (SaveID :type Integer))
  ;[1 1 1] Returns save ID of the actor.
  (return true (`self.SaveID`)))

(fn `InitUniqueSaveIDs`
  (locals (LocalCount :type Integer))
  ;[1 1 1] Try to init unique save IDs for all save actors on the level.
  (bind _saveactors (`/Game/EasySurvivalRPG/Blueprints/Game/Libraries/BP_SaveLibrary.FindAllSaveActors`))
  (for _array_element _saveactors
    (bind _success (`self.TryToSetUniqueSaveID` _array_element))
    (if _success
      (bind _output_get (set `local.LocalCount` (+ (stale _output_get) 1)))))
  (`KismetSystemLibrary.PrintText` (`|FormatText` "{Count} Save actors are initialized!" (`local.LocalCount`)) true true (struct :`G` 1.0 :`A` 1.0) 10.0))

(fn `LoadData_BPI`
  (params (SaveData :type "SaveGame Object Reference"))
  (returns (Success :type Boolean))
  (locals (LocalSaveData :type "SaveGame Object Reference"))
  ;[1 1 1] Load data and remove destroyed actors from the game.
  (bind _output_get (set `local.LocalSaveData` SaveData))
  (bind (_success _savedata) (message `/Game/EasySurvivalRPG/Blueprints/Interfaces/BPI_GameSave.GetActorSaveData_BPI` _output_get (`self.SaveID`)))
  (if _success
    (bind (_success_2 _saveids) (`/Game/EasySurvivalRPG/Blueprints/Game/Libraries/BP_SaveLibrary.GetFormattedIntegerArray` (`.FormattedVariables_38_8140374D4327F2E43E03C3B17B80F74B` (break `/Game/EasySurvivalRPG/Blueprints/Structures/SaveData/STR_SaveData_Actor` _savedata)) "DestroyedSaveIDs"))
    (if _success_2
      (bind _output_get_2 (set `self.DestroyedSaveIDs` _saveids))
      (for _array_element _output_get_2
        (bind (_success_3 _actor) (message `/Game/EasySurvivalRPG/Blueprints/Interfaces/BPI_GameSave.GetSavedActor_BPI` (`local.LocalSaveData`) _array_element))
        (`/Engine/EditorBlueprintResources/StandardMacros.IsValid` _actor
          (:`Is Valid`
            (`self.K2_DestroyActor` _actor))))
      (return true)
      (else
        _)))
  (return false))

(fn `ResetUniqueSaveIDs`
  (locals (LocalCount :type Integer))
  ;[1 1 1] Try to reset and init save IDs for all actors on the level. Use carefully.
  (if (`self.ReadyForConsequences`)
    (set `self.ReadyForConsequences` false)
    (set `self.LastUniqueSaveID` 0)
    (`KismetArrayLibrary.Array_Clear` (`self.UniqueSaveActors`))
    (`KismetArrayLibrary.Array_Clear` (`self.UniqueSaveIDs`))
    (bind _saveactors (`/Game/EasySurvivalRPG/Blueprints/Game/Libraries/BP_SaveLibrary.FindAllSaveActors`))
    (for _array_element _saveactors
      (`self.TryToSetUniqueSaveID` _array_element)
      (bind _output_get (set `local.LocalCount` (+ (stale _output_get) 1))))
    (`KismetSystemLibrary.PrintText` (`|FormatText` "Save IDs are reset!  \n{Count} Save actors are initialized!" (`local.LocalCount`)) true true (struct :`G` 1.0 :`A` 1.0) 10.0)
    (else
      (`KismetSystemLibrary.PrintText` (`|FormatText` "WARNING! Use carefully.  \nThis function reset save id for all save actors on the level! \nIt can affect on level save data.  \nIf you ready for concequences check the appropriated option.") true true (struct :`R` 1.0 :`G` 0.5 :`A` 1.0) 20.0))))

(fn `SaveData_BPI`
  (params (SaveData :type "SaveGame Object Reference"))
  (returns (Success :type Boolean))
  (locals (LocalSaveData :type "SaveGame Object Reference"))
  ;[1 1 1] Save data for the actor.
  (bind _formattedvariables (`/Game/EasySurvivalRPG/Blueprints/Interfaces/BPI_SaveData.GetFormattedVariables_BPI`))
  (bind _output_get (set `local.LocalSaveData` SaveData))
  (bind _success (message `/Game/EasySurvivalRPG/Blueprints/Interfaces/BPI_GameSave.SetActorSaveData_BPI` _output_get (`self.SaveID`) (make `/Game/EasySurvivalRPG/Blueprints/Structures/SaveData/STR_SaveData_Actor` (`GameplayStatics.GetObjectClass` self) (`self.GetTransform`) _formattedvariables)))
  (return _success))

(fn `SetSaveID_BPI`
  (params (SaveID :type Integer))
  (returns (Success :type Boolean))
  ;[1 1 1] Set save ID for the actor.
  (set `self.SaveID` SaveID)
  (return true))

(fn `TryToSetUniqueSaveID`
  (params (Actor :type "Actor Object Reference"))
  (returns (Success :type Boolean))
  (locals (LocalActor :type "Actor Object Reference") (LocalSaveID :type Integer))
  (bind _localsaveid (`local.LocalSaveID`))
  ;[1 1 1] Try to initialize actor with unique save ID.
  (bind _output_get (set `local.LocalActor` Actor))
  (if (`/Game/EasySurvivalRPG/Blueprints/Game/Libraries/BP_GameLibrary.RunInEditor`)
    (if (not (`KismetArrayLibrary.Array_Contains` (`self.UniqueSaveActors`) _output_get))
      (set `local.LocalSaveID` (- (`self.LastUniqueSaveID`) 1))
      (bind _success (`/Game/EasySurvivalRPG/Blueprints/Game/Libraries/BP_SaveLibrary.TryToSetSaveID` (`local.LocalActor`) (`local.LocalSaveID`)))
      (if _success
        (set `self.LastUniqueSaveID` _localsaveid)
        (`KismetArrayLibrary.Array_AddUnique` (`self.UniqueSaveActors`) (`local.LocalActor`))
        (`KismetArrayLibrary.Array_AddUnique` (`self.UniqueSaveIDs`) _localsaveid)
        (return true)
        (else
          (return false)))
      (else
        _)))
  (return false))

(fn `UpdateUniqueSaveID`
  (locals (LocalIndex :type Integer))
  (bind _localindex (`local.LocalIndex`))
  ;[1 1 1] Try to init save actor with new save ID. Use carefully.
  (`/Engine/EditorBlueprintResources/StandardMacros.IsValid` (`self.TargetActor`)
    (:`Is Valid`
      (if (`self.ReadyForConsequences`)
        (set `self.ReadyForConsequences` false)
        (bind _success (`self.CheckUniqueSaveID` (`self.TargetActor`)))
        (if _success
          (set `local.LocalIndex` (`KismetArrayLibrary.Array_Find` (`self.UniqueSaveActors`) (`self.TargetActor`)))
          (`KismetArrayLibrary.Array_Remove` (`self.UniqueSaveActors`) _localindex)
          (`KismetArrayLibrary.Array_Remove` (`self.UniqueSaveIDs`) _localindex)
          (`self.TryToSetUniqueSaveID` (`self.TargetActor`))
          (`KismetSystemLibrary.PrintText` (`|FormatText` "The target actor get new save ID!") true true (struct :`G` 1.0 :`A` 1.0) 10.0)
          (else
            (`KismetSystemLibrary.PrintText` (`|FormatText` "Target actor has wrong save ID!") true true (struct :`R` 1.0 :`A` 1.0) 10.0)))
        (else
          (`KismetSystemLibrary.PrintText` (`|FormatText` "WARNING! Use carefully.  \nThis function will update save of target actor! \nThe target actor will not be able to load it's data on game load.  \nIf you ready for concequences check the appropriated option.") true true (struct :`R` 1.0 :`G` 0.5 :`A` 1.0) 20.0))))))

(fn `UserConstructionScript`)