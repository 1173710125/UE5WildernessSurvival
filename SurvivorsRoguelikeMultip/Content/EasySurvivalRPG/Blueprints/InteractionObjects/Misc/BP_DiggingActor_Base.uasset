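; Base actor for diggable objects in EasySurvivalRPG, which destroys itself when the dig interface event fires.
; The construction script applies the StaticMesh variable to the Mesh component.
; It implements the save interface, writing its class, transform and formatted variables to the save data under its SaveID.
; LoadData only returns success, GetFormattedVariables supplies nothing of its own, and component save IDs are unsupported.
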(event `/Game/EasySurvivalRPG/Blueprints/Interfaces/BPI_DiggingActor.TryToDig_BPI`
  (params (Instigator :type "Controller Object Reference") (Value :type "Float (single-precision)"))
  ;[1 1 1] Interactions. Destroy actor when digged.
  (`self.K2_DestroyActor`))

(fn `DoesIgnoreSaveLoad_BPI`
  (returns (Result :type Boolean))
  (return false))

(fn `GetComponentSaveID_BPI`
  (returns (Success :type Boolean) (ComponentSaveID :type Integer))
  (return false 0))

(fn `GetFormattedVariables_BPI`
  (returns (FormattedVariables :type "Array of String"))
  (return))

(fn `GetSaveID_BPI`
  (returns (Success :type Boolean) (SaveID :type Integer))
  ;[1 1 1] Returns save ID.
  (return true (`self.SaveID`)))

(fn `LoadData_BPI`
  (params (SaveData :type "SaveGame Object Reference"))
  (returns (Success :type Boolean))
  ;[1 1 1] Load data for the actor.
  (return true))

(fn `SaveData_BPI`
  (params (SaveData :type "SaveGame Object Reference"))
  (returns (Success :type Boolean))
  (locals (LocalSaveData :type "SaveGame Object Reference"))
  ;[1 1 1] Save data for the actor.
  (bind _formattedvariables (`/Game/EasySurvivalRPG/Blueprints/Interfaces/BPI_SaveData.GetFormattedVariables_BPI`))
  (bind _output_get (set `local.LocalSaveData` SaveData))
  (message `/Game/EasySurvivalRPG/Blueprints/Interfaces/BPI_GameSave.SetActorSaveData_BPI` _output_get (`self.SaveID`) (make `/Game/EasySurvivalRPG/Blueprints/Structures/SaveData/STR_SaveData_Actor` (`GameplayStatics.GetObjectClass` self) (`self.GetTransform`) _formattedvariables))
  (return true))

(fn `SetSaveID_BPI`
  (params (SaveID :type Integer))
  (returns (Success :type Boolean))
  ;[1 1 1] Set save ID.
  (set `self.SaveID` SaveID)
  (return true))

(fn `UserConstructionScript`
  (`StaticMeshComponent.SetStaticMesh` (`self.Mesh`) (`self.StaticMesh`)))