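; BP_InteractionFoliage_Fern is an interactive fern foliage object that plays a rustling hit sound when something moving touches it.
; It extends a parent interaction foliage class and assigns its hit sound to the sound component during component initialization.
; On Hit, the sound plays only if it is not already playing, the fern is not hidden and the other actor has non-zero velocity.
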(event `self.ReceiveHit`
  (params (MyComp :type "PrimitiveComponent Object Reference") (Other :type "Actor Object Reference") (OtherComp :type "PrimitiveComponent Object Reference") (bSelfMoved :type Boolean) (HitLocation :type "Vector Structure") (HitNormal :type "Vector Structure") (NormalImpulse :type "Vector Structure") (Hit :type "HitResult Structure (by ref)"))
  ;[1 1 1] Play sound when someone interact with foliage.
  (if (not (`AudioComponent.IsPlaying` (`self.SoundComponent`)))
    (if (not (`self.IsHidden`))
      (if (> (`KismetMathLibrary.VSize` (`self.GetVelocity` Other)) 0.0)
        (`AudioComponent.Play` (`self.SoundComponent`) 0.0)))))

(fn `InitComponents`
  (returns (Success :type Boolean))
  ;[1 1 1] Init interaction foliage components.
  (`parent.InitComponents`)
  (`AudioComponent.SetSound` (`self.SoundComponent`) (`self.HitSound`))
  (return true))

(fn `UserConstructionScript`
  (`parent.UserConstructionScript`))