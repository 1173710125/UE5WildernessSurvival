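; BP_Boombox is an interactable boombox that fades in a music track and plays a dance-start animation on BeginPlay.
; It implements the interaction interface as "Disable" and also starts a one-shot 34-second timer.
; Releasing interact or taking any damage triggers a DoOnce shutdown.
; A multicast event fades out the audio and plays the dance-end animation, then the actor is destroyed after a short delay.
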(event `self.ReceiveBeginPlay`
  (bind _audio (`self.Audio`))
  ;[1 1 1] Begin play. Init and play music track.
  (`AudioComponent.SetSound` _audio (`self.Sound`))
  (`AudioComponent.FadeIn` _audio 0.44 1.0 0.0)
  (`AnimInstance.PlaySlotAnimationAsDynamicMontage` (`SkeletalMeshComponent.GetAnimInstance` (`self.SkeletalMesh`)) "/Game/EasySurvivalRPG/Meshes/SKMeshes/A_Boombox_Dance_Start.A_Boombox_Dance_Start" "DefaultSlot" 0.0 0.25 1.0 1 -1.0 0.0)
  (`KismetSystemLibrary.K2_SetTimerDelegate` (`|CreateDelegate` :!event `DisableBoombox`) 34.0))

(event `/Game/EasySurvivalRPG/Blueprints/Interfaces/BPI_InteractionObject.TryInteract_BPI`
  (params (Release :type Boolean) (PlayerController :type "PlayerController Object Reference"))
  ;[1 1 1] Disable boombox.
  (if Release
    (`self.DisableBoombox`)))

(event `self.ReceiveAnyDamage`
  (params (Damage :type "Float (single-precision)") (DamageType :type "DamageType Object Reference") (InstigatedBy :type "Controller Object Reference") (DamageCauser :type "Actor Object Reference"))
  ;[1 1 1] Disable boombox.
  (`self.DisableBoombox`))

(event `DisableBoombox`
  ;[1 1 1] Disable boombox.
  (`/Engine/EditorBlueprintResources/StandardMacros.DoOnce` false
    (:`Completed`
      (`self.DisableBoombox (Multicast)`)
      (`KismetSystemLibrary.Delay` 0.4)
      (`self.K2_DestroyActor`))))

(event `DisableBoombox (Multicast)`
  ;[1 1 1] Disable boombox.
  (`AudioComponent.FadeOut` (`self.Audio`) 0.4 0.0)
  (`AnimInstance.PlaySlotAnimationAsDynamicMontage` (`SkeletalMeshComponent.GetAnimInstance` (`self.SkeletalMesh`)) "/Game/EasySurvivalRPG/Meshes/SKMeshes/A_Boombox_Dance_End.A_Boombox_Dance_End" "DefaultSlot" 0.1 0.0 1.0 1 -1.0 0.0))

(fn `CheckCanInteract_BPI`
  (params (PlayerController :type "PlayerController Object Reference"))
  (returns (CanInteract :type Boolean))
  ;[1 1 1] Returns true if player can interact with the actor.
  (return true))

(fn `GetInteractionObjectName_BPI`
  (returns (Name :type Text))
  ;[1 1 1] Returns interaction object name.
  (return "Boombox"))

(fn `GetInteractionText_BPI`
  (params (PlayerController :type "PlayerController Object Reference"))
  (returns (InteractionText :type Text))
  ;[1 1 1] Returns interaction text.
  (return "Disable"))

(fn `IsTurnedOn_BPI`
  (returns (IsTurnedOn :type Boolean))
  (return false))

(fn `UserConstructionScript`)