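; Placeable spiked-wall gate building that players open and close, and that registers overlapping actors on its damage colliders.
; Interaction toggles GateIsOpened, whose OnRep plays or reverses a timeline swinging both leaves, while sounds are multicast.
; A BP_Building_Lock can attach to the lock socket; when locked, opening requires a successful TryQuickOpen, but closing is never blocked.
; The open state is saved and restored through the parent's formatted-variable save system.
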(event `/Game/EasySurvivalRPG/Blueprints/Interfaces/BPI_InteractionObject.TryInteract_BPI`
  (params (Release :type Boolean) (PlayerController :type "PlayerController Object Reference"))
  (bind _lockreference (`self.LockReference`))
  ;[1 1 1] Open / close gate interaction.
  (if Release
    (if (not (`self.GateIsOpened`))
      (`/Engine/EditorBlueprintResources/StandardMacros.IsValid` _lockreference
        (:`Is Valid`
          (if (`/Game/EasySurvivalRPG/Blueprints/InteractionObjects/BuildingObjects/Placeable/BP_Building_Lock.IsLocked` _lockreference)
            (bind _canopen (`/Game/EasySurvivalRPG/Blueprints/InteractionObjects/BuildingObjects/Placeable/BP_Building_Lock.TryQuickOpen` _lockreference PlayerController))
            (if _canopen
              (`self.OpenGate` :!label _label)
              (else
                (`self.PlaySound (Multicast)` (`self.LockedSound`))))
            (else
              (goto _label))))
        (:`Is Not Valid`
          (goto _label)))
      (else
        (`self.CloseGate`)))))

(event `PlayOpenGate`
  ;[1 1 1] Open and close gate.
  (bind (_direction _rotationz) (`Timeline|OpenGateTimeline` :!label _label_2)
    (:`Update`
      (`SceneComponent.K2_SetRelativeRotation` (`self.GateAxisB`) (`KismetMathLibrary.MakeRotator` 0.0 0.0 _rotationz) false true)
      (`SceneComponent.K2_SetRelativeRotation` (`self.GateAxisA`) (`KismetMathLibrary.MakeRotator` 0.0 0.0 (- 180.0 _rotationz)) false true))))

(event `self.TopDamageCollision2.OnComponentBeginOverlap`
  (params (OverlappedComponent :type "PrimitiveComponent Object Reference") (OtherActor :type "Actor Object Reference") (OtherComp :type "PrimitiveComponent Object Reference") (OtherBodyIndex :type Integer) (bFromSweep :type Boolean) (SweepResult :type "HitResult Structure (by ref)"))
  ;[1 1 1] Deal damage from top spikes.
  (`self.AddOverlappedActor` OtherActor))

(event `PlayCloseGate`
  ;[1 1 1] Open and close gate.
  (goto _label_2 :!via `Reverse`))

(event `self.TopDamageCollision2.OnComponentEndOverlap`
  (params (OverlappedComponent :type "PrimitiveComponent Object Reference") (OtherActor :type "Actor Object Reference") (OtherComp :type "PrimitiveComponent Object Reference") (OtherBodyIndex :type Integer))
  ;[1 1 1] Deal damage from top spikes.
  (`self.RemoveOverlappedActor` OtherActor))

(event `self.DamageCollisionB.OnComponentBeginOverlap`
  (params (OverlappedComponent :type "PrimitiveComponent Object Reference") (OtherActor :type "Actor Object Reference") (OtherComp :type "PrimitiveComponent Object Reference") (OtherBodyIndex :type Integer) (bFromSweep :type Boolean) (SweepResult :type "HitResult Structure (by ref)"))
  ;[1 1 1] Deal damage from top spikes.
  (`self.AddOverlappedActor` OtherActor))

(event `self.DamageCollisionB.OnComponentEndOverlap`
  (params (OverlappedComponent :type "PrimitiveComponent Object Reference") (OtherActor :type "Actor Object Reference") (OtherComp :type "PrimitiveComponent Object Reference") (OtherBodyIndex :type Integer))
  ;[1 1 1] Deal damage from top spikes.
  (`self.RemoveOverlappedActor` OtherActor))

(event `PlaySound (Multicast)`
  (params (Sound :type "SoundBase Object Reference"))
  ;[1 1 1] Play gate sounds.
  (`GameplayStatics.PlaySoundAtLocation` Sound (`self.K2_GetActorLocation`) (struct) 1.0 1.0 0.0 null null null null))

(event `self.DamageCollisionA.OnComponentBeginOverlap`
  (params (OverlappedComponent :type "PrimitiveComponent Object Reference") (OtherActor :type "Actor Object Reference") (OtherComp :type "PrimitiveComponent Object Reference") (OtherBodyIndex :type Integer) (bFromSweep :type Boolean) (SweepResult :type "HitResult Structure (by ref)"))
  ;[1 1 1] Deal damage from top spikes.
  (`self.AddOverlappedActor` OtherActor))

(event `self.DamageCollisionA.OnComponentEndOverlap`
  (params (OverlappedComponent :type "PrimitiveComponent Object Reference") (OtherActor :type "Actor Object Reference") (OtherComp :type "PrimitiveComponent Object Reference") (OtherBodyIndex :type Integer))
  ;[1 1 1] Deal damage from top spikes.
  (`self.RemoveOverlappedActor` OtherActor))

(fn `AttachTargetActorToSocket`
  (params (TargetActor :type "Actor Object Reference") (SocketName :type Name))
  (returns (Success :type Boolean))
  ;[1 1 1] Attach lock to the gate actor and set references.
  (bind _asbp_building_lock (cast `/Game/EasySurvivalRPG/Blueprints/InteractionObjects/BuildingObjects/Placeable/BP_Building_Lock` TargetActor)
    (:`then`
      (set `/Game/EasySurvivalRPG/Blueprints/InteractionObjects/BuildingObjects/Placeable/BP_Building_Lock.LockTargetReference` self _asbp_building_lock)
      (set `self.LockReference` _asbp_building_lock)
      (`self.K2_AttachToComponent` TargetActor (`self.LockSocket`) "None" "KeepWorld" "KeepWorld" "KeepWorld" true)
      (return true))
    (:`CastFailed`
      (return false))))

(fn `CheckCanInteract_BPI`
  (params (PlayerController :type "PlayerController Object Reference"))
  (returns (CanInteract :type Boolean))
  ;[1 1 1] Always allows interact with object.
  (return true))

(fn `CloseGate`
  ;[1 1 1] Close gate and update Is opened variables.
  (set `self.GateIsOpened` false)
  (`self.PlaySound (Multicast)` (`self.CloseGateSound`)))

(fn `GetFormattedVariables_BPI`
  (returns (FormattedVariables :type "Array of String"))
  ;[1 1 1] Save important variables.
  (bind _formattedvariables (`parent.GetFormattedVariables_BPI`))
  (`KismetArrayLibrary.Array_Append` _formattedvariables (`|MakeArray` (`/Game/EasySurvivalRPG/Blueprints/Game/Libraries/BP_SaveLibrary.FormatBooleanVariableToString` "GateIsOpened" (`self.GateIsOpened`))))
  (return _formattedvariables))

(fn `GetInteractionObjectName_BPI`
  (returns (Name :type Text))
  ;[1 1 1] Returns interaction object name.
  (return (`.Name_48_0C2E1CB24B48846B5E49308F12848518` (break `/Game/EasySurvivalRPG/Blueprints/Structures/BuildingSystem/STR_BuildingObjectSettings` (`self.BuildingObjectSettings`)))))

(fn `GetInteractionText_BPI`
  (params (PlayerController :type "PlayerController Object Reference"))
  (returns (InteractionText :type Text))
  ;[1 1 1] Returns interaction text.
  (return (select `bool` (`self.GateIsOpened`) :`false` "Open the gate" :`true` "Close the gate" :!type "Text")))

(fn `GetSocketTransform`
  (params (SocketName :type Name) (Index :type Integer))
  (returns (Transform :type "Transform Structure"))
  ;[1 1 1] Returns lock socket transform.
  (switch `name` SocketName
    (:`Default`
      (return (`parent.GetSocketTransform` SocketName Index)))
    (:`LockSocket`
      (return (`SceneComponent.K2_GetComponentToWorld` (`self.LockSocket`))))))

(fn `IsTurnedOn_BPI`
  (returns (IsTurnedOn :type Boolean))
  ;[1 1 1] Is not used.
  (return false))

(fn `LoadData_BPI`
  (params (SaveData :type "SaveGame Object Reference"))
  (returns (Success :type Boolean))
  ;[1 1 1] Load data for the gate.
  (bind _success (`parent.LoadData_BPI` SaveData))
  (bind (_success_2 _savedata) (message `/Game/EasySurvivalRPG/Blueprints/Interfaces/BPI_GameSave.GetActorSaveData_BPI` SaveData (`self.SaveID`)))
  (bind (_success_3 _value) (`/Game/EasySurvivalRPG/Blueprints/Game/Libraries/BP_SaveLibrary.GetFormattedVariableBooleanValue` (`.FormattedVariables_38_8140374D4327F2E43E03C3B17B80F74B` (break `/Game/EasySurvivalRPG/Blueprints/Structures/SaveData/STR_SaveData_Actor` _savedata)) "GateIsOpened"))
  (if _success_3
    (set `self.GateIsOpened` _value)
    (return _success)))

(fn `OnRep_GateIsOpened`
  ;[1 1 1] Play gate animation depending on DoorIsOpened variable.
  (if (`self.GateIsOpened`)
    (`self.PlayOpenGate`)
    (else
      (`self.PlayCloseGate`))))

(fn `OpenGate`
  ;[1 1 1] Open gate and update Is opened variables.
  (set `self.GateIsOpened` true)
  (`self.PlaySound (Multicast)` (`self.OpenGateSound`)))

(fn `UserConstructionScript`
  (`parent.UserConstructionScript`))