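; Base class for buildable traps that players can arm or disarm, with server-side state changes and an interaction cooldown.
; An overlap or optional damage trigger disarms the trap, plays multicast effects and fires after an optional delay.
; Activation swaps nearby instanced foliage trees for spawned trees, then sphere-traces for targets, applying status effects and randomized line-traced damage before optional self-destruction.
; Armed state and remaining block timers persist through save/load.
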(event `self.ReceiveBeginPlay`
  ;[1 1 1] Begin play. Try to arm trap on begin play.
  (`parent.ReceiveBeginPlay`)
  (`/Engine/EditorBlueprintResources/ActorMacros.Switch Has Authority`
    (:`Authority`
      (if (`self.Built`)
        (`|ExecutionSequence`
          (:`then_0`
            (if (`self.ArmOnBeginPlay`)
              (`self.SetArmedState` true)))
          (:`then_1`
            (`self.BlockActivation` (`self.InitialBlockActivationTime`))))))))

(event `PlayActivationEffects (Multicast)`
  (params (PreActivation :type Boolean))
  (bind _returnvalue (select `bool` PreActivation :`false` (`self.ActivationSound`) :`true` (`self.PreActivationSound`)))
  (bind _returnvalue_2 (select `bool` PreActivation :`false` (`self.ActivationParticle`) :`true` (`self.PreActivationParticle`)))
  ;[1 1 1] Trap effects.
  (`|ExecutionSequence`
    (:`then_0`
      (`/Engine/EditorBlueprintResources/StandardMacros.IsValid` _returnvalue
        (:`Is Valid`
          (`GameplayStatics.PlaySoundAtLocation` _returnvalue (`self.K2_GetActorLocation`) (struct) 1.0 1.0 0.0 null null null null))))
    (:`then_1`
      (`/Engine/EditorBlueprintResources/StandardMacros.IsValid` _returnvalue_2
        (:`Is Valid`
          (`GameplayStatics.SpawnEmitterAtLocation` _returnvalue_2 (`self.K2_GetActorLocation`) (`self.K2_GetActorRotation`)))))))

(event `PlayArmEffects (Multicast)`
  (bind _armsound (`self.ArmSound`))
  ;[1 1 1] Trap effects.
  (`/Engine/EditorBlueprintResources/StandardMacros.IsValid` _armsound
    (:`Is Valid`
      (`GameplayStatics.PlaySoundAtLocation` _armsound (`self.K2_GetActorLocation`) (struct) 1.0 1.0 0.0 null null null null))))

(event `/Game/EasySurvivalRPG/Blueprints/Interfaces/BPI_InteractionObject.TryInteract_BPI`
  (params (Release :type Boolean) (PlayerController :type "PlayerController Object Reference"))
  ;[1 1 1] Trap interaction events.
  (if Release
    (if (not (`self.IsInteractionBlocked`))
      (if (`self.IsArmed`)
        (if (`self.CanBeDisarmed`)
          (`self.TryDisarmTrap`))
        (elif (`self.CanBeArmed`)
          (`self.TryArmTrap`))))))

(event `PlayDisarmEffects (Multicast)`
  (bind _disarmsound (`self.DisarmSound`))
  ;[1 1 1] Trap effects.
  (`/Engine/EditorBlueprintResources/StandardMacros.IsValid` _disarmsound
    (:`Is Valid`
      (`GameplayStatics.PlaySoundAtLocation` _disarmsound (`self.K2_GetActorLocation`) (struct) 1.0 1.0 0.0 null null null null))))

(event `BlockInteractions`
  (params (Duration :type "Float (double-precision)" :default 1.0))
  ;[1 1 1] Trap interaction events.
  (set `self.IsInteractionBlocked` true)
  (if (> Duration 0.0)
    (bind _returnvalue (`KismetSystemLibrary.K2_SetTimerDelegate` (`|CreateDelegate` :!event `ResetBlockInteractions`) Duration))
    (set `self.BlockInteractionsTimer` _returnvalue)))

(event `ResetBlockInteractions`
  ;[1 1 1] Trap interaction events.
  (set `self.IsInteractionBlocked` false)
  (`KismetSystemLibrary.K2_ClearAndInvalidateTimerHandle` (`self.BlockInteractionsTimer`)))

(event `self.ActivationCollision.OnComponentBeginOverlap`
  (params (OverlappedComponent :type "PrimitiveComponent Object Reference") (OtherActor :type "Actor Object Reference") (OtherComp :type "PrimitiveComponent Object Reference") (OtherBodyIndex :type Integer) (bFromSweep :type Boolean) (SweepResult :type "HitResult Structure (by ref)"))
  ;[1 1 1] Trap activation events.
  (`/Engine/EditorBlueprintResources/ActorMacros.Switch Has Authority`
    (:`Authority`
      (if (not (`self.IsActivationBlocked`))
        (`self.TryActivateTrap`)))))

(event `BlockActivation`
  (params (Duration :type "Float (double-precision)" :default 1.0))
  ;[1 1 1] Trap activation events.
  (set `self.IsActivationBlocked` true)
  (if (> Duration 0.0)
    (bind _returnvalue (`KismetSystemLibrary.K2_SetTimerDelegate` (`|CreateDelegate` :!event `ResetBlockActivation`) Duration))
    (set `self.BlockActivationTimer` _returnvalue)))

(event `ResetBlockActivation`
  ;[1 1 1] Trap activation events.
  (set `self.IsActivationBlocked` false)
  (`KismetSystemLibrary.K2_ClearAndInvalidateTimerHandle` (`self.BlockActivationTimer`)))

(event `PlayActivationEffectsDelayed`
  (params (ActivationDelay :type "Float (double-precision)"))
  ;[1 1 1] Trap activation events.
  (`KismetSystemLibrary.Delay` ActivationDelay)
  (`self.PlayActivationEffects`))

(event `self.DamageTaken`
  (params (DamageData :type "/Game/EasySurvivalRPG/Blueprints/Structures/DamageSystem/STR_DamageData Structure (by ref)") (InstigatedBy :type "Controller Object Reference") (DamageCauser :type "Actor Object Reference") (HitInfo :type "HitResult Structure"))
  ;[1 1 1] Trap activation events.
  (`parent.DamageTaken` DamageData InstigatedBy DamageCauser HitInfo)
  (if (`self.ActivateOnDamageTaken`)
    (`/Engine/EditorBlueprintResources/StandardMacros.IsValid` self
      (:`Is Valid`
        (`self.TryActivateTrap`))
      (:`Is Not Valid`
        (`self.ActivateTrapImmediately`)))))

(fn `ActivateTrapImmediately`
  (returns (Success :type Boolean))
  (locals (LocalActor :type "Actor Object Reference") (LocalAffectedActors :type "Array of Actor Object Reference"))
  ;[1 1 1] Try to activate trap and play activation effects immediately.
  (if (`self.IsArmed`)
    (`self.SetArmedState` false)
    (`self.PlayActivationEffects`)
    (return true)
    (else
      (return false))))

(fn `CheckAndReplaceInstances`
  (returns (Success :type Boolean))
  (bind _returnvalue (`self.GetComponentByClass` (`GameplayStatics.GetGameState`) "/Game/EasySurvivalRPG/Blueprints/Components/BP_FoliageManagerComponent.BP_FoliageManagerComponent_C"))
  (bind _foliageactor (`/Game/EasySurvivalRPG/Blueprints/Components/BP_FoliageManagerComponent.GetInstancedFoliageActor` _returnvalue))
  ;[1 1 1] Check and replace foliage instances.
  (`/Engine/EditorBlueprintResources/StandardMacros.IsValid` _returnvalue
    (:`Is Valid`
      (`/Engine/EditorBlueprintResources/StandardMacros.IsValid` _foliageactor
        (:`Is Valid`
          (for _array_element (`self.K2_GetComponentsByClass` _foliageactor "/Game/EasySurvivalRPG/Blueprints/Components/InstancedComponents/BP_InstancedComponent_Tree_Base.BP_InstancedComponent_Tree_Base_C")
            (bind _returnarray (`/Game/EasySurvivalRPG/Blueprints/Components/InstancedComponents/BP_InstancedComponent_Base.GetInstancesInSphere` _array_element (`self.K2_GetActorLocation`) (`self.AreaOfEffect`)))
            (for _array_element_2 _returnarray
              (`/Game/EasySurvivalRPG/Blueprints/Components/InstancedComponents/BP_InstancedComponent_Tree_Base.SpawnTree` _array_element _array_element_2)))
          (return true))
        (:`Is Not Valid`
          _)))
    (:`Is Not Valid`
      _))
  (return false))

(fn `CheckCanInteract_BPI`
  (params (PlayerController :type "PlayerController Object Reference"))
  (returns (CanInteract :type Boolean))
  ;[1 1 1] Returns true if player can interact with trap.
  (if (not (`self.IsInteractionBlocked`))
    (if (`self.IsArmed`)
      (if (`self.CanBeDisarmed`)
        (return true)
        (else
          _))
      (elif (`self.CanBeArmed`)
        (return true)
        (else
          _))))
  (return false))

(fn `FindAffectedActors`
  (returns (Actors :type "Array of Actor Object Reference"))
  (locals (LocalAffectedActors :type "Array of Actor Object Reference"))
  (bind _returnvalue (`self.K2_GetActorLocation`))
  ;[1 1 1] Try to find affected actors depending on area of effect.
  (bind _outhits (`KismetSystemLibrary.SphereTraceMultiForObjects` _returnvalue _returnvalue (`self.AreaOfEffect`) (`self.AffectedObjectTypes`)))
  (for _array_element _outhits
    (`KismetArrayLibrary.Array_AddUnique` (`local.LocalAffectedActors`) (`.HitActor` (`GameplayStatics.BreakHitResult` _array_element))))
  (return (`local.LocalAffectedActors`)))

(fn `GetFormattedVariables_BPI`
  (returns (FormattedVariables :type "Array of String"))
  ;[1 1 1] Save trap variables.
  (bind _formattedvariables (`parent.GetFormattedVariables_BPI`))
  (`KismetArrayLibrary.Array_Append` _formattedvariables (`|MakeArray` (`/Game/EasySurvivalRPG/Blueprints/Game/Libraries/BP_SaveLibrary.FormatBooleanVariableToString` "IsArmed" (`self.IsArmed`)) (`/Game/EasySurvivalRPG/Blueprints/Game/Libraries/BP_SaveLibrary.FormatFloatVariableToString` "BlockInteractionsTime" (`KismetSystemLibrary.K2_GetTimerRemainingTimeHandle` (`self.BlockInteractionsTimer`))) (`/Game/EasySurvivalRPG/Blueprints/Game/Libraries/BP_SaveLibrary.FormatFloatVariableToString` "BlockActivationTime" (`KismetSystemLibrary.K2_GetTimerRemainingTimeHandle` (`self.BlockActivationTimer`)))))
  (return _formattedvariables))

(fn `GetInteractionObjectName_BPI`
  (returns (Name :type Text))
  ;[1 1 1] Returns trap name from the settings.
  (return (`.Name_48_0C2E1CB24B48846B5E49308F12848518` (break `/Game/EasySurvivalRPG/Blueprints/Structures/BuildingSystem/STR_BuildingObjectSettings` (`self.BuildingObjectSettings`)))))

(fn `GetInteractionText_BPI`
  (params (PlayerController :type "PlayerController Object Reference"))
  (returns (InteractionText :type Text))
  ;[1 1 1] Returns interaction text.
  (if (not (`self.IsInteractionBlocked`))
    (if (`self.IsArmed`)
      (if (`self.CanBeDisarmed`)
        (return "Try disarm trap")
        (else
          _))
      (elif (`self.CanBeArmed`)
        (return "Try arm trap")
        (else
          _))))
  (return ""))

(fn `IsTurnedOn_BPI`
  (returns (IsTurnedOn :type Boolean))
  (return true))

(fn `LoadData_BPI`
  (params (SaveData :type "SaveGame Object Reference"))
  (returns (Success :type Boolean))
  (locals (LocalIsArmed :type Boolean :default false) (LocalBlockInteractionTime :type "Float (double-precision)" :default 0.0) (LocalBlockActivationTime :type "Float (double-precision)" :default 0.0))
  (bind _localblockactivationtime (`local.LocalBlockActivationTime`))
  (bind _localblockinteractiontime (`local.LocalBlockInteractionTime`))
  ;[1 1 1] Load save data and update trap variables.
  (`parent.LoadData_BPI` SaveData)
  (bind (_success _savedata) (message `/Game/EasySurvivalRPG/Blueprints/Interfaces/BPI_GameSave.GetActorSaveData_BPI` SaveData (`self.SaveID`)))
  (bind ((`FormattedVariables_38_8140374D4327F2E43E03C3B17B80F74B` _formattedvariables)) (break `/Game/EasySurvivalRPG/Blueprints/Structures/SaveData/STR_SaveData_Actor` _savedata))
  (bind (_success_2 _value) (`/Game/EasySurvivalRPG/Blueprints/Game/Libraries/BP_SaveLibrary.GetFormattedVariableBooleanValue` _formattedvariables "IsArmed"))
  (bind (_success_3 _value_2) (`/Game/EasySurvivalRPG/Blueprints/Game/Libraries/BP_SaveLibrary.GetFormattedVariableFloatValue` _formattedvariables "BlockInteractionsTime"))
  (bind (_success_4 _value_3) (`/Game/EasySurvivalRPG/Blueprints/Game/Libraries/BP_SaveLibrary.GetFormattedVariableFloatValue` _formattedvariables "BlockActivationTime"))
  (if (and _success_2 _success_3 _success_4)
    (set `local.LocalIsArmed` _value)
    (set `local.LocalBlockInteractionTime` _value_2)
    (set `local.LocalBlockActivationTime` _value_3)
    (`|ExecutionSequence`
      (:`then_0`
        (if (> _localblockinteractiontime 0.0)
          (`self.BlockInteractions` _localblockinteractiontime)))
      (:`then_1`
        (`|ExecutionSequence`
          (:`then_0`
            (if (> _localblockactivationtime 0.0)
              (`self.BlockActivation` _localblockactivationtime)))
          (:`then_1`
            (`|ExecutionSequence`
              (:`then_0`
                (`self.SetArmedState` (`local.LocalIsArmed`)))
              (:`then_1`
                (return true)))))))))

(fn `OnRep_IsArmed`)

(fn `PlayActivationEffects`
  (returns (Success :type Boolean))
  (locals (LocalAffectedActors :type "Array of Actor Object Reference"))
  ;[1 1 1] Play activation effects and run actions for affected actors.
  (`self.PlayActivationEffects (Multicast)` false)
  (`|ExecutionSequence`
    (:`then_0`
      (`self.CheckAndReplaceInstances`)
      (bind _actors (`self.FindAffectedActors`))
      (bind _output_get (set `local.LocalAffectedActors` _actors))
      (for _array_element _output_get
        (`self.TryAffectActor` _array_element)))
    (:`then_1`
      (if (`self.DestroyOnActivate`)
        (`self.CompleteRemove` null true))
      (return true))))

(fn `PlayPreActivationEffects`
  (returns (Success :type Boolean))
  (locals (LocalAffectedActors :type "Array of Actor Object Reference"))
  ;[1 1 1] Play pre activation effects.
  (`self.PlayActivationEffects (Multicast)` true)
  (return true))

(fn `RandomizeDamage`
  (params (Damage :type "Float (double-precision)"))
  (returns (Result :type "Float (double-precision)"))
  ;[1 1 1] Randomize damage in range between min and max multipliers.
  (return (`KismetMathLibrary.RandomFloatInRange` (* Damage (`self.MinDamageMultiplier`)) (* Damage (`self.MaxDamageMultiplier`)))))

(fn `SetArmedState`
  (params (IsArmed :type Boolean))
  (returns (Success :type Boolean))
  ;[1 1 1] Set new armed state and update components.
  (bind _output_get (set `self.IsArmed` IsArmed))
  (`/Engine/EditorBlueprintResources/StandardMacros.IsValid` self
    (:`Is Valid`
      (`PrimitiveComponent.SetCollisionEnabled` (`self.ActivationCollision`) (select `bool` _output_get :`false` "NoCollision" :`true` "QueryOnly" :!type "ECollisionEnabled Enum")))
    (:`Is Not Valid`
      _))
  (return true))

(fn `TryActivateTrap`
  (returns (Success :type Boolean))
  (locals (LocalActor :type "Actor Object Reference") (LocalAffectedActors :type "Array of Actor Object Reference"))
  (bind _activationdelay (`self.ActivationDelay`))
  ;[1 1 1] Try activate trap and play activation effects.
  (if (`self.IsArmed`)
    (`self.SetArmedState` false)
    (`self.PlayPreActivationEffects`)
    (if (<= _activationdelay 0.0)
      (`self.PlayActivationEffects`)
      (else
        (`self.PlayActivationEffectsDelayed` _activationdelay)))
    (return true)
    (else
      (return false))))

(fn `TryAffectActor`
  (params (Actor :type "Actor Object Reference"))
  (returns (Success :type Boolean))
  (locals (LocalActor :type "Actor Object Reference"))
  ;[1 1 1] Apply damage and status effects to targets in the area.
  (set `local.LocalActor` Actor)
  (`|ExecutionSequence`
    (:`then_0`
      (for _array_element (`self.StatusEffects`)
        (`/Game/EasySurvivalRPG/Blueprints/Game/Libraries/BP_AbilitySystemLibrary.ApplyStatusEffectToActor` (`local.LocalActor`) _array_element (`self.GetInstigator`))))
    (:`then_1`
      (`|ExecutionSequence`
        (:`then_0`
          (`self.TryDealDamageToActor` (`local.LocalActor`)))
        (:`then_1`
          (return true))))))

(fn `TryArmTrap`
  (returns (Success :type Boolean))
  ;[1 1 1] Try arm trap and activate collision.
  (`/Engine/EditorBlueprintResources/ActorMacros.Switch Has Authority`
    (:`Authority`
      (`self.SetArmedState` true)
      (`self.PlayArmEffects (Multicast)`)
      (`self.BlockInteractions` (`self.InteractionCooldown`))
      (return true))))

(fn `TryDealDamageToActor`
  (params (Actor :type "Actor Object Reference"))
  (returns (Success :type Boolean))
  (locals (LocalActor :type "Actor Object Reference") (LocalHit :type "HitResult Structure"))
  ;[1 1 1] Try to deal damage to target actor.
  (bind _output_get (set `local.LocalActor` Actor))
  (`/Engine/EditorBlueprintResources/StandardMacros.IsValid` _output_get
    (:`Is Valid`
      (bind _outhits (`KismetSystemLibrary.LineTraceMultiForObjects` (`self.K2_GetActorLocation`) (`self.K2_GetActorLocation` _output_get) (`self.AffectedObjectTypes`)))
      (for _array_element _outhits
        (bind _output_get_2 (set `local.LocalHit` _array_element))
        (bind (_bblockinghit _binitialoverlap _time _distance _location _impactpoint _normal _impactnormal _physmat _hitactor) (`GameplayStatics.BreakHitResult` _array_element))
        (if (== (`local.LocalActor`) _hitactor)
          (bind _damagedata (`/Game/EasySurvivalRPG/Blueprints/Game/Libraries/BP_DamageSystemLibrary.MakeCommonDamageData` (`self.RandomizeDamage` (`self.Damage`)) (`self.DamageType`)))
          (`/Game/EasySurvivalRPG/Blueprints/Game/Libraries/BP_DamageSystemLibrary.ApplyAdvancedPointDamage` (`local.LocalActor`) _damagedata _normal _output_get_2 (`self.GetInstigatorController`) self)
          (return true)))
      (return false))))

(fn `TryDisarmTrap`
  (returns (Success :type Boolean))
  ;[1 1 1] Try disarm trap and deactivate collision.
  (`/Engine/EditorBlueprintResources/ActorMacros.Switch Has Authority`
    (:`Authority`
      (`self.SetArmedState` false)
      (`self.PlayDisarmEffects (Multicast)`)
      (`self.BlockInteractions` (`self.InteractionCooldown`))
      (return true))))

(fn `UserConstructionScript`
  (`parent.UserConstructionScript`))