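; Buildable mine trap for the survival building system, adding mesh and animation visuals on top of the logic inherited from its parent.
; BeginPlay shows the skeletal mesh when built, otherwise the static mesh.
; Multicast overrides for build completion, arm, disarm and pre-activation call the parent, then play slot animations as dynamic montages.
; Arming reuses the disarm animation played in reverse.
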(event `self.ReceiveBeginPlay`
  (bind _built (`self.Built`))
  ;[1 1 1] Begin play. Update visibility of meshes and activate trap.
  (`parent.ReceiveBeginPlay`)
  (`SceneComponent.SetVisibility` (`self.SkeletalMesh`) _built false)
  (`SceneComponent.SetVisibility` (`self.StaticMesh`) (not _built) false))

(event `self.CompleteBuild (Multicast)`
  (bind _returnvalue (`SkeletalMeshComponent.GetAnimInstance` (`self.SkeletalMesh`)))
  ;[1 1 1] Trap activation events. Play animations.
  (`parent.CompleteBuild (Multicast)`)
  (`/Engine/EditorBlueprintResources/StandardMacros.IsValid` _returnvalue
    (:`Is Valid`
      (`AnimInstance.PlaySlotAnimationAsDynamicMontage` _returnvalue (`self.SpawnAnimation`) "DefaultSlot" 0.0 0.0 1.0 1 -1.0 0.0))))

(event `self.PlayArmEffects (Multicast)`
  (bind _returnvalue (`SkeletalMeshComponent.GetAnimInstance` (`self.SkeletalMesh`)))
  ;[1 1 1] Trap activation events. Play animations.
  (`parent.PlayArmEffects (Multicast)`)
  (`/Engine/EditorBlueprintResources/StandardMacros.IsValid` _returnvalue
    (:`Is Valid`
      (`AnimInstance.PlaySlotAnimationAsDynamicMontage` _returnvalue (`self.DisarmAnimation`) "DefaultSlot" 0.0 0.0 -1.0 1 -1.0 0.0))))

(event `self.PlayDisarmEffects (Multicast)`
  (bind _returnvalue (`SkeletalMeshComponent.GetAnimInstance` (`self.SkeletalMesh`)))
  ;[1 1 1] Trap activation events. Play animations.
  (`parent.PlayDisarmEffects (Multicast)`)
  (`/Engine/EditorBlueprintResources/StandardMacros.IsValid` _returnvalue
    (:`Is Valid`
      (`AnimInstance.PlaySlotAnimationAsDynamicMontage` _returnvalue (`self.DisarmAnimation`) "DefaultSlot" 0.0 0.0 1.0 1 -1.0 0.0))))

(event `self.PlayActivationEffects (Multicast)`
  (params (PreActivation :type Boolean))
  (bind _returnvalue (`SkeletalMeshComponent.GetAnimInstance` (`self.SkeletalMesh`)))
  ;[1 1 1] Trap activation events. Play animations.
  (`parent.PlayActivationEffects (Multicast)` PreActivation)
  (if PreActivation
    (`/Engine/EditorBlueprintResources/StandardMacros.IsValid` _returnvalue
      (:`Is Valid`
        (`AnimInstance.PlaySlotAnimationAsDynamicMontage` _returnvalue (`self.ActivationAnimation`) "DefaultSlot" 0.0 0.0 1.0 1 -1.0 0.0)))))

(fn `UserConstructionScript`
  (`parent.UserConstructionScript`))