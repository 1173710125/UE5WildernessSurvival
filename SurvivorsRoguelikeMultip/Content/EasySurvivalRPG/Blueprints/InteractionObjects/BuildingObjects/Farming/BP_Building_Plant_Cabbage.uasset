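; Cabbage plant building object for the farming part of EasySurvivalRPG, with no active logic in its own graphs.
; Its interface events for turn-on, interaction and point damage are empty.
; The interface functions return defaults: interaction and turned-on checks are false, text is empty, and floor and save-ID calls report zero or failure.
; The construction script only calls the parent, and BeginPlay and Tick are disabled placeholders.
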(event `/Game/EasySurvivalRPG/Blueprints/Interfaces/BPI_InteractionObject.TryTurnOn_BPI`)

(event `/Game/EasySurvivalRPG/Blueprints/Interfaces/BPI_InteractionObject.TryInteract_BPI`
  (params (Release :type Boolean) (PlayerController :type "PlayerController Object Reference")))

(event `/Game/EasySurvivalRPG/Blueprints/Interfaces/BPI_DamageSystemActor.ApplyPointDamage_BPI`
  (params (DamageData :type "/Game/EasySurvivalRPG/Blueprints/Structures/DamageSystem/STR_DamageData Structure") (HitFromDirection :type "Vector Structure") (HitInfo :type "HitResult Structure") (EventInstigator :type "Controller Object Reference") (DamageCauser :type "Actor Object Reference")))

(fn `CheckCanInteract_BPI`
  (params (PlayerController :type "PlayerController Object Reference"))
  (returns (CanInteract :type Boolean))
  (return false))

(fn `GetComponentSaveID_BPI`
  (returns (Success :type Boolean) (ComponentSaveID :type Integer))
  (return false 0))

(fn `GetFloorNumber_BPI`
  (returns (FloorNumber :type Integer))
  (return 0))

(fn `GetFormattedVariables_BPI`
  (returns (FormattedVariables :type "Array of String"))
  (return))

(fn `GetInteractionText_BPI`
  (params (PlayerController :type "PlayerController Object Reference"))
  (returns (InteractionText :type Text))
  (return ""))

(fn `IsTurnedOn_BPI`
  (returns (IsTurnedOn :type Boolean))
  (return false))

(fn `SetFloorNumber_BPI`
  (params (FloorNumber :type Integer))
  (returns (Success :type Boolean))
  (return false))

(fn `UserConstructionScript`
  (`parent.UserConstructionScript`))