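; Buildable pig feeder for the farming system that holds feed in an item container players can open by interacting.
; When built, the server initializes the container and adds the starting feed.
; Slot changes update HasFood, whose RepNotify swaps the static mesh between full and empty versions.
; ConsumeFood removes one item from the first slot.
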(event `self.ReceiveBeginPlay`
  (bind _containercomponent (`self.ContainerComponent`))
  ;[1 1 1] Begin play. Update feeder mesh and add starting feed to the container.
  (`parent.ReceiveBeginPlay`)
  (`self.UpdateFeederMesh`)
  (if (`self.Built`)
    (`/Engine/EditorBlueprintResources/ActorMacros.Switch Has Authority`
      (:`Authority`
        (`/Game/EasySurvivalRPG/Blueprints/Components/BP_ContainerComponent.InitComponent` _containercomponent)
        (`/Game/EasySurvivalRPG/Blueprints/Components/BP_ContainerComponent.TryAddItemsOrDrop` _containercomponent (`/Game/EasySurvivalRPG/Blueprints/Game/Libraries/BP_ItemsLibrary.MakeLootItems` (`self.StartingFeedHandle`)))))))

(event `/Game/EasySurvivalRPG/Blueprints/Interfaces/BPI_InteractionObject.TryInteract_BPI`
  (params (Release :type Boolean) (PlayerController :type "PlayerController Object Reference"))
  ;[1 1 1] Interactions with feeder container.
  (if Release
    (message `/Game/EasySurvivalRPG/Blueprints/Interfaces/BPI_Player.OpenContainer_BPI` PlayerController (`self.ContainerComponent`))))

(event `self.ContainerComponent.OnSlotItemChanged`
  (params (Slot :type Integer) (Item :type "/Game/EasySurvivalRPG/Blueprints/Structures/Items/STR_ItemData Structure"))
  (bind _isvalid (`/Game/EasySurvivalRPG/Blueprints/Game/Libraries/BP_ItemsLibrary.ItemIsValid` Item))
  ;[1 1 1] Interactions with feeder container.
  (if (!= (`self.HasFood`) _isvalid)
    (set `self.HasFood` _isvalid)))

(fn `CheckCanInteract_BPI`
  (params (PlayerController :type "PlayerController Object Reference"))
  (returns (CanInteract :type Boolean))
  ;[1 1 1] Always allows interact with object.
  (return true))

(fn `ConsumeFood`
  ;[1 1 1] Consume food item in the pig feeder.
  (`/Game/EasySurvivalRPG/Blueprints/Components/BP_ContainerComponent.ConsumeItem` (`self.ContainerComponent`) 0 1))

(fn `GetInteractionObjectName_BPI`
  (returns (Name :type Text))
  ;[1 1 1] Returns interaction object name.
  (return (`.Name_48_0C2E1CB24B48846B5E49308F12848518` (break `/Game/EasySurvivalRPG/Blueprints/Structures/BuildingSystem/STR_BuildingObjectSettings` (`self.BuildingObjectSettings`)))))

(fn `GetInteractionText_BPI`
  (params (PlayerController :type "PlayerController Object Reference"))
  (returns (InteractionText :type Text))
  ;[1 1 1] Returns interaction text.
  (return (`.Name_48_0C2E1CB24B48846B5E49308F12848518` (break `/Game/EasySurvivalRPG/Blueprints/Structures/BuildingSystem/STR_BuildingObjectSettings` (`self.BuildingObjectSettings`)))))

(fn `IsTurnedOn_BPI`
  (returns (IsTurnedOn :type Boolean))
  ;[1 1 1] Is not used.
  (return false))

(fn `OnRep_HasFood`
  ;[1 1 1] Update feeder mesh when has food state is changed.
  (`self.UpdateFeederMesh`))

(fn `UpdateFeederMesh`
  ;[1 1 1] Update pig feeder mesh depending on has food state.
  (`StaticMeshComponent.SetStaticMesh` (`self.StaticMesh`) (select `bool` (`self.HasFood`) :`false` (`self.EmptyMesh`) :`true` (`self.FoodMesh`))))

(fn `UserConstructionScript`
  (`parent.UserConstructionScript`))