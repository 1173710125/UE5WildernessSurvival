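; Remote bomb projectile preset that turns into a placed building object where it hits.
; On an authority hit, it disables physics and collision, checks the hit, runs the replacement and destroys itself.
; The replacement spawns the class from the "Building" data table handle, attaches it to the hit component and bone, and passes it the instigator controller's remote key.
; The multicast hit effects event also aligns the projectile to the surface normal.
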(event `self.ReceiveHit`
  (params (MyComp :type "PrimitiveComponent Object Reference") (Other :type "Actor Object Reference") (OtherComp :type "PrimitiveComponent Object Reference") (bSelfMoved :type Boolean) (HitLocation :type "Vector Structure") (HitNormal :type "Vector Structure") (NormalImpulse :type "Vector Structure") (Hit :type "HitResult Structure (by ref)"))
  (bind _rootmeshcomponent (`self.RootMeshComponent`))
  ;[1 1 1] Hit event of projectile.
  (cast `Pawn` Other
    (:`then`
      _)
    (:`CastFailed`
      _))
  (`/Engine/EditorBlueprintResources/ActorMacros.Switch Has Authority`
    (:`Authority`
      (`PrimitiveComponent.SetSimulatePhysics` _rootmeshcomponent false)
      (`PrimitiveComponent.SetCollisionEnabled` _rootmeshcomponent "NoCollision")
      (`self.CheckHit` Hit)
      (`self.ReplaceToRemoteBuilding` Hit)
      (`self.K2_DestroyActor`))))

(event `self.PlayHitEffects (Multicast)`
  (params (HitSurface :type "EPhysicalSurface Enum" :default "SurfaceType_Default") (HitLocation :type "Vector Structure") (HitNormal :type "Vector Structure"))
  (bind _returnvalue (`self.GetTransform`))
  ;[1 1 1] Rotate projectile by hit surface normal.
  (`parent.PlayHitEffects (Multicast)` HitSurface HitLocation HitNormal)
  (`self.K2_SetActorRotation` (`KismetMathLibrary.TransformRotation` _returnvalue (`KismetMathLibrary.ComposeRotators` (`KismetMathLibrary.InverseTransformRotation` _returnvalue (`KismetMathLibrary.MakeRotFromZX` HitNormal (`self.GetActorForwardVector`))) (`KismetMathLibrary.MakeRotator` 0.0 -90.0))) true))

(event `ReplaceToRemoteBuilding`
  (params (HitResult :type "HitResult Structure"))
  (bind (_returnvalue_location _returnvalue_rotation _returnvalue_scale) (`KismetMathLibrary.BreakTransform` (`self.GetTransform`)))
  (bind (_bblockinghit _binitialoverlap _time _distance _location _impactpoint _normal _impactnormal _physmat _hitactor _hitcomponent _hitbonename) (`GameplayStatics.BreakHitResult` HitResult))
  (bind (_value _returnvalue) (`BlueprintMapLibrary.Map_Find` (`.Handles_44_8C993E244B07932FFEF6E1B1C39184F7` (break `/Game/EasySurvivalRPG/Blueprints/Structures/AbilitySystem/STR_ProjectileInstance` (`self.ProjectileSettings`))) "Building"))
  (bind (_datatable _rowname) (break `DataTableRowHandle` _value))
  ;[1 1 1] Replace projetile to building.
  (if _returnvalue
    (if (`/Game/EasySurvivalRPG/Blueprints/Game/Libraries/BP_GameLibrary.HandleIsValid` _value)
      (bind _returnvalue_2 (`|GetDataTableRow` _datatable _rowname)
        (:`then`
          (bind ((`Handle_65_2C8D1BB046C21623B1F418889A994FF0` _handle) (`Class_74_7F8BEA2E4BAD032DCA2206A1FED90A9B` _class)) (break `/Game/EasySurvivalRPG/Blueprints/Structures/BuildingSystem/STR_BuildingObjectSettings` _returnvalue_2))
          (bind _returnvalue_3 (`|SpawnActorFromClass` _class (`KismetMathLibrary.MakeTransform` (`.ImpactPoint` (`GameplayStatics.BreakHitResult` HitResult)) _returnvalue_rotation _returnvalue_scale) "AlwaysSpawn" "OverrideRootScale" null _handle true null))
          (`/Game/EasySurvivalRPG/Blueprints/InteractionObjects/BuildingObjects/Base/BP_Building_BaseObject.CheckAndAttachToComponent` _returnvalue_3 _hitcomponent _hitbonename)
          (bind (_success _remotekey) (message `/Game/EasySurvivalRPG/Blueprints/Interfaces/BPI_Remote.GetRemoteKey_BPI` (`self.GetInstigatorController`)))
          (if _success
            (message `/Game/EasySurvivalRPG/Blueprints/Interfaces/BPI_Remote.SetRemoteKey_BPI` _returnvalue_3 _remotekey)))))))

(fn `UserConstructionScript`
  (`parent.UserConstructionScript`))