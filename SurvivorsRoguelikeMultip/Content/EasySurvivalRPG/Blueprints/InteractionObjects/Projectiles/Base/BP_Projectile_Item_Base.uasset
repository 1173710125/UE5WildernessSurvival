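; Base projectile for launched items that can land in the world as a BP_Item actor.
; On begin play the server gets item data from the instigator through an interface, and the drop mesh's OnRep fills any unset collision and visual meshes.
; On hit the server applies flat or percentage durability loss, spawns the resulting item unless it broke and broken spawning is off, then runs CheckHit.
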(event `self.ReceiveBeginPlay`
  ;[1 1 1] Begin play. Try to init item drop mesh.
  (`parent.ReceiveBeginPlay`)
  (`/Engine/EditorBlueprintResources/ActorMacros.Switch Has Authority`
    (:`Authority`
      (bind (_success _itemdata) (message `/Game/EasySurvivalRPG/Blueprints/Interfaces/BPI_Character.GetLaunchItemData_BPI` (`self.GetInstigator`)))
      (if _success
        (bind _output_get (set `self.ItemData` _itemdata))
        (set `self.ItemDropMesh` (`/Game/EasySurvivalRPG/Blueprints/Game/Libraries/BP_ItemsLibrary.GetItemDropMesh` _output_get))))))

(event `self.ReceiveHit`
  (params (MyComp :type "PrimitiveComponent Object Reference") (Other :type "Actor Object Reference") (OtherComp :type "PrimitiveComponent Object Reference") (bSelfMoved :type Boolean) (HitLocation :type "Vector Structure") (HitNormal :type "Vector Structure") (NormalImpulse :type "Vector Structure") (Hit :type "HitResult Structure (by ref)"))
  ;[1 1 1] Hit event. Spawn item on hit.
  (`/Engine/EditorBlueprintResources/ActorMacros.Switch Has Authority`
    (:`Authority`
      (`self.TrySpawnItem`)
      (`self.CheckHit` Hit))))

(fn `OnRep_ItemDropMesh`
  ;[1 1 1] Update collision and projectile meshes.
  (`|ExecutionSequence`
    (:`then_0`
      (`/Engine/EditorBlueprintResources/StandardMacros.IsValid` (`self.CollisionMesh`)
        (:`Is Not Valid`
          (bind _output_get (set `self.CollisionMesh` (`self.ItemDropMesh`)))
          (`StaticMeshComponent.SetStaticMesh` (`self.RootMeshComponent`) _output_get))))
    (:`then_1`
      (`|ExecutionSequence`
        (:`then_0`
          (`/Engine/EditorBlueprintResources/StandardMacros.IsValid` (`self.StaticMesh`)
            (:`Is Not Valid`
              (bind _output_get_2 (set `self.StaticMesh` (`self.ItemDropMesh`)))
              (`StaticMeshComponent.SetStaticMesh` (`self.ProjectileMesh`) _output_get_2))))))))

(fn `TrySpawnItem`
  (returns (Success :type Boolean) (SpawnedItem :type "/Game/EasySurvivalRPG/Blueprints/InteractionObjects/Items/BP_Item Object Reference"))
  (bind _hitdurabilityloss (`self.HitDurabilityLoss`))
  ;[1 1 1] Decrease item durability and try to spawn item.
  (bind (_wasbroken _resultitem) (`/Game/EasySurvivalRPG/Blueprints/Game/Libraries/BP_ItemsLibrary.ChangeItemDurability` (`self.ItemData`) (* (select `bool` (`self.HitDurabilityLossPercent`) :`false` _hitdurabilityloss :`true` (* _hitdurabilityloss (`/Game/EasySurvivalRPG/Blueprints/Game/Libraries/BP_ItemsLibrary.GetItemMaxDurability` (`self.ItemData`)))) -1.0)))
  (if _wasbroken
    (if (`self.SpawnBrokenItem`)
      _
      (else
        (return false null))))
  (bind _returnvalue (`|SpawnActorFromClass` "/Game/EasySurvivalRPG/Blueprints/InteractionObjects/Items/BP_Item.BP_Item_C" (`SceneComponent.K2_GetComponentToWorld` (`self.ProjectileMesh`)) "AlwaysSpawn" "OverrideRootScale" null (`/Game/EasySurvivalRPG/Blueprints/Game/Libraries/BP_ItemsLibrary.GetItemHandle` _resultitem) (`/Game/EasySurvivalRPG/Blueprints/Game/Libraries/BP_ItemsLibrary.GetItemAmount` _resultitem) (`/Game/EasySurvivalRPG/Blueprints/Game/Libraries/BP_ItemsLibrary.GetItemCharges` _resultitem) (`/Game/EasySurvivalRPG/Blueprints/Game/Libraries/BP_ItemsLibrary.GetItemDurability` _resultitem) (`/Game/EasySurvivalRPG/Blueprints/Game/Libraries/BP_ItemsLibrary.GetItemDecay` _resultitem) true true false null))
  (return (`KismetSystemLibrary.IsValid` _returnvalue) _returnvalue))

(fn `UserConstructionScript`
  (`parent.UserConstructionScript`))