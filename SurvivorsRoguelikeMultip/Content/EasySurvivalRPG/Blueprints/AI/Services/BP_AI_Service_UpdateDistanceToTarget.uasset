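; Behavior tree service that keeps an AI pawn's distance to its target up to date in the blackboard.
; On each service tick it reads the TargetActorOrLocation key as an actor and measures that actor's distance to the controlled pawn.
; Without a valid actor it reads the same key as a vector and measures from the pawn's location, writing either result to the DistanceToTarget key.
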(event `self.ReceiveTickAI`
  (params (OwnerController :type "AIController Object Reference") (ControlledPawn :type "Pawn Object Reference") (DeltaSeconds :type "Float (single-precision)"))
  ;[1 1 1] Update distance to target actor on tick.
  (`self.UpdateDistanceToTarget` OwnerController ControlledPawn))

(fn `UpdateDistanceToTarget`
  (params (OwnerController :type "AIController Object Reference") (ControlledPawn :type "Pawn Object Reference"))
  (returns (Success :type Boolean))
  (locals (LocalOrderTarget :type "Actor Object Reference") (LocalTargetActor :type "Actor Object Reference"))
  (bind _distancetotarget (`self.DistanceToTarget`))
  (bind _targetactororlocation (`self.TargetActorOrLocation`))
  ;[1 1 1] Update distance to target actor blackboard value.
  (bind _output_get (set `local.LocalTargetActor` (`BTFunctionLibrary.GetBlackboardValueAsActor` _targetactororlocation)))
  (`/Engine/EditorBlueprintResources/StandardMacros.IsValid` _output_get
    (:`Is Valid`
      (`BTFunctionLibrary.SetBlackboardValueAsFloat` _distancetotarget (`Actor.GetDistanceTo` _output_get ControlledPawn)))
    (:`Is Not Valid`
      (`BTFunctionLibrary.SetBlackboardValueAsFloat` _distancetotarget (`KismetMathLibrary.VSize` (- (`BTFunctionLibrary.GetBlackboardValueAsVector` _targetactororlocation) (`Actor.K2_GetActorLocation` ControlledPawn))))))
  (return true))