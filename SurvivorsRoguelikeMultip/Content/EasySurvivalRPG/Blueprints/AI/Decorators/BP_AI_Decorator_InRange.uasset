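; Behavior tree decorator for AI that passes when the controlled pawn is within range of a blackboard target.
; It measures distance to the target actor, or to the target's vector location when no valid actor is set.
; The range comes from a fixed value, a blackboard float, or the sum of both, depending on two flags.
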(fn `GetTargetRange`
  (returns (AcceptanceRadius :type "Float (double-precision)"))
  (bind _range (`self.Range`))
  (bind _returnvalue (`BTFunctionLibrary.GetBlackboardValueAsFloat` (`self.BlackboardRange`)))
  ;[1 1 1] Returns target range value.
  (if (`self.UseBlackboardRange`)
    (return (select `bool` (`self.SumRangeValues`) :`false` _returnvalue :`true` (+ _range _returnvalue)))
    (else
      (return _range))))

(fn `PerformConditionCheckAI`
  (params (OwnerController :type "AIController Object Reference") (ControlledPawn :type "Pawn Object Reference"))
  (returns (ReturnValue :type Boolean))
  (bind _acceptanceradius (`self.GetTargetRange`))
  (bind _target (`self.Target`))
  (bind _returnvalue (`BTFunctionLibrary.GetBlackboardValueAsActor` _target))
  ;[1 1 1] Return true if target actor or location in range.
  (`/Engine/EditorBlueprintResources/StandardMacros.IsValid` _returnvalue
    (:`Is Valid`
      (return (<= (`Actor.GetDistanceTo` ControlledPawn _returnvalue) _acceptanceradius)))
    (:`Is Not Valid`
      (return (<= (`KismetMathLibrary.VSize` (- (`Actor.K2_GetActorLocation` ControlledPawn) (`BTFunctionLibrary.GetBlackboardValueAsVector` _target))) _acceptanceradius)))))