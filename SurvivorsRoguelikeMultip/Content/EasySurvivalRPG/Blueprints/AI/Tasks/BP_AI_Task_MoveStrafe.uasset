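; Behavior tree task that makes an AI pawn strafe around its blackboard target actor while keeping focus on it.
; It tests preset rotations around the target at the current distance plus per-step and optional rush offsets, flipping side after each failed candidate.
; The first navmesh-projected point passing trace and navigation raycast checks becomes the move destination.
; It fails only when no point is found, finishing successfully even if the move fails.
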(event `self.ReceiveExecuteAI`
  (params (OwnerController :type "AIController Object Reference") (ControlledPawn :type "Pawn Object Reference"))
  (bind _updatetargetlocation (`self.UpdateTargetLocation`))
  ;[1 1 1] Move strafe arount target actor.
  (set `self.OwnerController` OwnerController)
  (set `self.ControlledPawn` ControlledPawn)
  (`AIController.K2_SetFocus` OwnerController (`BTFunctionLibrary.GetBlackboardValueAsActor` (`self.TargetActor`)))
  (bind (_found _location) (`self.FindStrafeLocation`))
  (if _found
    (`BTFunctionLibrary.SetBlackboardValueAsVector` (`self.UpdateTargetLocation`) _location)
    (`|AIMoveTo` (`self.ControlledPawn`) _location null (`self.AcceptanceRadius`) true
      (:`OnSuccess`
        (`BTFunctionLibrary.ClearBlackboardValue` _updatetargetlocation))
      (:`OnFail`
        (`BTFunctionLibrary.ClearBlackboardValue` _updatetargetlocation)))
    (`self.FinishExecute` true)
    (else
      (`self.FinishExecute` false))))

(fn `FindStrafeLocation`
  (returns (Found :type Boolean) (Location :type "Vector Structure"))
  (locals (LocalCenterLocation :type "Vector Structure") (LocalPawnLocation :type "Vector Structure") (LocalTargetActor :type "Actor Object Reference") (LocalLookRotation :type "Rotator Structure") (LocalVectorLength :type "Float (double-precision)") (LocalTargetLocation :type "Vector Structure"))
  (bind _localcenterlocation (`local.LocalCenterLocation`))
  (bind _returnvalue (`BTFunctionLibrary.GetBlackboardValueAsActor` (`self.TargetActor`)))
  (bind _returnvalue_2 (`Actor.K2_GetActorLocation` (`self.ControlledPawn`)))
  ;[1 1 1] Try to find possible strafe location.
  (`/Engine/EditorBlueprintResources/StandardMacros.IsValid` _returnvalue
    (:`Is Valid`
      (set `local.LocalCenterLocation` (`Actor.K2_GetActorLocation` _returnvalue))
      (bind _output_get (set `local.LocalPawnLocation` _returnvalue_2))
      (set `local.LocalTargetActor` _returnvalue)
      (set `local.LocalLookRotation` (`KismetMathLibrary.MakeRotator` 0.0 0.0 (.yaw (`KismetMathLibrary.FindLookAtRotation` _localcenterlocation _output_get))))
      (set `local.LocalVectorLength` (`KismetMathLibrary.VSize` (- _returnvalue_2 _localcenterlocation)))
      (for (_array_element _array_index) (`self.StrafeRotations`)
        (bind _output_get_2 (set `local.LocalTargetLocation` (+ (`NavigationSystemV1.K2_ProjectPointToNavigation` (+ (* (`KismetMathLibrary.GetForwardVector` (`KismetMathLibrary.ComposeRotators` (`local.LocalLookRotation`) (select `bool` (`self.LastDirectionRight`) :`false` (`KismetMathLibrary.NegateRotator` _array_element) :`true` _array_element))) (+ (`local.LocalVectorLength`) (`|GetArrayItem` (`self.StrafeOffsets`) _array_index) (select `bool` (`self.Rush`) :`true` (`self.RushOffset`)))) (`local.LocalCenterLocation`))) (0.0 0.0 50.0))))
        (bind _result (`/Game/EasySurvivalRPG/Blueprints/Game/Libraries/BP_GameLibrary.CheckPathByTrace` (`self.ControlledPawn`) _output_get_2 25.0))
        (if _result
          (bind (_hitlocation _returnvalue_3) (`NavigationSystemV1.NavigationRaycast` (`local.LocalPawnLocation`) (`local.LocalTargetLocation`) null (`self.OwnerController`)))
          (if (not _returnvalue_3)
            (return true (`local.LocalTargetLocation`))
            (else
              _)))
        (set `self.LastDirectionRight` (not (`self.LastDirectionRight`))))
      (return false (0.0 0.0 0.0)))))