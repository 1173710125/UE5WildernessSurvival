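; BP_Character_Player_Survivor is a survivor player character Blueprint in EasySurvivalRPG that adds no gameplay logic of its own.
; Its construction script only calls the parent, and its BeginPlay, overlap and Tick events are disabled placeholders.
; The interface functions for menu preview, starting items, hair color, player ID and fishing state are stubs returning false, zero or empty values.
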(fn `AddStartingItems_BPI`
  (returns (Success :type Boolean))
  (return false))

(fn `GetFishingState_BPI`
  (returns (IsFishing :type Boolean))
  (return false))

(fn `GetHairColorIndexes_BPI`
  (returns (CurrentIndex :type Integer) (MaxIndex :type Integer))
  (return 0 0))

(fn `GetPlayerID_BPI`
  (returns (Success :type Boolean) (PlayerID :type String))
  (return false ""))

(fn `MenuPreviewMode_BPI`
  (returns (Success :type Boolean))
  (return false))

(fn `UserConstructionScript`
  (`parent.UserConstructionScript`))