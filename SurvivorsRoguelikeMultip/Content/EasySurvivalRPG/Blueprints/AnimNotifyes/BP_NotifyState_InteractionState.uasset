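; Anim notify state that marks the owning actor as being in a configurable interaction state during an animation window.
; It sets the state through a Blueprint interface message on begin and clears it on end, naming itself after the enum value.
; Each tick casts the owner to My_Character_shengchun and, if that succeeds, forces its 角色状态 (character state) to a fixed value and re-asserts the interaction state.
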(fn `GetNotifyName`
  (returns (ReturnValue :type String))
  (return (`KismetStringLibrary.Concat_StrStr` "InteractionState_" (`|GetEnumeratorNameAsString` (`self.InteractionState`)))))

(fn `Received_NotifyBegin`
  (params (MeshComp :type "SkeletalMeshComponent Object Reference") (Animation :type "AnimSequenceBase Object Reference") (TotalDuration :type "Float (single-precision)") (EventReference :type "AnimNotifyEventReference Structure (by ref)"))
  (returns (ReturnValue :type Boolean))
  ;[1 1 1] Set interaction state.
  (message `/Game/EasySurvivalRPG/Blueprints/Interfaces/BPI_Character.SetInteractionState_BPI` (`ActorComponent.GetOwner` MeshComp) (`self.InteractionState`) true)
  (return false))

(fn `Received_NotifyEnd`
  (params (MeshComp :type "SkeletalMeshComponent Object Reference") (Animation :type "AnimSequenceBase Object Reference") (EventReference :type "AnimNotifyEventReference Structure (by ref)"))
  (returns (ReturnValue :type Boolean))
  ;[1 1 1] Clear interaction state.
  (message `/Game/EasySurvivalRPG/Blueprints/Interfaces/BPI_Character.SetInteractionState_BPI` (`ActorComponent.GetOwner` MeshComp) (`self.InteractionState`) false)
  (return false))

(fn `Received_NotifyTick`
  (params (MeshComp :type "SkeletalMeshComponent Object Reference") (Animation :type "AnimSequenceBase Object Reference") (FrameDeltaTime :type "Float (single-precision)") (EventReference :type "AnimNotifyEventReference Structure (by ref)"))
  (returns (ReturnValue :type Boolean))
  (bind _returnvalue (`ActorComponent.GetOwner` MeshComp))
  ;[1 1 1] Check and set interaction state by tick.
  (bind _asmy_character (cast `/Game/my_game/Blueprints/My_Character_shengchun` _returnvalue))
  (set `/Game/my_game/Blueprints/My_Character_shengchun.角色状态` "NewEnumerator4" _asmy_character)
  (message `/Game/EasySurvivalRPG/Blueprints/Interfaces/BPI_Character.SetInteractionState_BPI` _returnvalue (`self.InteractionState`) true)
  (return false))