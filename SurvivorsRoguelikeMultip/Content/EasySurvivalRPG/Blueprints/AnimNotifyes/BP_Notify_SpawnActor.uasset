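; Anim notify that spawns an actor of a configured class near the animated mesh's owner, on the server only and outside the editor.
; An optional sphere trace around the owner skips the spawn if an actor of that class is already in range.
; Otherwise, a line trace at random pitch and yaw offsets from the owner's facing picks the hit point, where the actor spawns yawed toward the owner plus a relative rotation.
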(fn `CheckSpawnedActor`
  (params (Owner :type "Actor Object Reference"))
  (returns (Spawned :type Boolean))
  (bind _returnvalue (`Actor.K2_GetActorLocation` Owner))
  ;[1 1 1] Returns true if sphere trace hit actor of specific class in specific range.
  (bind _outhits (`KismetSystemLibrary.SphereTraceMultiForObjects` _returnvalue _returnvalue (`self.CheckSpawnedActorsRange`) (`self.CheckSpawnedActorsTypes`)))
  (for _array_element _outhits
    (if (`KismetMathLibrary.ClassIsChildOf` (`GameplayStatics.GetObjectClass` (`.HitActor` (`GameplayStatics.BreakHitResult` _array_element))) (`self.SpawnClass`))
      (return true)))
  (return false))

(fn `Received_Notify`
  (params (MeshComp :type "SkeletalMeshComponent Object Reference") (Animation :type "AnimSequenceBase Object Reference"))
  (returns (ReturnValue :type Boolean))
  (bind _returnvalue (`ActorComponent.GetOwner` MeshComp))
  ;[1 1 1] Try to spawn actor on the server.
  (if (not (`/Game/EasySurvivalRPG/Blueprints/Game/Libraries/BP_GameLibrary.RunInEditor`))
    (if (`KismetSystemLibrary.IsServer`)
      (if (`self.CheckSpawnedActors`)
        (bind _spawned (`self.CheckSpawnedActor` _returnvalue)))
      (if (not _spawned)
        (`self.SpawnActor` _returnvalue)
        (return true)))))

(fn `SpawnActor`
  (params (Owner :type "Actor Object Reference"))
  (locals (LocalActorsToIgnore :type "Array of Actor Object Reference") (LocalOwnerLocation :type "Vector Structure" :default (0.0 0.0 0.0)) (LocalOwner :type "Actor Object Reference"))
  (bind (_returnvalue_roll _returnvalue_pitch _returnvalue_yaw) (`KismetMathLibrary.BreakRotator` (`Actor.K2_GetActorRotation` Owner)))
  (bind _localownerlocation (`local.LocalOwnerLocation`))
  (bind _owner (`local.Owner`))
  ;[1 1 1] Spawn actor of specific class near the owner actor.
  (bind _output_get (set `local.LocalOwner` Owner))
  (set `local.LocalOwnerLocation` (`Actor.K2_GetActorLocation` Owner))
  (bind _output_get_2 (set `local.LocalActorsToIgnore` (`Actor.GetAttachedActors` _output_get)))
  (`KismetArrayLibrary.Array_Add` _output_get_2 (`local.LocalOwner`))
  (bind (_outhit _returnvalue) (`KismetSystemLibrary.LineTraceSingle` _localownerlocation (+ _localownerlocation (* (`KismetMathLibrary.GetForwardVector` (`KismetMathLibrary.MakeRotator` 0.0 (`KismetMathLibrary.RandomFloatInRange` (`self.MinPitchAngle`) (`self.MaxPitchAngle`)) (+ _returnvalue_yaw (`KismetMathLibrary.RandomFloatInRange` (`self.MinAdditionalYaw`) (`self.MaxAdditionalYaw`))))) (`self.TraceDistance`))) "TraceTypeQuery1" false (`local.LocalActorsToIgnore`)))
  (if _returnvalue
    (bind (_bblockinghit _binitialoverlap _time _distance _location) (`GameplayStatics.BreakHitResult` _outhit))
    (bind (_returnvalue_roll_2 _returnvalue_pitch_2 _returnvalue_yaw_2) (`KismetMathLibrary.BreakRotator` (`KismetMathLibrary.FindLookAtRotation` _location (`local.LocalOwnerLocation`))))
    (`|SpawnActorFromClass` (`self.SpawnClass`) (`KismetMathLibrary.MakeTransform` _location (`KismetMathLibrary.ComposeRotators` (`KismetMathLibrary.MakeRotator` 0.0 0.0 _returnvalue_yaw_2) (`self.SpawnRelativeRotation`))) "AdjustIfPossibleButAlwaysSpawn" "OverrideRootScale" _owner (`Actor.Instigator` _owner))))