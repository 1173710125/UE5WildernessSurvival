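; Animation notify state that marks a window in which a named interaction can continue.
; On begin, it sends a ContinueInteraction interface message to the mesh owner, adding its InteractionName and InteractionHandle to the continue interaction list.
; On end, it sends the same message to remove that interaction from the list.
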(fn `GetNotifyName`
  (returns (ReturnValue :type String))
  (return "ContinueInteraction"))

(fn `Received_NotifyBegin`
  (params (MeshComp :type "SkeletalMeshComponent Object Reference") (Animation :type "AnimSequenceBase Object Reference") (TotalDuration :type "Float (double-precision)"))
  (returns (ReturnValue :type Boolean))
  ;[1 1 1] Add interaction to the continue interaction list.
  (message `/Game/EasySurvivalRPG/Blueprints/Interfaces/BPI_PlayerCharacter.ContinueInteraction_BPI` (`ActorComponent.GetOwner` MeshComp) (`self.InteractionName`) (`self.InteractionHandle`) true)
  (return false))

(fn `Received_NotifyEnd`
  (params (MeshComp :type "SkeletalMeshComponent Object Reference") (Animation :type "AnimSequenceBase Object Reference"))
  (returns (ReturnValue :type Boolean))
  ;[1 1 1] Remove interaction from the continue interaction list.
  (message `/Game/EasySurvivalRPG/Blueprints/Interfaces/BPI_PlayerCharacter.ContinueInteraction_BPI` (`ActorComponent.GetOwner` MeshComp) (`self.InteractionName`) (`self.InteractionHandle`) false)
  (return false))