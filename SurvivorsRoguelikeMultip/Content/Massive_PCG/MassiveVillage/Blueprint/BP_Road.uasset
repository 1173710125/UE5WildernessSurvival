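; Spline-based road actor for the Massive Village PCG toolset, driven by a PCG graph.
; On construction it passes a valid RoadList to the PCG graph instance and places the billboard above the spline's middle point.
; DestroyRoad deletes directly attached actors, anything tracked in AllActors, then the road itself.
; The village data lookup and WaterLevel hookup are disconnected, so that step does nothing.
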(fn ConstructionScript
  (CallFunction|GetMassiveVillageData)
  (CallFunction|UpdateRoadData)
  (CallFunction|UpdateBillboard))

(fn DestroyRoad
  (for _array_element (Actor|GetAttachedActors true false)
    (Utilities|Array|AddUnique (LocalVariables|GetAllActors) _array_element))
  (for _array_element_2 (LocalVariables|GetAllActors)
    (Actor|DestroyActor _array_element_2))
  (Actor|DestroyActor))

(fn GetMassiveVillageData
  (return))

(fn UpdateRoadData
  (bind _roadlist (Variables|Default|GetRoadList)
    (:then
      (Audio|Parameter|SetObjectParameter (Variables|/Script/PCG.PCGComponent|GetGraphInstance (Variables|Default|GetPCG)) "RoadList" _roadlist)
      (return))
    (:else)))

(fn UpdateBillboard
  (bind _spline (Variables|Default|GetSpline))
  (Transformation|SetWorldLocation (Variables|Default|GetBillboard) (+ (Spline|GetLocationatSplinePoint _spline (/ (Spline|GetNumberOfSplinePoints _spline) 2) "World") "0.000000,0.000000,800.000000") false false))