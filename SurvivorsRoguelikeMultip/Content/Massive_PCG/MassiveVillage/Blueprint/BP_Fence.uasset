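; BP_Fence is a spline-based fence actor for MassiveVillage that drives a PCG graph.
; On construction it passes fence and optional pole mesh lists to the graph, with segment lengths derived from each first mesh's clamped X bounds.
; It also floats a billboard above the spline's middle point.
; DestroyFence removes attached actors and itself; the village water-level lookup is disconnected, leaving that function empty.
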(fn ConstructionScript
  (CallFunction|GetMassiveVillageData)
  (CallFunction|UpdateFenceData)
  (CallFunction|UpdateBillboard))

(fn DestroyFence
  (for _array_element (Actor|GetAttachedActors true false)
    (Utilities|Array|AddUnique (LocalVariables|GetAllActors) _array_element))
  (for _array_element_2 (LocalVariables|GetAllActors)
    (Actor|DestroyActor _array_element_2))
  (Actor|DestroyActor))

(fn GetMassiveVillageData
  (return))

(fn UpdateFenceData
  (bind _fencelist (Variables|Default|GetFenceList)
    (:then
      (bind _structout (Utilities|Struct|SetmembersinST_Object (Utilities|Array|Get(acopy) (Variables|/Game/Massive_PCG/MassiveVillage/Data/Structure/PDA_VillageObject.PDA_VillageObject_C|GetMeshes _fencelist)))))
    (:else
      _))
  (Effects|Components|ParticleSystem|SetFloatParameter (Variables|/Script/PCG.PCGComponent|GetGraphInstance (Variables|Default|GetPCG)) "VillageFenceLength" (Math|Float|Clamp(Float) (* (.x (.boxextent (StaticMesh|GetBounds (.mesh _structout)))) 2.0) 25.0 1e+03))
  (Audio|Parameter|SetObjectParameter (Variables|/Script/PCG.PCGComponent|GetGraphInstance (Variables|Default|GetPCG)) "FenceList" (Variables|Default|GetFenceList))
  (if (Variables|Default|GetAddPoleToFence?)
    (bind _polelist (Variables|Default|GetPoleList)
      (:then
        (bind _structout_2 (Utilities|Struct|SetmembersinST_Object (Utilities|Array|Get(acopy) (Variables|/Game/Massive_PCG/MassiveVillage/Data/Structure/PDA_VillageObject.PDA_VillageObject_C|GetMeshes _polelist)))))
      (:else
        _))
    (Effects|Components|ParticleSystem|SetFloatParameter (Variables|/Script/PCG.PCGComponent|GetGraphInstance (Variables|Default|GetPCG)) "PoleLength" (Math|Float|Clamp(Float) (* (.x (.boxextent (StaticMesh|GetBounds (.mesh _structout_2)))) 2.0) 1e+01 1e+04))
    (bind _polelist_2 (Variables|Default|GetPoleList)
      (:then
        (Audio|Parameter|SetObjectParameter (Variables|/Script/PCG.PCGComponent|GetGraphInstance (Variables|Default|GetPCG)) "PoleList" _polelist_2))
      (:else
        _))
    (return)
    (else
      (return))))

(fn UpdateBillboard
  (bind _spline (Variables|Default|GetSpline))
  (Transformation|SetWorldLocation (Variables|Default|GetBillboard) (+ (Spline|GetLocationatSplinePoint _spline (/ (Spline|GetNumberOfSplinePoints _spline) 2) "World") "0.000000,0.000000,800.000000") false false))