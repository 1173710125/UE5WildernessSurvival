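; BP_Door is a door actor that swings open and closed.
; Each Open/CloseDoor call alternates through a FlipFlop, playing a timeline forward from start or in reverse from end to lerp the mesh's yaw between closed and open.
; A separate UpdateDoorMesh function picks the exterior or interior mesh from the IsExit flag when that mesh is valid, and is not called within this Blueprint.
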(event `Open / Close Door`
  (`/Engine/EditorBlueprintResources/StandardMacros.FlipFlop`
    (:`A`
      (bind (_direction _doortimerfloat) (`Timeline|Timeline_0` :!via `PlayFromStart` :!label _label)
        (:`Update`
          (`SceneComponent.K2_SetRelativeRotation` (`self.StaticMesh`) (`KismetMathLibrary.MakeRotator` 0.0 0.0 (`KismetMathLibrary.Lerp` 0.0 80.0 _doortimerfloat)) false false))))
    (:`B`
      (goto _label :!via `ReverseFromEnd`))))

(fn `Update Door Mesh`
  (if (`self.isExit?`)
    (bind _doorexterior (`self.DoorExterior`)
      (:`then`
        (`StaticMeshComponent.SetStaticMesh` (`self.StaticMesh`) _doorexterior))
      (:`else`))
    (else
      (bind _doorinterior (`self.DoorInterior`)
        (:`then`
          (`StaticMeshComponent.SetStaticMesh` (`self.StaticMesh`) _doorinterior))
        (:`else`)))))

(fn `UserConstructionScript`
  (`parent.UserConstructionScript`))