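; Editor drag tool that lets a designer draw spawner override areas for enemies, NPCs and animals in the level.
; Dragging traces from the cursor, recording points at a set spacing and marking them with temporary debug spheres.
; On release it spawns a BP_SpawnerOverride at their centroid, builds its spline, copies the tool's spawner settings and triggers PCG generation.
; Settings persist between sessions through a saved property set.
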(event EventOnScriptSetup
  (bind _returnvalue (CallFunction|AddPropertySetOfType 0 "OverrideSpawnerSettings")
    (:Success
      (bind _asbp_spawner_override_property (Utilities|Casting|CastTo _returnvalue))
      (bind _output_get (Variables|Default|SetSpawner%20Property _asbp_spawner_override_property))
      (CallFunction|RestorePropertySetSettings _output_get "OverrideSpawnerSettings")
      (Variables|Default|SetbWantMouseHover true)
      (CallFunction|GetActortoIgnore))))

(event EventOnScriptShutdown
  (params (ShutdownType :type EToolShutdownType%20Enum :default "Completed"))
  (CallFunction|SavePropertySetSettings (Variables|Default|GetSpawner%20Property) "OverrideSpawnerSettings")
  (Variables|Default|SetbWantMouseHover false))

(event EventOnDragUpdatePosition
  (params (NewPosition :type Input%20Device%20Ray%20Structure) (Modifiers :type %20Structure%20%28by%20ref%29))
  (bind _worldray (Utilities|Struct|BreakInputDeviceRay NewPosition))
  (bind _worldray_2 (Utilities|Struct|BreakInputDeviceRay (Utilities|Struct|MakeInputDeviceRay _worldray false "(X=0.000000,Y=0.000000)")))
  (bind _outhit (Collision|LineTraceByChannel (.origin _worldray_2) (+ (.origin _worldray_2) (* (.direction _worldray_2) 5e+05)) "TraceTypeQuery1" false (Variables|Default|GetActors%20to%20Ignore) "None" true "(R=1.000000,G=0.000000,B=0.403293,A=1.000000)"))
  (if (>= (Math|Vector|Distance2D(Vector) (.location _outhit) (Variables|Default|GetLastDistancePosition)) (Variables|Default|GetPointDistance))
    (bind _returnvalue (Game|SpawnActorfromClass "/Game/Massive_PCG/MassiveShared/Blueprint/Editor/BP_DebugSphere.BP_DebugSphere_C" (Math|Transform|MakeTransform (.location _outhit) "0, 0, 0" "2.000000,2.000000,2.000000") "AlwaysSpawn" "MultiplyWithRoot" 0 0))
    (Utilities|Array|AddUnique (Variables|Default|GetAllDebug) _returnvalue)
    (bind _output_get (Variables|Default|SetLastDistancePosition (.location _outhit)))
    (Utilities|Array|Add (Variables|Default|GetAllPoints) _output_get)))

(event EventOnDragBegin
  (params (StartPosition :type Input%20Device%20Ray%20Structure) (Modifiers :type %20Structure%20%28by%20ref%29))
  (bind _worldray (Utilities|Struct|BreakInputDeviceRay StartPosition))
  (bind _worldray_2 (Utilities|Struct|BreakInputDeviceRay (Utilities|Struct|MakeInputDeviceRay _worldray false "(X=0.000000,Y=0.000000)")))
  (Variables|Default|SetbWantMouseHover false)
  (Utilities|Array|Clear (Variables|Default|GetAllPoints))
  (Variables|Default|SetPointDistance (Variables|Default|GetPointDistance (Variables|Default|GetSpawner%20Property)))
  (bind _outhit (Collision|LineTraceByChannel (.origin _worldray_2) (+ (.origin _worldray_2) (* (.direction _worldray_2) 5e+05)) "TraceTypeQuery1" false (Variables|Default|GetActors%20to%20Ignore) "None" true "(R=1.000000,G=0.000000,B=0.403293,A=1.000000)"))
  (bind _output_get (Variables|Default|SetLastDistancePosition (.location _outhit)))
  (Utilities|Array|Add (Variables|Default|GetAllPoints) _output_get)
  (bind _returnvalue (Game|SpawnActorfromClass "/Game/Massive_PCG/MassiveShared/Blueprint/Editor/BP_DebugSphere.BP_DebugSphere_C" (Math|Transform|MakeTransform _output_get "0, 0, 0" "2.000000,2.000000,2.000000") "AlwaysSpawn" "MultiplyWithRoot" 0 0))
  (Utilities|Array|AddUnique (Variables|Default|GetAllDebug) _returnvalue))

(event EventOnDragEnd
  (params (EndPosition :type Input%20Device%20Ray%20Structure) (Modifiers :type %20Structure%20%28by%20ref%29))
  (bind _spawner_property (Variables|Default|GetSpawner%20Property))
  (bind _alldebug (Variables|Default|GetAllDebug))
  (Variables|Default|SetbWantMouseHover true)
  (Variables|Default|SetAllPointsDistance "0, 0, 0")
  (for _array_element (Variables|Default|GetAllPoints)
    (Variables|Default|SetAllPointsDistance (+ _array_element (Variables|Default|GetAllPointsDistance))))
  (bind _returnvalue (Game|SpawnActorfromClass "/Game/Massive_PCG/MassiveShared/Blueprint/BP_SpawnerOverride.BP_SpawnerOverride_C" (Math|Transform|MakeTransform (/ (Variables|Default|GetAllPointsDistance) (Utilities|Array|Length (Variables|Default|GetAllPoints))) "0, 0, 0" "1.000000,1.000000,1.000000") "AlwaysSpawn" "MultiplyWithRoot" 0 0))
  (bind _output_get (Variables|Default|SetActor _returnvalue))
  (Spline|ClearSplinePoints (Variables|/Game/Massive_PCG/MassiveShared/Blueprint/BP_SpawnerOverride.BP_SpawnerOverride_C|GetSpline _output_get) true)
  (for _array_element_2 (Variables|Default|GetAllPoints)
    (Spline|AddSplinePoint (Variables|/Game/Massive_PCG/MassiveShared/Blueprint/BP_SpawnerOverride.BP_SpawnerOverride_C|GetSpline _output_get) _array_element_2 "World" false))
  (Spline|UpdateSpline (Variables|/Game/Massive_PCG/MassiveShared/Blueprint/BP_SpawnerOverride.BP_SpawnerOverride_C|GetSpline _output_get))
  (for _array_element_3 _alldebug
    (Actor|DestroyActor _array_element_3))
  (Utilities|Array|Clear _alldebug)
  (CallFunction|GetActortoIgnore)
  (Variables|/Game/Massive_PCG/MassiveShared/Blueprint/BP_SpawnerOverride.BP_SpawnerOverride_C|SetShowSpawner (Variables|Default|GetActor) (Variables|Default|GetShowSpawner _spawner_property))
  (Variables|/Game/Massive_PCG/MassiveShared/Blueprint/BP_SpawnerOverride.BP_SpawnerOverride_C|SetSpawn%20Enemy? (Variables|Default|GetActor) (Variables|Default|GetSpawn%20Enemy? _spawner_property))
  (Variables|/Game/Massive_PCG/MassiveShared/Blueprint/BP_SpawnerOverride.BP_SpawnerOverride_C|SetSpawn%20NPC? (Variables|Default|GetActor) (Variables|Default|GetSpawn%20NPC? _spawner_property))
  (Variables|/Game/Massive_PCG/MassiveShared/Blueprint/BP_SpawnerOverride.BP_SpawnerOverride_C|SetSpawn%20Animal? (Variables|Default|GetActor) (Variables|Default|GetSpawn%20Animal? _spawner_property))
  (Variables|/Game/Massive_PCG/MassiveShared/Blueprint/BP_SpawnerOverride.BP_SpawnerOverride_C|SetEnemy%20Density (Variables|Default|GetActor) (Variables|Default|GetEnemy%20Density _spawner_property))
  (Variables|/Game/Massive_PCG/MassiveShared/Blueprint/BP_SpawnerOverride.BP_SpawnerOverride_C|SetNPC%20Density (Variables|Default|GetActor) (Variables|Default|GetNPC%20Density _spawner_property))
  (Variables|/Game/Massive_PCG/MassiveShared/Blueprint/BP_SpawnerOverride.BP_SpawnerOverride_C|SetAnimal%20Density (Variables|Default|GetActor) (Variables|Default|GetAnimal%20Density _spawner_property))
  (Variables|/Game/Massive_PCG/MassiveShared/Blueprint/BP_SpawnerOverride.BP_SpawnerOverride_C|SetSpawnerMaxSlope (Variables|Default|GetActor) (Variables|Default|GetSpawnerMaxSlope _spawner_property))
  (Variables|/Game/Massive_PCG/MassiveShared/Blueprint/BP_SpawnerOverride.BP_SpawnerOverride_C|SetSpawner%20Enemy (Variables|Default|GetActor) (Variables|Default|GetSpawner%20Enemy _spawner_property))
  (Variables|/Game/Massive_PCG/MassiveShared/Blueprint/BP_SpawnerOverride.BP_SpawnerOverride_C|SetSpawner%20NPC (Variables|Default|GetActor) (Variables|Default|GetSpawner%20NPC _spawner_property))
  (Variables|/Game/Massive_PCG/MassiveShared/Blueprint/BP_SpawnerOverride.BP_SpawnerOverride_C|SetSpawner%20Animal (Variables|Default|GetActor) (Variables|Default|GetSpawner%20Animal _spawner_property))
  (PCG|Generate (Variables|/Game/Massive_PCG/MassiveShared/Blueprint/BP_SpawnerOverride.BP_SpawnerOverride_C|GetPCG (Variables|Default|GetActor)) false))