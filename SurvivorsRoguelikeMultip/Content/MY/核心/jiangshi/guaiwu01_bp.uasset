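; Zombie enemy character that wanders slowly, screams on spotting the player (with cooldown), then chases with a snarl loudly attached.
; Tick gates a forward sphere trace on the blackboard sight flag, toggling the AnimBP attack state and rotation mode.
; 攻击范围 traces between sockets to damage the player, skipping the last actor hit.
; Damage triggers hit reactions outside attacks; zero health ragdolls it, then destroys it after a delay.
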(event `self.ReceiveBeginPlay`
  (bind _outactors (`GameplayStatics.GetAllActorsOfClass` "/Game/MY/核心/juese/my_zhujue.my_zhujue_C"))
  (set `self.玩家蓝图实例` (`|GetArrayItem` _outactors)))

(event `随机找点移动`
  (bind `_怪我追逐音效` (`self.怪我追逐音效`))
  (if (not (`self.是否死亡`))
    (set `CharacterMovementComponent.MaxWalkSpeed` 40.0 (`self.CharacterMovement`))
    (`|ExecutionSequence`
      (:`then_0`
        (`/Engine/EditorBlueprintResources/StandardMacros.IsValid` `_怪我追逐音效`
          (:`Is Valid`
            (`ActorComponent.K2_DestroyComponent` `_怪我追逐音效`)
            (set `self.怪我追逐音效` null))))
      (:`then_1`
        (`/Engine/EditorBlueprintResources/StandardMacros.DoOnce` false :!label _label
          (:`Completed`
            (`KismetSystemLibrary.K2_SetTimer` null "重置尖叫" 15.0)))))))

(event `reset`
  (goto _label :!via `Reset`))

(event `重置尖叫`
  (set `self.是否可以尖叫` true))

(event `发现玩家要做的事`
  ;[1 1 1] 判断死亡后是否继续发现玩家
  (if (`|EnumEquality` (`/Game/MY/核心/juese/my_zhujue.playerFunction_state_ailisi` (`self.玩家蓝图实例`)) "NewEnumerator4")
    (`BlackboardComponent.SetValueAsBool` (`AIBlueprintHelperLibrary.GetBlackboard` (`AIBlueprintHelperLibrary.GetAIController` self)) "是否看到玩家" false)
    (elif (not (`self.是否死亡`))
      (`self.reset`)
      (`KismetSystemLibrary.K2_ClearTimer` null "重置尖叫")
      (if (`self.是否可以尖叫`)
        (set `self.是否可以尖叫` false)
        (set `self.正在尖叫` true)
        (bind _returnvalue (`AnimInstance.Montage_Play` (`SkeletalMeshComponent.GetAnimInstance` (`self.Mesh`)) "/Game/怪物素材01/导出的动画/guaiwu01_Zombie_Scream_Montage.guaiwu01_Zombie_Scream_Montage" 1.0 "MontageLength" 0.0 true))
        (set `CharacterMovementComponent.MaxWalkSpeed` 0.0 (`self.CharacterMovement`))
        (`KismetSystemLibrary.Delay` _returnvalue)
        (set `self.正在尖叫` false)
        (set `CharacterMovementComponent.MaxWalkSpeed` (`KismetMathLibrary.RandomFloatInRange` 400.0 500.0) (`self.CharacterMovement`) :!label _label)
        (if (not (`self.是否死亡`))
          (bind _returnvalue_2 (`GameplayStatics.SpawnSoundAttached` "/Game/教程游戏备份资源/丧尸素材/Sounds/Aggressive_Zombie_Snarls_Cue.Aggressive_Zombie_Snarls_Cue" (`self.Mesh`) "None" (0.0 0.0 0.0) (struct) "KeepRelativeOffset" false 1.0 1.0 (`KismetMathLibrary.RandomFloatInRange` 0.0 6.0) null null))
          (set `self.怪我追逐音效` _returnvalue_2))
        (elif (not (`self.正在尖叫`))
          (`/Engine/EditorBlueprintResources/StandardMacros.IsValid` (`self.怪我追逐音效`)
            (:`Is Not Valid`
              (goto _label))))))))

(event `self.ReceiveTick`
  (params (DeltaSeconds :type "Float (single-precision)"))
  (bind _returnvalue (`self.K2_GetActorLocation`))
  (bind _asguaiwu_01_anim (cast `/Game/MY/核心/jiangshi/guaiwu01_anim` (`SkeletalMeshComponent.GetAnimInstance` (`self.Mesh`)) :!pure true))
  (if (`self.是否死亡`)
    _
    (elif (`BlackboardComponent.GetValueAsBool` (`AIBlueprintHelperLibrary.GetBlackboard` (`AIBlueprintHelperLibrary.GetAIController` self)) "是否看到玩家")
      (bind (_outhit _returnvalue_2) (`KismetSystemLibrary.SphereTraceSingle` _returnvalue (+ _returnvalue (* (`self.GetActorForwardVector`) 110.0)) 100.0 "TraceTypeQuery4"))
      (if _returnvalue_2
        (bind _asmy_zhujue (cast `/Game/MY/核心/juese/my_zhujue` (`.HitActor` (`GameplayStatics.BreakHitResult` _outhit)))
          (:`then`
            (if (`/Game/MY/核心/juese/my_zhujue.是否死亡` _asmy_zhujue)
              (set `/Game/MY/核心/jiangshi/guaiwu01_anim.是否攻击` false _asguaiwu_01_anim :!label _label)
              (`self.更改控制旋转模式` true)
              (`AIController.K2_ClearFocus` (`AIBlueprintHelperLibrary.GetAIController` self))
              (`KismetSystemLibrary.K2_ClearTimer` null "攻击范围")
              (set `self.hitplayer` null)
              (else
                (set `/Game/MY/核心/jiangshi/guaiwu01_anim.是否攻击` true _asguaiwu_01_anim)
                (`self.更改控制旋转模式` false true))))
          (:`CastFailed`
            (goto _label)))
        (else
          (goto _label)))
      (else
        (goto _label)))))

(event `左脚脚步声`
  (if (not (`self.是否死亡`))
    (`/Game/MY/核心/juese/my_zhujue.脚步声判断` (`self.玩家蓝图实例`) (`self.左脚`))))

(event `右脚脚步声`
  (if (not (`self.是否死亡`))
    (`/Game/MY/核心/juese/my_zhujue.脚步声判断` (`self.玩家蓝图实例`) (`self.右键`))))

(event `随机怪物模型`
  (`SkeletalMeshComponent.SetSkeletalMeshAsset` (`self.Mesh`) (`|GetArrayItem` (`self.怪物的模型`) (`KismetMathLibrary.RandomIntegerInRange` 0))))

(event `self.ReceiveAnyDamage`
  (params (Damage :type "Float (single-precision)") (DamageType :type "DamageType Object Reference") (InstigatedBy :type "Controller Object Reference") (DamageCauser :type "Actor Object Reference"))
  (bind _asguaiwu_01_anim (`self.通信到动画蓝图`))
  (bind `_怪我追逐音效` (`self.怪我追逐音效`))
  (bind _output_get (set `self.怪物的血量` (- (`self.怪物的血量`) Damage)))
  (if (<= _output_get 0.0)
    ;[1 1 1] 物理
    (`/Engine/EditorBlueprintResources/StandardMacros.DoOnce` false
      (:`Completed`
        (`PrimitiveComponent.SetSimulatePhysics` (`self.Mesh`) true)
        (set `CharacterMovementComponent.MaxWalkSpeed` 0.0 (`self.CharacterMovement`))
        (set `self.是否死亡` true)
        (`PrimitiveComponent.SetCollisionEnabled` (`self.CapsuleComponent`) "NoCollision")
        (set `/Game/MY/核心/jiangshi/guaiwu01_anim.是否攻击` false (`self.通信到动画蓝图`))
        (`KismetSystemLibrary.K2_ClearTimer` null "攻击范围")
        (set `self.hitplayer` null)
        (`|ExecutionSequence`
          (:`then_0`
            (`/Engine/EditorBlueprintResources/StandardMacros.IsValid` `_怪我追逐音效`
              (:`Is Valid`
                (`ActorComponent.K2_DestroyComponent` `_怪我追逐音效`))))
          (:`then_1`
            (`KismetSystemLibrary.Delay` 15.0)
            (`self.K2_DestroyActor`)))))
    (elif (not (`/Game/MY/核心/jiangshi/guaiwu01_anim.是否攻击` _asguaiwu_01_anim))
      (set `/Game/MY/核心/jiangshi/guaiwu01_anim.是否被击中` true _asguaiwu_01_anim)
      (`KismetSystemLibrary.Delay` 1.0)
      (set `/Game/MY/核心/jiangshi/guaiwu01_anim.是否被击中` false _asguaiwu_01_anim))))

(event `攻击范围`
  (bind (_outhit _returnvalue) (`KismetSystemLibrary.SphereTraceSingle` (`SceneComponent.GetSocketLocation` (`self.Mesh`) (`self.攻击检测起始的骨骼`)) (`SceneComponent.GetSocketLocation` (`self.Mesh`) (`self.攻击范围终点骨骼`)) 40.0 "TraceTypeQuery4"))
  ;[1 1 1] 每次碰到玩家只会造成一次伤害
  (if _returnvalue
    (bind (_bblockinghit _binitialoverlap _time _distance _location _impactpoint _normal _impactnormal _physmat _hitactor) (`GameplayStatics.BreakHitResult` _outhit))
    (if (!= (`self.hitplayer`) _hitactor)
      (bind _asmy_zhujue (cast `/Game/MY/核心/juese/my_zhujue` _hitactor))
      (set `self.hitplayer` _hitactor)
      (`GameplayStatics.ApplyDamage` _asmy_zhujue 20.0)
      (`GameplayStatics.SpawnEmitterAtLocation` "/Game/粒子特效/Effects1/SmokeBuilder/Particles/P_SmokePuff1b.P_SmokePuff1b" _location (`KismetMathLibrary.Conv_VectorToRotator` _impactnormal) (0.1 0.1 0.1)))))

(fn `UserConstructionScript`)

(fn `更改控制旋转模式`
  (params (`将旋转朝向运动` :type Boolean) (`使用控制器旋转Yaw` :type Boolean))
  (set `CharacterMovementComponent.bOrientRotationToMovement` `将旋转朝向运动` (`self.CharacterMovement`))
  (set `self.bUseControllerRotationYaw` `使用控制器旋转Yaw`))

(fn `通信到动画蓝图`
  (returns (`AsGuaiwu 01 Anim` :type "/Game/MY/核心/jiangshi/guaiwu01_anim Object Reference"))
  ;[1 1 1] 注释
  (bind _asguaiwu_01_anim (cast `/Game/MY/核心/jiangshi/guaiwu01_anim` (`SkeletalMeshComponent.GetAnimInstance` (`self.Mesh`))))
  (return _asguaiwu_01_anim))