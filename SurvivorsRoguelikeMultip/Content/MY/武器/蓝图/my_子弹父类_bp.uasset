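; Parent bullet Blueprint that plays a weapon sound on spawn and resolves damage and impact effects on hit.
; A cast sequence handles spiders, monsters with headshot bonus damage, flying bugs, and victim variants with attached blood decals and bleeding.
; Several failed casts share a bullet-hole fallback, so it can fire even on creature hits; its sphere trace picks surface-specific effects.
; Shared tails push simulating physics components and destroy the bullet.
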(event `self.ReceiveBeginPlay`
  (`GameplayStatics.PlaySoundAtLocation` (`self.武器音效`) (`self.K2_GetActorLocation`) (struct) 1.0 1.0 0.0 null null null null))

(event `self.ReceiveHit`
  (params (MyComp :type "PrimitiveComponent Object Reference") (Other :type "Actor Object Reference") (OtherComp :type "PrimitiveComponent Object Reference") (bSelfMoved :type Boolean) (HitLocation :type "Vector Structure") (HitNormal :type "Vector Structure") (NormalImpulse :type "Vector Structure") (Hit :type "HitResult Structure (by ref)"))
  (bind `_击中旋转` (`self.击中旋转`))
  (bind `_击中旋转_2` (`self.击中旋转`))
  (bind `_击中旋转_3` (`self.击中旋转`))
  (set `self.Other` Other)
  (set `self.击中旋转` (`KismetMathLibrary.Conv_VectorToRotator` HitNormal))
  (set `self.击中位置` HitLocation)
  (`|ExecutionSequence`
    (:`then_0`
      ;[1 1 1] 蜘蛛
      (bind _asmy_zhizhu (cast `/Game/MY/核心/zhizhu/my_zhizhu` Other)
        (:`then`
          (`GameplayStatics.SpawnEmitterAtLocation` "/Game/粒子特效/GunImpacts/Particles/P_ImpactBlood.P_ImpactBlood" (`self.击中位置`) `_击中旋转_3` (0.6 0.6 0.6))
          (`GameplayStatics.SpawnEmitterAtLocation` "/Game/粒子特效/Effects1/SmokeBuilder/Particles/P_SmokePuff1b.P_SmokePuff1b" (`self.击中位置`) `_击中旋转_3` (0.1 0.1 0.1))
          (`GameplayStatics.ApplyDamage` _asmy_zhizhu 20.0)
          ;[1 1 1] 是否击中头部(伤害值)
          (`GameplayStatics.PlaySoundAtLocation` "/Game/音效/BulletImpact/Body/bullet_impact_body_flesh_01_Cue.bullet_impact_body_flesh_01_Cue" (`self.击中位置`) (struct) 1.0 1.0 0.0 null null null null :!label _label))
        (:`CastFailed`
          ;[1 1 1] 子弹的属性特效
          (`GameplayStatics.SpawnDecalAtLocation` "/Game/粒子特效/Bullet_Impact_Decal.Bullet_Impact_Decal" (7.0 7.0 7.0) (`self.击中位置`) (`self.击中旋转`) 20.0 :!label _label_2)
          (`self.击中物体特效` Hit))))
    (:`then_1`
      ;[1 1 1] 怪物01
      (bind _asguaiwu_01_bp (cast `/Game/MY/核心/jiangshi/guaiwu01_bp` Other)
        (:`then`
          (`GameplayStatics.SpawnEmitterAtLocation` "/Game/粒子特效/GunImpacts/Particles/P_ImpactBlood.P_ImpactBlood" (`self.击中位置`) (`self.击中旋转`) (0.4 0.4 0.4))
          (`GameplayStatics.SpawnEmitterAtLocation` "/Game/粒子特效/Effects1/SmokeBuilder/Particles/P_SmokePuff1b.P_SmokePuff1b" (`self.击中位置`) (`self.击中旋转`) (0.1 0.1 0.1))
          (if (== (`.HitBoneName` (`GameplayStatics.BreakHitResult` Hit)) "head")
            (`GameplayStatics.ApplyDamage` _asguaiwu_01_bp 20.0)
            (goto _label)
            (else
              ;;[1 1 1] 其他部位
              (`GameplayStatics.ApplyDamage` _asguaiwu_01_bp 6.0)
              (goto _label))))
        (:`CastFailed`
          (goto _label_2))))
    (:`then_2`
      (`|ExecutionSequence`
        (:`then_0`
          ;[1 1 1 1 28] 受害人
          (bind _asmy_shouhairen_actor_01 (cast `/Game/MY/核心/shouhairen/my_shouhairen_actor01` (`self.Other`))
            (:`then`
              (`NiagaraFunctionLibrary.SpawnSystemAtLocation` "/Game/Blood_VFX_Pack/Particles/Parts/P_E_Explosion_Splash.P_E_Explosion_Splash" (`self.击中位置`) `_击中旋转`)
              (`NiagaraFunctionLibrary.SpawnSystemAtLocation` "/Game/Blood_VFX_Pack/Particles/Parts/P_E_Blood_Smoke.P_E_Blood_Smoke" (`self.击中位置`) `_击中旋转` (2.0 2.0 2.0))
              (bind _returnvalue (`|SpawnActorFromClass` "/Game/Blood_VFX_Pack/Blueprints/BP_Decal.BP_Decal_C" (`KismetMathLibrary.MakeTransform` (`self.击中位置`) `_击中旋转` (1.0 1.0 1.0)) "Undefined" "OverrideRootScale" null 0.0 0.7 3.0 "/Game/Blood_VFX_Pack/Materials/MI_BloodDecal.MI_BloodDecal" 0.0 true false null))
              (bind _mesh (`Character.Mesh` _asmy_shouhairen_actor_01))
              (`self.K2_AttachToComponent` _returnvalue _mesh "pelvis" "SnapToTarget" "KeepWorld" "KeepWorld" true)
              (`GameplayStatics.ApplyDamage` _asmy_shouhairen_actor_01 6.0)
              (if (`/Game/MY/核心/shouhairen/my_shouhairen_actor01.是否严重受伤` _asmy_shouhairen_actor_01)
                (`NiagaraFunctionLibrary.SpawnSystemAttached` "/Game/Blood_VFX_Pack/Particles/Systems/Pixelated/P_Bleeding_Ribbon_Pix.P_Bleeding_Ribbon_Pix" _mesh "None" (`self.击中位置`) (`self.击中旋转`) "KeepWorldPosition" (`/Game/MY/核心/shouhairen/my_shouhairen_actor01.是否死亡` _asmy_shouhairen_actor_01))
                (goto _label)
                (else
                  (goto _label))))
            (:`CastFailed`
              (goto _label_2))))
        (:`then_1`
          (bind _asmy_shouhairen_actor_01_2 (cast `/Game/MY/核心/shouhairen/my_shouhairen_actor01_2` (`self.Other`)))
          (`NiagaraFunctionLibrary.SpawnSystemAtLocation` "/Game/Blood_VFX_Pack/Particles/Parts/P_E_Explosion_Splash.P_E_Explosion_Splash" (`self.击中位置`) (`self.击中旋转`))
          (`NiagaraFunctionLibrary.SpawnSystemAtLocation` "/Game/Blood_VFX_Pack/Particles/Parts/P_E_Blood_Smoke.P_E_Blood_Smoke" (`self.击中位置`) (`self.击中旋转`) (2.0 2.0 2.0))
          (bind _returnvalue_2 (`|SpawnActorFromClass` "/Game/Blood_VFX_Pack/Blueprints/BP_Decal.BP_Decal_C" (`KismetMathLibrary.MakeTransform` (`self.击中位置`) (`self.击中旋转`) (1.0 1.0 1.0)) "Undefined" "OverrideRootScale" null 0.0 0.7 3.0 "/Game/Blood_VFX_Pack/Materials/MI_BloodDecal.MI_BloodDecal" 0.0 true false null))
          (bind _mesh_2 (`Character.Mesh` _asmy_shouhairen_actor_01_2))
          (`self.K2_AttachToComponent` _returnvalue_2 _mesh_2 "pelvis" "SnapToTarget" "KeepWorld" "KeepWorld" true)
          (`GameplayStatics.ApplyDamage` _asmy_shouhairen_actor_01_2 6.0)
          (if (`/Game/MY/核心/shouhairen/my_shouhairen_actor01_2.是否严重受伤` _asmy_shouhairen_actor_01_2)
            (`NiagaraFunctionLibrary.SpawnSystemAttached` "/Game/Blood_VFX_Pack/Particles/Systems/Pixelated/P_Bleeding_Ribbon_Pix.P_Bleeding_Ribbon_Pix" _mesh_2 "None" (`self.击中位置`) (`self.击中旋转`) "KeepWorldPosition" false (`/Game/MY/核心/shouhairen/my_shouhairen_actor01_2.是否死亡` _asmy_shouhairen_actor_01_2))
            (goto _label)
            (else
              (goto _label))))
        (:`then_2`
          (bind _asmy_shouhairen_actor_01_4 (cast `/Game/MY/核心/shouhairen/my_shouhairen_actor01_4` (`self.Other`)))
          (`NiagaraFunctionLibrary.SpawnSystemAtLocation` "/Game/Blood_VFX_Pack/Particles/Parts/P_E_Explosion_Splash.P_E_Explosion_Splash" (`self.击中位置`) (`self.击中旋转`))
          (`NiagaraFunctionLibrary.SpawnSystemAtLocation` "/Game/Blood_VFX_Pack/Particles/Parts/P_E_Blood_Smoke.P_E_Blood_Smoke" (`self.击中位置`) (`self.击中旋转`) (2.0 2.0 2.0))
          (bind _returnvalue_3 (`|SpawnActorFromClass` "/Game/Blood_VFX_Pack/Blueprints/BP_Decal.BP_Decal_C" (`KismetMathLibrary.MakeTransform` (`self.击中位置`) (`self.击中旋转`) (1.0 1.0 1.0)) "Undefined" "OverrideRootScale" null 0.0 0.7 3.0 "/Game/Blood_VFX_Pack/Materials/MI_BloodDecal.MI_BloodDecal" 0.0 true false null))
          (bind _mesh_3 (`Character.Mesh` _asmy_shouhairen_actor_01_4))
          (`self.K2_AttachToComponent` _returnvalue_3 _mesh_3 "pelvis" "SnapToTarget" "KeepWorld" "KeepWorld" true)
          (`GameplayStatics.ApplyDamage` _asmy_shouhairen_actor_01_4 6.0)
          (if (`/Game/MY/核心/shouhairen/my_shouhairen_actor01_4.是否严重受伤` _asmy_shouhairen_actor_01_4)
            (`NiagaraFunctionLibrary.SpawnSystemAttached` "/Game/Blood_VFX_Pack/Particles/Systems/Pixelated/P_Bleeding_Ribbon_Pix.P_Bleeding_Ribbon_Pix" _mesh_3 "None" (`self.击中位置`) (`self.击中旋转`) "KeepWorldPosition" false (`/Game/MY/核心/shouhairen/my_shouhairen_actor01_4.是否死亡` _asmy_shouhairen_actor_01_4))
            (goto _label)
            (else
              (goto _label))))
        (:`then_3`
          (bind _asmy_shouhairen_actor_01_3 (cast `/Game/MY/核心/shouhairen/my_shouhairen_actor01_3` (`self.Other`)))
          (`NiagaraFunctionLibrary.SpawnSystemAtLocation` "/Game/Blood_VFX_Pack/Particles/Parts/P_E_Explosion_Splash.P_E_Explosion_Splash" (`self.击中位置`) (`self.击中旋转`))
          (`NiagaraFunctionLibrary.SpawnSystemAtLocation` "/Game/Blood_VFX_Pack/Particles/Parts/P_E_Blood_Smoke.P_E_Blood_Smoke" (`self.击中位置`) (`self.击中旋转`) (2.0 2.0 2.0))
          (bind _returnvalue_4 (`|SpawnActorFromClass` "/Game/Blood_VFX_Pack/Blueprints/BP_Decal.BP_Decal_C" (`KismetMathLibrary.MakeTransform` (`self.击中位置`) (`self.击中旋转`) (1.0 1.0 1.0)) "Undefined" "OverrideRootScale" null 0.0 0.7 3.0 "/Game/Blood_VFX_Pack/Materials/MI_BloodDecal.MI_BloodDecal" 0.0 true false null))
          (bind _mesh_4 (`Character.Mesh` _asmy_shouhairen_actor_01_3))
          (`self.K2_AttachToComponent` _returnvalue_4 _mesh_4 "pelvis" "SnapToTarget" "KeepWorld" "KeepWorld" true)
          (`GameplayStatics.ApplyDamage` _asmy_shouhairen_actor_01_3 6.0)
          (if (`/Game/MY/核心/shouhairen/my_shouhairen_actor01_3.是否严重受伤` _asmy_shouhairen_actor_01_3)
            (`NiagaraFunctionLibrary.SpawnSystemAttached` "/Game/Blood_VFX_Pack/Particles/Systems/Pixelated/P_Bleeding_Ribbon_Pix.P_Bleeding_Ribbon_Pix" _mesh_4 "None" (`self.击中位置`) (`self.击中旋转`) "KeepWorldPosition" false (`/Game/MY/核心/shouhairen/my_shouhairen_actor01_3.是否死亡` _asmy_shouhairen_actor_01_3))
            (goto _label)
            (else
              (goto _label))))))
    (:`then_3`
      ;[1 1 1] 飞虫01
      (bind _asfeicong_01 (cast `/Game/MY/核心/feicong01_yewai/feicong01` (`self.Other`))
        (:`then`
          (`GameplayStatics.SpawnEmitterAtLocation` "/Game/粒子特效/GunImpacts/Particles/P_ImpactBlood.P_ImpactBlood" (`self.击中位置`) `_击中旋转_2` (0.4 0.4 0.4))
          (`GameplayStatics.SpawnEmitterAtLocation` "/Game/粒子特效/Effects1/SmokeBuilder/Particles/P_SmokePuff1b.P_SmokePuff1b" (`self.击中位置`) `_击中旋转_2` (0.1 0.1 0.1))
          (`GameplayStatics.ApplyDamage` _asfeicong_01 20.0)
          (goto _label))
        (:`CastFailed`
          (goto _label_2)))))
  (`|ExecutionSequence`
    (:`then_0`
      (`/Engine/EditorBlueprintResources/StandardMacros.IsValid` OtherComp
        (:`Is Valid`
          (if (`SceneComponent.IsSimulatingPhysics` OtherComp "None")
            (`PrimitiveComponent.AddImpulse` OtherComp (* (`self.GetVelocity`) 2.0) "None" false)))))
    (:`then_1`
      (`self.K2_DestroyActor`))))

(fn `UserConstructionScript`)

(fn `击中物体特效`
  (params (Hit :type "HitResult Structure"))
  (bind (_bblockinghit _binitialoverlap _time _distance _location _impactpoint _normal) (`GameplayStatics.BreakHitResult` Hit))
  (bind _returnvalue (`KismetMathLibrary.Conv_VectorToRotator` _normal))
  (bind _outhit (`KismetSystemLibrary.SphereTraceSingle` _location _location 10.0 "TraceTypeQuery3"))
  (switch `EPhysicalSurface` (`GameplayStatics.GetSurfaceType` _outhit)
    (:`SurfaceType_Default`
      ;[1 1 1] 默认
      (`GameplayStatics.SpawnEmitterAtLocation` "/Game/粒子特效/GunImpacts1/Particles/P_ImpactDirt.P_ImpactDirt" _location _returnvalue (0.3 0.3 0.3))
      (`GameplayStatics.PlaySoundAtLocation` "/Game/音效/BulletImpact/Gravel/bullet_impact_gravel_01_Cue.bullet_impact_gravel_01_Cue" _location (struct) 1.0 1.0 0.0 null null null null))
    (:`SurfaceType1`
      (`GameplayStatics.SpawnEmitterAtLocation` "/Game/粒子特效/GunImpacts1/Particles/P_ImpactRock.P_ImpactRock" _location _returnvalue (0.3 0.3 0.3))
      (`GameplayStatics.PlaySoundAtLocation` "/Game/音效/BulletImpact/Rock/bullet_impact_rock_01_Cue.bullet_impact_rock_01_Cue" _location (struct) 1.0 1.0 0.0 null null null null))
    (:`SurfaceType2`
      (`GameplayStatics.SpawnEmitterAtLocation` "/Game/粒子特效/GunImpacts1/Particles/P_ImpactWood.P_ImpactWood" _location _returnvalue (0.3 0.3 0.3))
      (`GameplayStatics.PlaySoundAtLocation` "/Game/音效/Wood/footstep_wood_run_01_Cue.footstep_wood_run_01_Cue" _location (struct) 1.0 1.0 0.0 null null null null))
    (:`SurfaceType3`
      ;[1 1 1] 金属特效
      (`GameplayStatics.SpawnEmitterAtLocation` "/Game/粒子特效/GunImpacts1/Particles/P_ImpactMetal.P_ImpactMetal" _location _returnvalue (0.3 0.3 0.3))
      (`GameplayStatics.PlaySoundAtLocation` "/Game/音效/BulletImpact/Metal/bullet_impact_metal_heavy_01_Cue.bullet_impact_metal_heavy_01_Cue" _location (struct) 1.0 1.0 0.0 null null null null))
    (:`SurfaceType6`
      (`GameplayStatics.SpawnEmitterAtLocation` "/Game/粒子特效/GunImpacts1/Particles/P_ImpactGrass.P_ImpactGrass" _location _returnvalue (0.3 0.3 0.3))
      (`GameplayStatics.PlaySoundAtLocation` "/Game/音效/Grass/footstep_grass_run_01_Cue.footstep_grass_run_01_Cue" _location (struct) 1.0 1.0 0.0 null null null null))))